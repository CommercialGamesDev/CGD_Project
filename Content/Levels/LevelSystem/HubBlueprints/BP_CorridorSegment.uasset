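; Hub corridor segment that displays one level's stats and loads that level through GM_Multiplayer once a second character joins its trigger volume.
; A DT_LevelData row sets the name, colour, icon and framed picture.
; Save slots supply best time, gold horseshoe objectives and fastest-level sparkle, refreshed through BP_Level's OnSave event.
; Tick uses a Delay and curve to pulse the time text's scale in a loop.
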(event `self.ReceiveBeginPlay`
  (set `self.TimeAccumulator` 0.0)
  (bind _asgm_multiplayer (cast `/Game/ThirdPerson/Blueprints/GM_Multiplayer` (`GameplayStatics.GetGameMode`)))
  (set `self.Muliplayer` _asgm_multiplayer)
  (bind _asbp_level (cast `/Game/ThirdPerson/Blueprints/Util/BP_Level` (`GameplayStatics.GetGameInstance`)))
  (add `/Game/ThirdPerson/Blueprints/Util/BP_Level.OnSave` _asbp_level (delegate `Update Corridor Stats`)))

(event `Update Corridor Stats`
  ; Update the values based on completion data
  (`self.Set Save Data Values` :!label _label))

(event `Initialise Level Spawn`
  (params (`Data Table Row Name` :type Name))
  (bind _returnvalue (`|GetDataTableRow` "/Game/Levels/LevelSystem/DT_LevelData.DT_LevelData" `Data Table Row Name`)
    (:`then`
      (set `self.Level Data` _returnvalue)
      ; Parts of the corridor that will never change (level name and decoration)
      (`self.Set Static Display`)
      (goto _label))))

(event `self.LevelTrigger.OnComponentBeginOverlap`
  (params (OverlappedComponent :type "PrimitiveComponent Object Reference") (OtherActor :type "Actor Object Reference") (OtherComp :type "PrimitiveComponent Object Reference") (OtherBodyIndex :type Integer) (bFromSweep :type Boolean) (SweepResult :type "HitResult Structure (by ref)"))
  (bind (_level_data_levelname _level_data_levelindex _level_data_displaycolour _level_data_levelicon _level_data_levelblueprint) (break `/Game/Levels/LevelSystem/F_LevelStruct` (`self.Level Data`)))
  (bind _ascharacter (cast `Character` OtherActor))
  (bind _returnvalue (`KismetArrayLibrary.Array_Add` (`self.Players in volume`) _ascharacter))
  (if (>= _returnvalue 1)
    (`/Game/ThirdPerson/Blueprints/GM_Multiplayer.Load Level` (`self.Muliplayer`) _level_data_levelindex 0.0 0 0 false _level_data_levelblueprint)))

(event `self.LevelTrigger.OnComponentEndOverlap`
  (params (OverlappedComponent :type "PrimitiveComponent Object Reference") (OtherActor :type "Actor Object Reference") (OtherComp :type "PrimitiveComponent Object Reference") (OtherBodyIndex :type Integer))
  (bind _ascharacter (cast `Character` OtherActor))
  (`KismetArrayLibrary.Array_RemoveItem` (`self.Players in volume`) _ascharacter))

(event `self.ReceiveTick`
  (params (DeltaSeconds :type "Float (single-precision)"))
  (bind _returnvalue (`CurveFloat.GetFloatValue` (`self.ScaleCurve`) (`self.TimeAccumulator`)))
  (`KismetSystemLibrary.Delay` (`self.AnimationInterval`))
  (`SceneComponent.SetRelativeScale3D` (`self.FastestTime`) (`KismetMathLibrary.MakeVector` _returnvalue _returnvalue _returnvalue))
  (set `self.TimeAccumulator` (+ (`self.AnimationInterval`) (`self.TimeAccumulator`)))
  (if (>= (`self.TimeAccumulator`) (`self.AnimDuration`))
    (set `self.TimeAccumulator` 0.0)))

(fn `Convert To HMS`
  (params (CumulativeSeconds :type "Float (double-precision)"))
  (returns (`HMS String` :type String))
  (locals (Minutes :type String) (Seconds :type String))
  (bind _returnvalue (`KismetMathLibrary.FFloor` (/ CumulativeSeconds 60.0)))
  (bind _returnvalue_2 (- CumulativeSeconds (* _returnvalue 60)))
  (if (< _returnvalue 10)
    (set `local.Minutes` (`KismetStringLibrary.Concat_StrStr` "0" (`KismetStringLibrary.Conv_IntToString` _returnvalue)))
    (else
      (set `local.Minutes` (`KismetStringLibrary.Conv_IntToString` _returnvalue))))
  (if (< _returnvalue_2 10)
    (set `local.Seconds` (`KismetStringLibrary.Concat_StrStr` "0" (`KismetStringLibrary.Conv_IntToString` _returnvalue_2)))
    (else
      (set `local.Seconds` (`KismetStringLibrary.Conv_IntToString` _returnvalue_2))))
  (return (`KismetStringLibrary.Concat_StrStr` (`KismetStringLibrary.Concat_StrStr` (`local.Minutes`) ":") (`local.Seconds`))))

(fn `UserConstructionScript`)