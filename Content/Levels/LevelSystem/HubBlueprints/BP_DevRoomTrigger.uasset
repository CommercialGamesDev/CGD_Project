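; BP_DevRoomTrigger is a box trigger that switches lights and videos when a player enters its area, likely for a hub dev room.
; It counts overlaps from both local players and fires only for the first one inside, on first activation or when a light to deactivate is found visible.
; Firing plays and pauses assigned videos, hides one light set, then shows another after a short delay, with a sound at each step.
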(event `self.Box.OnComponentBeginOverlap`
  (params (OverlappedComponent :type "PrimitiveComponent Object Reference") (OtherActor :type "Actor Object Reference") (OtherComp :type "PrimitiveComponent Object Reference") (OtherBodyIndex :type Integer) (bFromSweep :type Boolean) (SweepResult :type "HitResult Structure (by ref)"))
  (if (or (== OtherActor (`GameplayStatics.GetPlayerPawn` 0)) (== OtherActor (`GameplayStatics.GetPlayerPawn` 1)))
    (bind _result (`/Engine/EditorBlueprintResources/StandardMacros.IncrementInt` (`self.PlayersInside`))
      (:`  `
        (for _array_element (`self.LightsToDeactivate`)
          (if (`SceneComponent.bVisible` (`Light.LightComponent` _array_element))
            (set `self.AnyStillOn?` true)))
        (if (and (or (`self.AnyStillOn?`) (not (`self.HasActivated`))) (== _result 1))
          (set `self.HasActivated` true)
          (for _array_element_2 (`self.VideosToPlay`)
            (`MediaPlayer.Play` _array_element_2))
          (for _array_element_3 (`self.VideosToStop`)
            (`MediaPlayer.Pause` _array_element_3))
          (for _array_element_4 (`self.LightsToDeactivate`)
            (`SceneComponent.SetVisibility` (`Light.LightComponent` _array_element_4) false false))
          (`GameplayStatics.PlaySound2D` "/Game/Audio/sound/Light1.Light1" 1.0 1.0 0.0 null null)
          (`KismetSystemLibrary.Delay` 0.6)
          (for _array_element_5 (`self.LightsToActivate`)
            (`SceneComponent.SetVisibility` (`Light.LightComponent` _array_element_5) true false))
          (`GameplayStatics.PlaySound2D` "/Game/Audio/sound/Light2.Light2" 1.0 1.0 0.0 null null))))))

(event `self.Box.OnComponentEndOverlap`
  (params (OverlappedComponent :type "PrimitiveComponent Object Reference") (OtherActor :type "Actor Object Reference") (OtherComp :type "PrimitiveComponent Object Reference") (OtherBodyIndex :type Integer))
  (if (or (== OtherActor (`GameplayStatics.GetPlayerPawn` 0)) (== OtherActor (`GameplayStatics.GetPlayerPawn` 1)))
    (`/Engine/EditorBlueprintResources/StandardMacros.DecrementInt` (`self.PlayersInside`))))

(fn `UserConstructionScript`)