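; Hub trigger that teleports all third-person player characters to a fixed showcase destination once a second character is inside it.
; The overlap locks movement and pausing on the BP_Level game instance, starts a delayed teleport timer and runs the RedCurtain macro.
; The guarded macro hides the move behind a curtain widget, snaps the camera drone to the corridor's rail and FOV, then restores control and cleans up.
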(event `self.ReceiveBeginPlay`
  (`KismetArrayLibrary.Array_Clear` (`self.Players in Collider`)))

(event `self.Trigger.OnComponentBeginOverlap`
  (params (OverlappedComponent :type "PrimitiveComponent Object Reference") (OtherActor :type "Actor Object Reference") (OtherComp :type "PrimitiveComponent Object Reference") (OtherBodyIndex :type Integer) (bFromSweep :type Boolean) (SweepResult :type "HitResult Structure (by ref)"))
  (bind _ascharacter (cast `Character` OtherActor))
  (bind _returnvalue (`KismetArrayLibrary.Array_Add` (`self.Players in Collider`) _ascharacter))
  (if (>= _returnvalue 1)
    (`KismetSystemLibrary.K2_SetTimerDelegate` (delegate `Teleport Players`) 2.2)
    (bind _asbp_level (cast `/Game/ThirdPerson/Blueprints/Util/BP_Level` (`GameplayStatics.GetGameInstance`)))
    (set `/Game/ThirdPerson/Blueprints/Util/BP_Level.CanMove` false _asbp_level)
    (set `/Game/ThirdPerson/Blueprints/Util/BP_Level.CanPause` false _asbp_level)
    (`self.Red Curtain`)))

(event `self.Trigger.OnComponentEndOverlap`
  (params (OverlappedComponent :type "PrimitiveComponent Object Reference") (OtherActor :type "Actor Object Reference") (OtherComp :type "PrimitiveComponent Object Reference") (OtherBodyIndex :type Integer))
  (bind _ascharacter (cast `Character` OtherActor))
  (`KismetArrayLibrary.Array_RemoveItem` (`self.Players in Collider`) _ascharacter))

(event `Teleport Players`
  (bind _outactors (`GameplayStatics.GetAllActorsOfClass` "/Game/ThirdPerson/Blueprints/BP_ThirdPersonCharacter.BP_ThirdPersonCharacter_C"))
  (for _array_element _outactors
    (`self.K2_TeleportTo` :`self` _array_element :`DestLocation` (1140.0 -2270.0 232.0))))

(fn `UserConstructionScript`)