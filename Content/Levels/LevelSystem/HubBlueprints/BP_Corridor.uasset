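; Hub corridor that builds itself from DT_LevelData, with exit triggers that move players out behind a curtain transition.
; On BeginPlay it spawns an attached corridor segment per level, excluding hub and tutorial, and places StageRight at the end.
; Two exit colliders share a character list; a second entry locks movement and pause via BP_Level.
; A timed teleport moves all players to a fixed spot while RedCurtain snaps the camera drone to NextRail.
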(event `self.ReceiveBeginPlay`
  (bind _stageright (`self.StageRight`))
  (bind (_relativelocation_x _relativelocation_y _relativelocation_z) (`KismetMathLibrary.BreakVector` (`SceneComponent.RelativeLocation` _stageright)))
  (`KismetArrayLibrary.Array_Clear` (`self.Characters In Volume`))
  (bind _outrownames (`DataTableFunctionLibrary.GetDataTableRowNames` "/Game/Levels/LevelSystem/DT_LevelData.DT_LevelData"))
  ; Set the amount of levels from the data table
  (set `self.Out Row Names` _outrownames)
  (set `self.Total Levels` (- (`KismetArrayLibrary.Array_Length` (`self.Out Row Names`)) 2))
  (`self.Setup Corridor Segments`
    (:`Completed`
      ; Place stage right at the end of the corridor
      (`SceneComponent.K2_SetRelativeLocation` _stageright (`KismetMathLibrary.MakeVector` (+ (* (`self.Total Levels`) (`self.Segment Width`)) 50.0) _relativelocation_y _relativelocation_z) false true))))

(event `self.ExitCollider.OnComponentBeginOverlap`
  (params (OverlappedComponent :type "PrimitiveComponent Object Reference") (OtherActor :type "Actor Object Reference") (OtherComp :type "PrimitiveComponent Object Reference") (OtherBodyIndex :type Integer) (bFromSweep :type Boolean) (SweepResult :type "HitResult Structure (by ref)"))
  (bind _ascharacter (cast `Character` OtherActor))
  (bind _returnvalue (`KismetArrayLibrary.Array_Add` (`self.Characters In Volume`) _ascharacter))
  (if (>= _returnvalue 1)
    (`KismetSystemLibrary.K2_SetTimerDelegate` (delegate `Teleport To`) 2.2 :!label _label)
    (bind _asbp_level (cast `/Game/ThirdPerson/Blueprints/Util/BP_Level` (`GameplayStatics.GetGameInstance`)))
    (set `/Game/ThirdPerson/Blueprints/Util/BP_Level.CanMove` false _asbp_level)
    (set `/Game/ThirdPerson/Blueprints/Util/BP_Level.CanPause` false _asbp_level)
    (`self.Red Curtain`)))

(event `self.ExitCollider1.OnComponentBeginOverlap`
  (params (OverlappedComponent :type "PrimitiveComponent Object Reference") (OtherActor :type "Actor Object Reference") (OtherComp :type "PrimitiveComponent Object Reference") (OtherBodyIndex :type Integer) (bFromSweep :type Boolean) (SweepResult :type "HitResult Structure (by ref)"))
  (bind _ascharacter (cast `Character` OtherActor))
  (bind _returnvalue (`KismetArrayLibrary.Array_Add` (`self.Characters In Volume`) _ascharacter))
  (if (>= _returnvalue 1)
    (goto _label)))

(event `Teleport To`
  (bind _outactors (`GameplayStatics.GetAllActorsOfClass` "/Game/ThirdPerson/Blueprints/BP_ThirdPersonCharacter.BP_ThirdPersonCharacter_C"))
  (for _array_element _outactors
    (`self.K2_TeleportTo` :`self` _array_element :`DestLocation` (1140.0 -2270.0 232.0))))

(event `self.ExitCollider1.OnComponentEndOverlap`
  (params (OverlappedComponent :type "PrimitiveComponent Object Reference") (OtherActor :type "Actor Object Reference") (OtherComp :type "PrimitiveComponent Object Reference") (OtherBodyIndex :type Integer))
  (bind _ascharacter (cast `Character` OtherActor))
  (`KismetArrayLibrary.Array_RemoveItem` (`self.Characters In Volume`) _ascharacter))

(event `self.ExitCollider.OnComponentEndOverlap`
  (params (OverlappedComponent :type "PrimitiveComponent Object Reference") (OtherActor :type "Actor Object Reference") (OtherComp :type "PrimitiveComponent Object Reference") (OtherBodyIndex :type Integer))
  (bind _ascharacter (cast `Character` OtherActor))
  (`KismetArrayLibrary.Array_RemoveItem` (`self.Characters In Volume`) _ascharacter))

(fn `UserConstructionScript`)