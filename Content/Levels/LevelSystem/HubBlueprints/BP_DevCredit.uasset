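; BP_DevCredit is a developer credit display actor in the hub level blueprints, showing a person's name, image and quote.
; On BeginPlay it copies its name, colour, material and quote variables into text components and an image component.
; The construction script is empty, so this setup applies only when play begins.
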(event `self.ReceiveBeginPlay`
  (bind _first_name_text (`self.First name text`))
  (bind _secondname_text (`self.SecondName Text`))
  (`TextRenderComponent.K2_SetText` _first_name_text (`self.FirstName`))
  (`TextRenderComponent.SetTextRenderColor` _first_name_text (`self.Colour`))
  (`TextRenderComponent.K2_SetText` _secondname_text (`self.SecondName`))
  (`TextRenderComponent.SetTextRenderColor` _secondname_text (`self.Colour`))
  (`PrimitiveComponent.SetMaterial` (`self.PlayerImage`) 0 (`self.Material`))
  (`TextRenderComponent.K2_SetText` (`self.Quote Text`) (`self.Quote`)))

(fn `UserConstructionScript`)