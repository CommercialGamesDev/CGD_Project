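; Hub manager for the dev room that controls which BP_DevRoomTrigger area is active.
; On BeginPlay it deactivates every trigger in the level, then opens each media player's matching source and pauses it.
; TriggerTrigger ignores the current trigger; for a new one, it deactivates any previous trigger and waits briefly before activating the replacement.
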(event `self.ReceiveBeginPlay`
  (bind _outactors (`GameplayStatics.GetAllActorsOfClass` "/Game/Levels/LevelSystem/HubBlueprints/BP_DevRoomTrigger.BP_DevRoomTrigger_C"))
  (for _array_element _outactors
    (`/Game/Levels/LevelSystem/HubBlueprints/BP_DevRoomTrigger.DeactivateThese` _array_element false))
  (for (_array_element_2 _array_index) (`self.Players`)
    (`MediaPlayer.OpenSource` _array_element_2 (`|GetArrayItem` (`self.Sources`) _array_index))
    (`MediaPlayer.Pause` _array_element_2)))

(event `TriggerTrigger`
  (params (`Trigger Trigger Trigger` :type "/Game/Levels/LevelSystem/HubBlueprints/BP_DevRoomTrigger Object Reference"))
  (bind _mostrecentdevroomtrigger (`self.MostRecentDevRoomTrigger`))
  (if (!= `Trigger Trigger Trigger` _mostrecentdevroomtrigger)
    (if (!= null _mostrecentdevroomtrigger)
      (`/Game/Levels/LevelSystem/HubBlueprints/BP_DevRoomTrigger.DeactivateThese` _mostrecentdevroomtrigger true)
      (set `self.MostRecentDevRoomTrigger` `Trigger Trigger Trigger`)
      (`KismetSystemLibrary.Delay` 0.6)
      (else
        (set `self.MostRecentDevRoomTrigger` `Trigger Trigger Trigger`)))
    (`/Game/Levels/LevelSystem/HubBlueprints/BP_DevRoomTrigger.ActivateThese` `Trigger Trigger Trigger` true)))

(fn `UserConstructionScript`)