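; Hub trigger volume that loads a numbered level once at least two characters stand inside it.
; Overlap events maintain a list of characters in the volume, and reaching two fires an event that switches on a Function setting and calls LoadLevel on the cached GM_Multiplayer game mode.
; The construction script writes the Text variable to a TextRender component as the volume's label.
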(event `self.ReceiveBeginPlay`
  (`KismetArrayLibrary.Array_Clear` (`self.PlayersInVolume`))
  (bind _asgm_multiplayer (cast `/Game/ThirdPerson/Blueprints/GM_Multiplayer` (`GameplayStatics.GetGameMode`)))
  (set `self.Muliplayer` _asgm_multiplayer))

(event `self.Volume.OnComponentBeginOverlap`
  (params (OverlappedComponent :type "PrimitiveComponent Object Reference") (OtherActor :type "Actor Object Reference") (OtherComp :type "PrimitiveComponent Object Reference") (OtherBodyIndex :type Integer) (bFromSweep :type Boolean) (SweepResult :type "HitResult Structure (by ref)"))
  (bind _ascharacter (cast `Character` OtherActor))
  (`KismetArrayLibrary.Array_Add` (`self.PlayersInVolume`) _ascharacter)
  (if (>= (`KismetArrayLibrary.Array_Length` (`self.PlayersInVolume`)) 2)
    (`self.Players trigger volume`)))

(event `self.Volume.OnComponentEndOverlap`
  (params (OverlappedComponent :type "PrimitiveComponent Object Reference") (OtherActor :type "Actor Object Reference") (OtherComp :type "PrimitiveComponent Object Reference") (OtherBodyIndex :type Integer))
  (bind _ascharacter (cast `Character` OtherActor))
  (`KismetArrayLibrary.Array_RemoveItem` (`self.PlayersInVolume`) _ascharacter))

(event `Players trigger volume`
  (switch `name` (`self.Function`)
    (:`Default`
      _)
    (:`LoadLevel`
      _))
  (`/Game/ThirdPerson/Blueprints/GM_Multiplayer.Load Level` (`self.Muliplayer`) (`self.LevelNumber`)))

(fn `UserConstructionScript`
  (`TextRenderComponent.K2_SetText` (`self.TextRender`) (`KismetTextLibrary.Conv_NameToText` (`self.Text`))))