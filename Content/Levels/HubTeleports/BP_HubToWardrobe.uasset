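; Hub teleport trigger that sends players to a fixed location, the wardrobe going by the asset name, once at least two characters stand in its Volume.
; Overlap events track occupants, and reaching two disables movement and pausing on the BP_Level game instance and starts a delayed teleport of every BP_ThirdPersonCharacter.
; A guarded RedCurtain transition masks the move, then restores both flags and removes its widget.
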(event `self.ReceiveBeginPlay`
  (`KismetArrayLibrary.Array_Clear` (`self.PlayersInVolume`)))

(event `self.Volume.OnComponentBeginOverlap`
  (params (OverlappedComponent :type "PrimitiveComponent Object Reference") (OtherActor :type "Actor Object Reference") (OtherComp :type "PrimitiveComponent Object Reference") (OtherBodyIndex :type Integer) (bFromSweep :type Boolean) (SweepResult :type "HitResult Structure (by ref)"))
  (bind _ascharacter (cast `Character` OtherActor))
  (`KismetArrayLibrary.Array_Add` (`self.PlayersInVolume`) _ascharacter)
  (if (>= (`KismetArrayLibrary.Array_Length` (`self.PlayersInVolume`)) 2)
    (`KismetSystemLibrary.K2_SetTimerDelegate` (delegate `PlayersTP`) 2.2)
    (bind _asbp_level (cast `/Game/ThirdPerson/Blueprints/Util/BP_Level` (`GameplayStatics.GetGameInstance`)))
    (set `/Game/ThirdPerson/Blueprints/Util/BP_Level.CanMove` false _asbp_level)
    (set `/Game/ThirdPerson/Blueprints/Util/BP_Level.CanPause` false _asbp_level)
    (`self.Red Curtain`)))

(event `PlayersTP`
  (bind _outactors (`GameplayStatics.GetAllActorsOfClass` "/Game/ThirdPerson/Blueprints/BP_ThirdPersonCharacter.BP_ThirdPersonCharacter_C"))
  (for _array_element _outactors
    (`self.K2_TeleportTo` :`self` _array_element :`DestLocation` (-15660.0 -3300.0 370.0))))

(event `self.Volume.OnComponentEndOverlap`
  (params (OverlappedComponent :type "PrimitiveComponent Object Reference") (OtherActor :type "Actor Object Reference") (OtherComp :type "PrimitiveComponent Object Reference") (OtherBodyIndex :type Integer))
  (bind _ascharacter (cast `Character` OtherActor))
  (`KismetArrayLibrary.Array_RemoveItem` (`self.PlayersInVolume`) _ascharacter))

(fn `UserConstructionScript`)