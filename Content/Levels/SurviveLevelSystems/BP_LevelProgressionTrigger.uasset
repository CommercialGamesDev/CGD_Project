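; Level progression trigger for the survive level that moves the stage on when the player enters its box.
; A Player-tagged overlap passes a DoOnce into IncrementStage, which steps LevelStage once along Start, three speed stages and End.
; StageSwitch sends each new stage's signal through CallBPCommunicator.
; Speed 1 also starts the level's countdown board and rotates the start drawbridge, while End rotates the end drawbridge.
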(event `self.ReceiveBeginPlay`
  (bind _returnvalue (`GameplayStatics.GetActorOfClass` "/Game/Levels/SurviveLevelSystems/BP_CountdownBoard.BP_CountdownBoard_C"))
  (set `self.CountdownBoard` _returnvalue))

(event `StageSwitch`
  (params (Stage :type "/Game/Levels/SurviveLevelSystems/E_SurviveStage Enum" :default "NewEnumerator0"))
  (switch `/Game/Levels/SurviveLevelSystems/E_SurviveStage` Stage
    (:`NewEnumerator1`
      (`self.BPCommunicator` "NewEnumerator0")
      (`/Game/Levels/SurviveLevelSystems/BP_CountdownBoard.StartCoutndown` (`self.CountdownBoard`))
      (`self.K2_SetActorRotation` :`self` (`self.StartDrawbridge`)))
    (:`NewEnumerator2`
      (`self.BPCommunicator` "NewEnumerator6"))
    (:`NewEnumerator3`
      (`self.BPCommunicator` "NewEnumerator7"))
    (:`NewEnumerator4`
      (`self.BPCommunicator` "NewEnumerator1")
      (`self.K2_SetActorRotation` (`self.EndDrawbridge`) (struct :`Yaw` 180.0) false))))

(event `self.Box.OnComponentBeginOverlap`
  (params (OverlappedComponent :type "PrimitiveComponent Object Reference") (OtherActor :type "Actor Object Reference") (OtherComp :type "PrimitiveComponent Object Reference") (OtherBodyIndex :type Integer) (bFromSweep :type Boolean) (SweepResult :type "HitResult Structure (by ref)"))
  (if (`self.ActorHasTag` OtherActor "Player")
    (`/Engine/EditorBlueprintResources/StandardMacros.DoOnce` false
      (:`Completed`
        (`self.IncrementStage`)))))

(fn `IncrementStage`
  (switch `/Game/Levels/SurviveLevelSystems/E_SurviveStage` (`self.LevelStage`)
    (:`NewEnumerator0`
      (bind _output_get (set `self.LevelStage` "NewEnumerator1"))
      (`self.StageSwitch` _output_get))
    (:`NewEnumerator1`
      (bind _output_get_2 (set `self.LevelStage` "NewEnumerator2"))
      (`self.StageSwitch` _output_get_2))
    (:`NewEnumerator2`
      (bind _output_get_3 (set `self.LevelStage` "NewEnumerator3"))
      (`self.StageSwitch` _output_get_3))
    (:`NewEnumerator3`
      (bind _output_get_4 (set `self.LevelStage` "NewEnumerator4"))
      (`self.StageSwitch` _output_get_4))))

(fn `UserConstructionScript`)