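; BP_CountdownBoard is a survive-level board that displays a countdown and advances the level's stages as time runs out.
; StartCoutndown plays a Timeline in reverse from its end, writing the track value to a TextRender as formatted time.
; Separate DoOnce gates call IncrementStage on the BP_LevelProgressionTrigger found at BeginPlay, at two time thresholds and when the countdown finishes.
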(event `self.ReceiveBeginPlay`
  (bind _returnvalue (`GameplayStatics.GetActorOfClass` "/Game/Levels/SurviveLevelSystems/BP_LevelProgressionTrigger.BP_LevelProgressionTrigger_C"))
  (set `self.SurviveManager` _returnvalue))

(event `StartCoutndown`
  (bind (_direction _newtrack_0) (`Timeline|Timeline` :!via `ReverseFromEnd`)
    (:`Update`
      (`|ExecutionSequence`
        (:`then_0`
          (`TextRenderComponent.K2_SetText` (`self.TextRender`) (`KismetTextLibrary.Conv_StringToText` (`KismetStringLibrary.TimeSecondsToString` _newtrack_0))))
        (:`then_1`
          (if (<= _newtrack_0 20.0)
            (`/Engine/EditorBlueprintResources/StandardMacros.DoOnce` false
              (:`Completed`
                (`/Game/Levels/SurviveLevelSystems/BP_LevelProgressionTrigger.IncrementStage` (`self.SurviveManager`))))
            (elif (<= _newtrack_0 40.0)
              (`/Engine/EditorBlueprintResources/StandardMacros.DoOnce` false
                (:`Completed`
                  (`/Game/Levels/SurviveLevelSystems/BP_LevelProgressionTrigger.IncrementStage` (`self.SurviveManager`)))))))))
    (:`Finished`
      (`/Engine/EditorBlueprintResources/StandardMacros.DoOnce` false
        (:`Completed`
          (`/Game/Levels/SurviveLevelSystems/BP_LevelProgressionTrigger.IncrementStage` (`self.SurviveManager`)))))))

(fn `UserConstructionScript`)