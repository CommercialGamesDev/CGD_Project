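; BP_Bobject is a configurable decorative actor that shows a static mesh which rotates and bobs vertically.
; The construction script applies the chosen mesh, material, shadow setting, rotation rate and bob speed to the mesh, RotatingMovement component and Bob timeline.
; Tick calls Play on the timeline, whose updates add the track value times BOBHeight to the mesh's current relative Z, so offsets accumulate rather than use a stored origin.
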(event `self.ReceiveTick`
  (params (DeltaSeconds :type "Float (single-precision)"))
  (bind _staticmesh (`self.StaticMesh`))
  (bind (_relativelocation_x _relativelocation_y _relativelocation_z) (`KismetMathLibrary.BreakVector` (`SceneComponent.RelativeLocation` _staticmesh)))
  (bind (_direction _newtrack_0) (`Timeline|Bob`)
    (:`Update`
      (`SceneComponent.K2_SetRelativeLocation` _staticmesh (`KismetMathLibrary.MakeVector` _relativelocation_x _relativelocation_y (+ _relativelocation_z (* _newtrack_0 (`self.BOBHeight`)))) false false))))

(fn `UserConstructionScript`
  (`StaticMeshComponent.SetStaticMesh` (`self.StaticMesh`) (`self.Mesh`))
  (set `RotatingMovementComponent.RotationRate` (`self.Rotation`) (`self.RotatingMovement`))
  (`PrimitiveComponent.SetMaterial` (`self.StaticMesh`) (`self.MaterialIndex`) (`self.Material`))
  (`PrimitiveComponent.SetCastShadow` (`self.StaticMesh`) (`self.CastShadow`))
  (`TimelineComponent.SetPlayRate` (`self.Bob`) (`self.BOBSpeed`)))