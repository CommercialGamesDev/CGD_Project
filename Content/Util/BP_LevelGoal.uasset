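; Level goal actor that fires a completion event when a player character reaches it.
; An overlap on its collider is accepted only from the characters of player 0 or player 1, and a completion flag, reset on begin play, keeps it from triggering more than once.
; CompleteLevel is an empty event in this Blueprint.
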(event `self.ReceiveBeginPlay`
  (set `self.IsComplete` false))

(event `self.Collider.OnComponentBeginOverlap`
  (params (OverlappedComponent :type "PrimitiveComponent Object Reference") (OtherActor :type "Actor Object Reference") (OtherComp :type "PrimitiveComponent Object Reference") (OtherBodyIndex :type Integer) (bFromSweep :type Boolean) (SweepResult :type "HitResult Structure (by ref)"))
  (if (not (`self.IsComplete`))
    (if (or (== (`GameplayStatics.GetPlayerCharacter` 0) OtherActor) (== OtherActor (`GameplayStatics.GetPlayerCharacter` 1)))
      (set `self.IsComplete` true)
      (`self.CompleteLevel`))))

(event `CompleteLevel`)

(fn `UserConstructionScript`)