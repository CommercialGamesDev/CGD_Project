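; Global manager for crowd audiences, controlling every BP_AudienceCluster in the level and relaying timed cheers to them.
; On construction it gathers the clusters and estimates total population after gaps.
; At BeginPlay and on the bound save event, it reloads the Settings save, turning density into a clamped gap percentage.
; It then toggles cluster animations, regenerates each crowd and recounts, using StartAnimated when settings are missing.
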(event `self.ReceiveBeginPlay`
  (bind _asbp_level (cast `/Game/ThirdPerson/Blueprints/Util/BP_Level` (`GameplayStatics.GetGameInstance`))
    (:`then`
      (add `/Game/ThirdPerson/Blueprints/Util/BP_Level.OnSave` _asbp_level (delegate `SettingsUpdated`)))
    (:`CastFailed`
      (`KismetSystemLibrary.PrintString` "Warning: Audience manager could not find Game Instance")))
  (bind _returnvalue (`GameplayStatics.LoadGameFromSlot` "Settings"))
  (bind _asbp_settings_data (cast `/Game/Data/BP_SettingsData` _returnvalue)
    (:`then`
      (set `self.Settings Data` _asbp_settings_data))
    (:`CastFailed`
      (`KismetSystemLibrary.PrintString` "Warning: Audience manager could not find settings data")))
  (`self.SettingsUpdated`))

(event `CheerAudience`
  (params (`Cheer Duration` :type "Float (double-precision)"))
  (for _array_element (`self.AudienceClusters`)
    (`/Game/Audience/BP_AudienceCluster.AudienceCheer` _array_element `Cheer Duration`)))

(event `SettingsUpdated`
  (`/Engine/EditorBlueprintResources/StandardMacros.IsValid` (`self.Settings Data`)
    (:`Is Valid`
      (bind _returnvalue (`GameplayStatics.LoadGameFromSlot` "Settings"))
      (bind _asbp_settings_data (cast `/Game/Data/BP_SettingsData` _returnvalue))
      (bind _output_get (set `self.Settings Data` _asbp_settings_data))
      (set `self.AudienceGap%` (`KismetMathLibrary.FClamp` (- 100.0 (`/Game/Data/BP_SettingsData.AudienceDensity` _output_get)) 0.0 80.0))
      (set `self.TellToAnimate` (`/Game/Data/BP_SettingsData.AudienceAnimations` _output_get)))
    (:`Is Not Valid`
      (set `self.TellToAnimate` (`self.StartAnimated`))))
  (for _array_element (`self.AudienceClusters`)
    (`/Game/Audience/BP_AudienceCluster.ToggleAnimations` _array_element (`self.TellToAnimate`)))
  (for _array_element_2 (`self.AudienceClusters`)
    (`/Game/Audience/BP_AudienceCluster.RegenerateAudience` _array_element_2 (`self.AudienceGap%`))
    (`self.CalculateAudienceMembers`)))

(fn `CalculateAudienceMembers`
  (set `self.TotalPopulationEstimate` 0)
  (bind _outactors (`GameplayStatics.GetAllActorsOfClass` "/Game/Audience/BP_AudienceCluster.BP_AudienceCluster_C"))
  (bind _output_get (set `self.AudienceClusters` _outactors))
  (for _array_element _output_get
    (set `self.TotalPopulationEstimate` (+ (- (`/Game/Audience/BP_AudienceCluster.AudiencePopulation` _array_element) (* (`/Game/Audience/BP_AudienceCluster.AudiencePopulation` _array_element) (* (`/Game/Audience/BP_AudienceCluster.GapProbablity` _array_element) 0.01))) (`self.TotalPopulationEstimate`)))))

(fn `UserConstructionScript`
  (`self.CalculateAudienceMembers`))