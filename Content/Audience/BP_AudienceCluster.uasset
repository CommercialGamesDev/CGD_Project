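; Audience cluster actor that spawns a row of randomly coloured paper sprites, with rare horse, goose and all-green-geese variants.
; RegenerateAudience rebuilds the row outwards from the centre in alternating sides, randomly removing members to leave gaps.
; A gated, delay-stepped Tick bobs recently rendered sprites along a float curve with per-member phase offsets and occasional flips.
; AudienceCheer temporarily swaps that curve, then restores positions; the construction script places editor stand-ins marking the row's extents.
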(event `self.ReceiveBeginPlay`)

(event `RegenAudience`
  (bind _spacing_accumulator (`self.Spacing Accumulator`))
  (bind _outitem (`KismetArrayLibrary.Array_Random` (`self.SpriteFlipRotator`)))
  (if (and (`KismetMathLibrary.RandomBoolWithWeight` (/ (`self.GreenGeese%Chance`) 100.0)) (`self.GreenGeeseTeam`))
    ; Green geese easter egg
    (for _index (range 10)
      (set `self.LoopIndex` _index)
      (set `self.GapProbablity` 0.0)
      (`self.GreenGeeseGen`))
    (else
      (for _index_2 (range (`self.AudiencePopulation`))
        (set `self.LoopIndex` _index_2)
        (bind _returnvalue (`AddComponent|NODE_AddPaperSpriteComponent-0` :`bManualAttachment` true))
        (`PaperSpriteComponent.SetSpriteColor` _returnvalue (`KismetArrayLibrary.Array_Random` (`self.RandomColour`)))
        (`PrimitiveComponent.SetMaterial` _returnvalue 0 "/Game/Particles/SpriteMats/LevelIconMat.LevelIconMat")
        (`PrimitiveComponent.SetCollisionEnabled` _returnvalue "NoCollision")
        (`PrimitiveComponent.SetCastShadow` _returnvalue false)
        (`BlueprintMapLibrary.Map_Add` (`self.MemberList`) _returnvalue (`KismetMathLibrary.RandomFloatInRange` 0.0 4.0))
        (switch `int` (`KismetMathLibrary.RandomInteger` 89)
          (:`Default`
            (`PaperSpriteComponent.SetSprite` _returnvalue (`KismetArrayLibrary.Array_Random` (`self.Sprites`))))
          (:`0`
            (`PaperSpriteComponent.SetSpriteColor` _returnvalue (struct :`R` 0.279514 :`G` 0.140829 :`B` 0.071335 :`A` 1.0))
            (`PaperSpriteComponent.SetSprite` _returnvalue "/Game/Audience/2D/Horse_Sprite.Horse_Sprite"))
          (:`1`
            (`PaperSpriteComponent.SetSpriteColor` _returnvalue (struct :`G` 1.0 :`B` 0.094799 :`A` 1.0))
            (`PaperSpriteComponent.SetSprite` _returnvalue "/Game/Audience/2D/Goose_Sprite.Goose_Sprite")))
        (`SceneComponent.K2_AttachToComponent` _returnvalue (`self.MemberContainer`) "None" "KeepRelative" "KeepRelative" "KeepRelative" false)
        ; Positions sprites equally, starting from the middle going outwards, further each time. e.g. 5,3,1,2,4,6
        (bind _isa (`/Engine/EditorBlueprintResources/StandardMacros.FlipFlop`)
          (:`A`
            (`self.StartingPosition` _returnvalue _isa
              (:`then`
                (`SceneComponent.K2_SetRelativeLocationAndRotation` _returnvalue (`KismetMathLibrary.MakeVector` _spacing_accumulator) (`KismetMathLibrary.MakeRotator` 0.0 0.0 _outitem) false false))))
          (:`B`
            (`self.StartingPosition` _returnvalue _isa
              (:`then`
                (`SceneComponent.K2_SetRelativeLocationAndRotation` _returnvalue (`KismetMathLibrary.MakeVector` (* _spacing_accumulator -1.0)) (`KismetMathLibrary.MakeRotator` 0.0 0.0 _outitem) false false)
                (set `self.Spacing Accumulator` (+ (`self.Spacing Accumulator`) (`self.SpacingIncrement`)))))))
        ; Random chance to be deleted to create gaps (and saves on performance)
        (if (`KismetMathLibrary.RandomBoolWithWeight` (/ (`self.GapProbablity`) 100.0))
          (`BlueprintMapLibrary.Map_Remove` (`self.MemberList`) _returnvalue)
          (`ActorComponent.K2_DestroyComponent` _returnvalue)
          (else
            (`KismetArrayLibrary.Array_Add` (`self.OriginalPosition`) (`SceneComponent.RelativeLocation` _returnvalue))))))))

(event `self.ReceiveTick`
  (params (DeltaSeconds :type "Float (single-precision)"))
  (`/Engine/EditorBlueprintResources/StandardMacros.Gate` true :!label _label
    (:`Exit`
      (`KismetSystemLibrary.Delay` (`self.AnimStepInc`))
      (bind _keys (`BlueprintMapLibrary.Map_Keys` (`self.MemberList`)))
      (for _array_element _keys
        (if (`PrimitiveComponent.WasRecentlyRendered` _array_element 0.2)
          (bind _newtrans (`self.AnimateSprite` _array_element))
          (`SceneComponent.K2_SetRelativeTransform` _array_element _newtrans false false)))
      (set `self.AnimStepAccum` (+ (`self.AnimStepAccum`) (`self.AnimStepInc`))))))

(event `ToggleAnimations`
  (params (`Animate?` :type Boolean))
  (if `Animate?`
    (goto _label :!via `Open`)
    (else
      (goto _label :!via `Close`))))

(event `RegenerateAudience`
  (params (`Gap%` :type "Float (double-precision)" :default 33.0))
  (bind _memberlist (`self.MemberList`))
  (set `self.GapProbablity` `Gap%`)
  (bind _keys (`BlueprintMapLibrary.Map_Keys` _memberlist))
  (`ActorComponent.K2_DestroyComponent` _keys)
  (`BlueprintMapLibrary.Map_Clear` _memberlist)
  (`KismetArrayLibrary.Array_Clear` (`self.OriginalPosition`))
  (set `self.LoopIndex` 0)
  (set `self.Spacing Accumulator` 500.0)
  (set `self.AnimStepAccum` 0.0)
  (`self.RegenAudience`))

(event `AudienceCheer`
  (params (`Cheer Duration` :type "Float (double-precision)"))
  (set `self.OriginalAccum` (`self.AnimStepAccum`))
  (set `self.AnimCurve` "/Game/Audience/FC_AudienceCheer.FC_AudienceCheer")
  (`KismetSystemLibrary.Delay` `Cheer Duration`)
  (bind _keys (`BlueprintMapLibrary.Map_Keys` (`self.MemberList`)))
  (set `self.AnimStepAccum` (`self.OriginalAccum`))
  (for (_array_element _array_index) _keys
    (`SceneComponent.K2_SetRelativeLocation` _array_element (`|GetArrayItem` (`self.OriginalPosition`) _array_index) false false))
  (set `self.AnimCurve` "/Game/Audience/FC_AudienceFloatAnim.FC_AudienceFloatAnim"))

(fn `AnimateSprite`
  (params (Sprite :type "PaperSpriteComponent Object Reference"))
  (returns (NewTrans :type "Transform Structure"))
  (bind (_minvalue _maxvalue) (`CurveBase.GetValueRange` (`self.AnimCurve`)))
  (bind _new_rotator (`self.RandomFlipAnim` Sprite))
  (return (`KismetMathLibrary.MakeTransform` (+ (`SceneComponent.RelativeLocation` Sprite) (`KismetMathLibrary.MakeVector` 0.0 0.0 (`KismetMathLibrary.FClamp` (`CurveFloat.GetFloatValue` (`self.AnimCurve`) (+ (`BlueprintMapLibrary.Map_Find` (`self.MemberList`) Sprite) (`self.AnimStepAccum`))) _minvalue _maxvalue))) (`KismetMathLibrary.MakeRotator` 0.0 0.0 _new_rotator))))

(fn `RandomFlipAnim`
  (params (Sprite :type "PaperSpriteComponent Object Reference"))
  (returns (`New Rotator` :type "Float (double-precision)"))
  (bind (_relativerotation_roll _relativerotation_pitch _relativerotation_yaw) (`KismetMathLibrary.BreakRotator` (`SceneComponent.RelativeRotation` Sprite)))
  (switch `int` (`KismetMathLibrary.RandomInteger` 600)
    (:`Default`
      (return _relativerotation_yaw))
    (:`0`
      (if (== _relativerotation_yaw 180.0)
        (return 0.0)
        (else
          (return 180.0))))))

(fn `UserConstructionScript`
  (bind _audiencepopulation (`self.AudiencePopulation`))
  (bind _editorspaceaccum (`self.EditorSpaceAccum`))
  (set `self.StartingSpacing` (/ (`self.SpacingIncrement`) 2.0))
  (set `self.EditorSpaceInc` (`self.SpacingIncrement`))
  (if (> _audiencepopulation 2)
    (for _ (range (+ (`KismetMathLibrary.Round` (/ _audiencepopulation 2)) 1))
      (set `self.EditorSpaceAccum` (+ (`self.EditorSpaceAccum`) (`self.EditorSpaceInc`))))
    (`SceneComponent.K2_SetRelativeLocation` (`self.EditorStandIn`) (`KismetMathLibrary.MakeVector` _editorspaceaccum) false false)
    (`SceneComponent.K2_SetRelativeLocation` (`self.EditorStandIn1`) (`KismetMathLibrary.MakeVector` (* _editorspaceaccum -1.0)) false false)))