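; BP_AudienceCluster builds a row of 2D audience members from flipbook sprites.
; On BeginPlay it creates a Paper Flipbook component per population count under MemberContainer, all using the audience members flipbook.
; A FlipFlop places them alternately either side of the container's origin, widening by the spacing cached in the construction script.
; It then stops playback and sets a random frame, so the flipbook serves as still poses.
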(event `self.ReceiveBeginPlay`
  (bind _spacing_increment (`self.Spacing Increment`))
  (bind _memberlist (`self.MemberList`))
  (for _ (range (+ (`self.AudiencePopulation`) 1))
    (bind _returnvalue (`AddComponent|NODE_AddPaperFlipbookComponent-4` :`bManualAttachment` true))
    (`KismetArrayLibrary.Array_Add` (`self.MemberList`) _returnvalue)
    (`PaperFlipbookComponent.SetFlipbook` _returnvalue "/Game/Audience/2D/SFB_AudienceMembers.SFB_AudienceMembers")
    (`SceneComponent.SetMobility` _returnvalue "Movable")
    (`SceneComponent.K2_AttachToComponent` _returnvalue (`self.MemberContainer`) "None" "KeepRelative" "KeepRelative" "KeepRelative" false)
    (`/Engine/EditorBlueprintResources/StandardMacros.FlipFlop`
      (:`A`
        (`SceneComponent.K2_SetRelativeLocation` _returnvalue (`KismetMathLibrary.MakeVector` _spacing_increment) false false))
      (:`B`
        (`SceneComponent.K2_SetRelativeLocation` _returnvalue (`KismetMathLibrary.MakeVector` (* _spacing_increment -1.0)) false false)
        (set `self.Spacing Increment` (+ (`self.Spacing Increment`) (`self.StartingSpacing`))))))
  (`PaperFlipbookComponent.Stop` _memberlist)
  (`PaperFlipbookComponent.SetPlaybackPositionInFrames` (`self.MemberList`) (`KismetMathLibrary.RandomInteger` (`PaperFlipbookComponent.GetFlipbookLengthInFrames` (`|GetArrayItem` _memberlist))) false))

(event `self.ReceiveTick`
  (params (DeltaSeconds :type "Float (single-precision)")))

(fn `UserConstructionScript`
  (set `self.StartingSpacing` (`self.Spacing Increment`)))