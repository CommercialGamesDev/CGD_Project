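; Component that gives its owner a randomly tinted 2D audience member sprite and animates it moving vertically.
; On BeginPlay it adds a shadowless, collision-free Paper sprite from a random pool, with rare horse and goose variants in fixed colours.
; After a random delay to desynchronise members, a Tick-fed gate adds curve-sampled Z offsets at stepped intervals.
; StartAnimation and StopAnimation toggle the gate; CheerAnimation is an empty stub.
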(event `self.ReceiveBeginPlay`
  (set `self.Owner` (`self.GetOwner`))
  (`|ExecutionSequence`
    (:`then_0`
      (bind _returnvalue (`|AddComponentByClass` :`self` (`self.Owner`) :`Class` "/Script/Paper2D.PaperSpriteComponent"))
      (`PaperSpriteComponent.SetSpriteColor` _returnvalue (`KismetArrayLibrary.Array_Random` (`self.RandomColour`)))
      (`PrimitiveComponent.SetCollisionEnabled` _returnvalue "NoCollision")
      (`PrimitiveComponent.SetCastShadow` _returnvalue false)
      (switch `int` (`KismetMathLibrary.RandomInteger` 99)
        (:`Default`
          (`PaperSpriteComponent.SetSprite` _returnvalue (`KismetArrayLibrary.Array_Random` (`self.Sprites`))))
        (:`0`
          (`PaperSpriteComponent.SetSpriteColor` _returnvalue (struct :`R` 0.279514 :`G` 0.140829 :`B` 0.071335 :`A` 1.0))
          (`PaperSpriteComponent.SetSprite` _returnvalue "/Game/Audience/2D/Horse_Sprite.Horse_Sprite"))
        (:`1`
          (`PaperSpriteComponent.SetSpriteColor` _returnvalue (struct :`G` 1.0 :`B` 0.094799 :`A` 1.0))
          (`PaperSpriteComponent.SetSprite` _returnvalue "/Game/Audience/2D/Goose_Sprite.Goose_Sprite"))))
    (:`then_1`
      (`KismetSystemLibrary.Delay` (`KismetMathLibrary.RandomFloat`))
      (goto _label :!via `Open`))))

(event `CheerAnimation`)

(event `self.ReceiveTick`
  (params (DeltaSeconds :type "Float (single-precision)"))
  (`/Engine/EditorBlueprintResources/StandardMacros.Gate` true :!label _label
    (:`Exit`
      (`KismetSystemLibrary.Delay` (`self.AnimStepInc`))
      (`SceneComponent.K2_AddLocalOffset` (stale `self.ReceiveBeginPlay` _returnvalue) (`KismetMathLibrary.MakeVector` 0.0 0.0 (`CurveFloat.GetFloatValue` (`self.AnimCurve`) (`self.AnimStepAccum`))) false false)
      (set `self.AnimStepAccum` (+ (`self.AnimStepAccum`) (`self.AnimStepInc`))))))

(event `StartAnimation`
  (goto _label :!via `Open`))

(event `StopAnimation`
  (goto _label :!via `Close`))