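; BP_AxeBaseClass is a base class for rotating axe obstacles, with either continuous spinning or timeline-driven motion chosen by FullyRotate.
; On BeginPlay, full rotation sets the RotatingMovement rate from RotationSpeed.
; Otherwise RotationSpeed becomes the Timeline play rate, and the track value is added to StartRotation to drive the actor's pitch.
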(event `self.ReceiveBeginPlay`
  (if (`self.Fully Rotate?`)
    (set `RotatingMovementComponent.RotationRate` (`KismetMathLibrary.MakeRotator` 0.0 (* (`self.RotationSpeed`) 180.0)) (`self.RotatingMovement`))
    (else
      (`TimelineComponent.SetPlayRate` (`self.Timeline`) (`self.RotationSpeed`))
      (`self.RotateAxeToEnd`))))

(event `RotateAxeToEnd`
  (bind (_direction _newtrack_2) (`Timeline|Timeline` :!via `PlayFromStart`)
    (:`Update`
      (`self.K2_SetActorRotation` (`KismetMathLibrary.MakeRotator` 0.0 (+ (`self.StartRotation`) _newtrack_2))))))

(fn `UserConstructionScript`)