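; Spinner obstacle with a configurable number, length, colour, speed and direction of arms rotating around a central core.
; The construction script builds evenly spaced static mesh body and end pieces as a preview of the arms, and colours them and the core.
; BeginPlay swaps that preview for spawned BP_SpinnerArm actors, which Tick yaws individually at a frame-rate-independent speed.
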(event `self.ReceiveBeginPlay`
  (bind _arm_colour (`self.Arm_Colour`))
  (bind _speed_of_arms (`self.Speed_Of_Arms`))
  ; While there still aren't enough arms in the array
  (for _array_element (`self.Display_Bodys`)
    (`ActorComponent.K2_DestroyComponent` _array_element))
  (for _array_element_2 (`self.Display_Ends`)
    (`ActorComponent.K2_DestroyComponent` _array_element_2))
  (while (!= (`KismetArrayLibrary.Array_Length` (`self.Arms`)) (`self.Number_Of_Arms`))
    ; Set each arm's position and scale to that of the core
    (bind _returnvalue (`|SpawnActorFromClass` "/Game/obstacles/Spinner/BP_SpinnerArm.BP_SpinnerArm_C" (`SceneComponent.K2_GetComponentToWorld` (`self.Core`)) "Undefined" "MultiplyWithRoot" null null))
    (`/Game/obstacles/Spinner/BP_SpinnerArm.SetLength` _returnvalue (`self.Length_Of_Arms`))
    ; Rotate each arm to be around the core
    (`SceneComponent.K2_AddLocalRotation` (`Actor.RootComponent` _returnvalue) (`KismetMathLibrary.MakeRotator` 0.0 0.0 (* (`KismetArrayLibrary.Array_Length` (`self.Arms`)) (/ 360 (`self.Number_Of_Arms`)))) false false)
    ; Add each arm to the array of arms
    (`KismetArrayLibrary.Array_Add` (`self.Arms`) _returnvalue))
  ; Reverse Direction
  (set `self.Speed_Of_Arms` (`KismetMathLibrary.SelectFloat` (* -1.0 _speed_of_arms) _speed_of_arms (`self.Anti-Clockwise`)))
  (for _array_element_3 (`self.Arms`)
    (`|ExecutionSequence`
      (:`then_0`
        (`MeshComponent.SetColorParameterValueOnMaterials` (`/Game/obstacles/Spinner/BP_SpinnerArm.Body` _array_element_3) "Colour" _arm_colour))
      (:`then_1`
        (`MeshComponent.SetColorParameterValueOnMaterials` (`/Game/obstacles/Spinner/BP_SpinnerArm.End` _array_element_3) "Colour" _arm_colour)))))

(event `self.ReceiveTick`
  (params (DeltaSeconds :type "Float (single-precision)"))
  ; Spin
  (for _array_element (`self.Arms`)
    (`/Engine/EditorBlueprintResources/StandardMacros.IsValid` _array_element
      (:`Is Valid`
        (`SceneComponent.K2_AddLocalRotation` (`Actor.RootComponent` _array_element) (`KismetMathLibrary.MakeRotator` 0.0 0.0 (* DeltaSeconds (`self.Speed_Of_Arms`))) false false)))))

(fn `UserConstructionScript`
  (bind (_returnvalue_x _returnvalue_y _returnvalue_z) (`KismetMathLibrary.BreakVector` (`SceneComponent.K2_GetComponentScale` (`self.Core`))))
  ; While there still aren't enough arms in the array
  (while (!= (`KismetArrayLibrary.Array_Length` (`self.Display_Bodys`)) (`self.Number_Of_Arms`))
    ; Set each arm's position and scale to that of the core
    (bind _returnvalue (`AddComponent|NODE_AddStaticMeshComponent-0` :`bManualAttachment` true))
    (`StaticMeshComponent.SetStaticMesh` _returnvalue "/Game/obstacles/Spinner/SM_SpinnerArmCore.SM_SpinnerArmCore")
    (`SceneComponent.K2_AttachToComponent` _returnvalue (`self.Core`) "None" "KeepRelative" "KeepRelative" "KeepRelative" false)
    (`SceneComponent.SetWorldScale3D` _returnvalue (`KismetMathLibrary.MakeVector` (* (`self.Length_Of_Arms`) _returnvalue_x) _returnvalue_y _returnvalue_z))
    (bind _returnvalue_2 (`AddComponent|NODE_AddStaticMeshComponent-2` :`bManualAttachment` true))
    (`StaticMeshComponent.SetStaticMesh` _returnvalue_2 "/Game/obstacles/Spinner/SM_SpinnerArmEnd.SM_SpinnerArmEnd")
    (`SceneComponent.K2_AttachToComponent` _returnvalue_2 _returnvalue "None" "KeepRelative" "KeepRelative" "KeepRelative" false)
    (`SceneComponent.SetWorldScale3D` _returnvalue_2 (`SceneComponent.K2_GetComponentScale` (`self.Core`)))
    (bind (_min _max) (`StaticMeshComponent.GetLocalBounds` _returnvalue))
    (bind _returnvalue_x_2 (`KismetMathLibrary.BreakVector` (+ _min _max)))
    (`SceneComponent.K2_SetRelativeLocation` _returnvalue_2 (`KismetMathLibrary.MakeVector` _returnvalue_x_2) false false)
    ; Rotate each arm to be around the core
    (`KismetArrayLibrary.Array_Add` (`self.Display_Ends`) _returnvalue_2)
    (`SceneComponent.K2_AddLocalRotation` _returnvalue (`KismetMathLibrary.MakeRotator` 0.0 0.0 (* (`KismetArrayLibrary.Array_Length` (`self.Display_Bodys`)) (/ 360 (`self.Number_Of_Arms`)))) false false)
    (`KismetArrayLibrary.Array_Add` (`self.Display_Bodys`) _returnvalue))
  (`MeshComponent.SetColorParameterValueOnMaterials` (`self.Core`) "Colour" (`self.Core_Colour`))
  (for _index (range (`self.Number_Of_Arms`))
    (`MeshComponent.SetColorParameterValueOnMaterials` (`|GetArrayItem` (`self.Display_Bodys`) _index) "Colour" (`self.Arm_Colour`))
    (`MeshComponent.SetColorParameterValueOnMaterials` (`|GetArrayItem` (`self.Display_Ends`) _index) "Colour" (`self.Arm_Colour`))))