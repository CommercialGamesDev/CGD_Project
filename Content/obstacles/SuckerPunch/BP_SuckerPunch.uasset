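; Sucker Punch obstacle whose arm slides out of and back into a body along local X in an endless loop from BeginPlay.
; Chained events extend, hold, retract and hold, optionally randomising each timing per cycle.
; Travel derives from mesh bounds and ArmLength, with DoubleSided changing the retract target.
; The construction script stretches the arm by ArmLength, counter-scales both end pieces and applies body and arm colours.
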(event `Stay_Extended`
  ;[0 0.5 0 0.5] Stay Extended
  (`KismetSystemLibrary.Delay` (`self.Time_Stay_Extended`))
  (`self.Retract`))

(event `self.ReceiveBeginPlay`
  ;[0.25 0.25 0.25 0.5] Begin Play
  (`self.Randomise_Timings`))

(event `Stay_Retracted`
  ;[0.5 0 0 0.5] Stay Retracted
  (`KismetSystemLibrary.Delay` (`self.Time_Stay_Retracted`))
  (`self.Randomise_Timings`))

(event `Randomise_Timings`
  ;[1 0 1 0.5] Randomise Timings
  (`|ExecutionSequence`
    (:`then_0`
      (if (`self.Random_Time_To_Extend`)
        (set `self.Time_To_Extend` (`KismetMathLibrary.RandomFloatInRange` 0.25 2.5))))
    (:`then_1`
      (if (`self.Random_Time_To_Retract`)
        (set `self.Time_To_Retract` (`KismetMathLibrary.RandomFloatInRange` 0.25 2.5))))
    (:`then_2`
      (if (`self.Random_Time_Stay_Extended`)
        (set `self.Time_Stay_Extended` (`KismetMathLibrary.RandomFloatInRange` 1.0 3.0))))
    (:`then_3`
      (if (`self.Random_Time_Stay_Retracted`)
        (set `self.Time_Stay_Retracted` (`KismetMathLibrary.RandomFloatInRange` 1.0 3.0))))
    (:`then_4`
      (`self.Extend`))))

(event `Extend`
  (bind (_min _max) (`StaticMeshComponent.GetLocalBounds` (`self.Body`)))
  (bind (_relativelocation_x _relativelocation_y _relativelocation_z) (`KismetMathLibrary.BreakVector` (`SceneComponent.RelativeLocation` (`self.Arm_Core`))))
  (bind _returnvalue_x (`KismetMathLibrary.BreakVector` (/ (+ (`KismetMathLibrary.Vector_GetAbs` _min) (`KismetMathLibrary.Vector_GetAbs` _max)) 2.0)))
  ;[0 1 0 0.5] Extend
  (`KismetSystemLibrary.MoveComponentTo` (`self.Arm_Core`) (`KismetMathLibrary.MakeVector` _returnvalue_x _relativelocation_y _relativelocation_z) (struct) false false (`self.Time_To_Extend`))
  (`self.Stay_Extended`))

(event `Retract`
  (bind (_min _max) (`StaticMeshComponent.GetLocalBounds` (`self.Arm_Front_End`)))
  (bind (_min_2 _max_2) (`StaticMeshComponent.GetLocalBounds` (`self.Arm_Core`)))
  (bind (_min_3 _max_3) (`StaticMeshComponent.GetLocalBounds` (`self.Arm_Front_End`)))
  (bind (_min_4 _max_4) (`StaticMeshComponent.GetLocalBounds` (`self.Body`)))
  (bind (_min_5 _max_5) (`StaticMeshComponent.GetLocalBounds` (`self.Arm_Core`)))
  (bind (_min_6 _max_6) (`StaticMeshComponent.GetLocalBounds` (`self.Arm_Back_End`)))
  (bind (_min_7 _max_7) (`StaticMeshComponent.GetLocalBounds` (`self.Body`)))
  (bind (_relativelocation_x _relativelocation_y _relativelocation_z) (`KismetMathLibrary.BreakVector` (`SceneComponent.RelativeLocation` (`self.Arm_Core`))))
  (bind (_relativelocation_x_2 _relativelocation_y_2 _relativelocation_z_2) (`KismetMathLibrary.BreakVector` (`SceneComponent.RelativeLocation` (`self.Arm_Core`))))
  (bind (_returnvalue_x _returnvalue_y _returnvalue_z) (`KismetMathLibrary.BreakVector` (+ (`KismetMathLibrary.Vector_GetAbs` _min_2) (`KismetMathLibrary.Vector_GetAbs` _max_2))))
  (bind (_returnvalue_x_2 _returnvalue_y_2 _returnvalue_z_2) (`KismetMathLibrary.BreakVector` (+ (`KismetMathLibrary.Vector_GetAbs` _min_5) (`KismetMathLibrary.Vector_GetAbs` _max_5))))
  (bind _returnvalue_x_3 (`KismetMathLibrary.BreakVector` (* (+ (`KismetMathLibrary.MakeVector` (* (`self.Arm_Length`) _returnvalue_x) _returnvalue_y _returnvalue_z) (+ (`KismetMathLibrary.Vector_GetAbs` _min_3) (`KismetMathLibrary.Vector_GetAbs` _max_3)) (/ (+ (`KismetMathLibrary.Vector_GetAbs` _min_4) (`KismetMathLibrary.Vector_GetAbs` _max_4)) -2.0)) -1.0)))
  (bind _returnvalue_x_4 (`KismetMathLibrary.BreakVector` (* (+ (`KismetMathLibrary.MakeVector` (* (`self.Arm_Length`) _returnvalue_x_2) _returnvalue_y_2 _returnvalue_z_2) (+ (`KismetMathLibrary.Vector_GetAbs` _min) (`KismetMathLibrary.Vector_GetAbs` _max)) (* (+ (`KismetMathLibrary.Vector_GetAbs` _min_6) (`KismetMathLibrary.Vector_GetAbs` _max_6)) -1.0) (/ (+ (`KismetMathLibrary.Vector_GetAbs` _min_7) (`KismetMathLibrary.Vector_GetAbs` _max_7)) 2.0)) -1.0)))
  ;[1 0 0 0.5] Retract
  (if (`self.Double_Sided`)
    (`KismetSystemLibrary.MoveComponentTo` (`self.Arm_Core`) (`KismetMathLibrary.MakeVector` _returnvalue_x_4 _relativelocation_y_2 _relativelocation_z_2) (struct) false false (`self.Time_To_Retract`))
    (`self.Stay_Retracted`)
    (else
      (`KismetSystemLibrary.MoveComponentTo` (`self.Arm_Core`) (`KismetMathLibrary.MakeVector` _returnvalue_x_3 _relativelocation_y _relativelocation_z) (struct) false false (`self.Time_To_Retract`))
      (`self.Stay_Retracted`))))

(fn `UserConstructionScript`
  (bind (_min _max) (`StaticMeshComponent.GetLocalBounds` (`self.Body`)))
  (bind (_min_2 _max_2) (`StaticMeshComponent.GetLocalBounds` (`self.Arm_Core`)))
  (bind (_min_3 _max_3) (`StaticMeshComponent.GetLocalBounds` (`self.Arm_Core`)))
  (bind (_min_4 _max_4) (`StaticMeshComponent.GetLocalBounds` (`self.Arm_Back_End`)))
  (bind _returnvalue_x (`KismetMathLibrary.BreakVector` (+ _min_2 _max_2)))
  (bind _returnvalue_x_2 (`KismetMathLibrary.BreakVector` (+ (`KismetMathLibrary.Vector_GetAbs` _min_4) (`KismetMathLibrary.Vector_GetAbs` _max_4))))
  (bind _returnvalue_x_3 (`KismetMathLibrary.BreakVector` (+ (`KismetMathLibrary.Vector_GetAbs` _min_3) (`KismetMathLibrary.Vector_GetAbs` _max_3))))
  (bind (_returnvalue_x_4 _returnvalue_y _returnvalue_z) (`KismetMathLibrary.BreakVector` (/ (+ (`KismetMathLibrary.Vector_GetAbs` _min) (`KismetMathLibrary.Vector_GetAbs` _max)) 2.0)))
  (`SceneComponent.K2_SetRelativeLocation` (`self.Arm_Core`) (`KismetMathLibrary.MakeVector` (+ (- (* _returnvalue_x_4 -1.0) (* _returnvalue_x_3 (- (`self.Arm_Length`) 1.0))) _returnvalue_x_2) 0.0 _returnvalue_z) false false)
  (`SceneComponent.SetRelativeScale3D` (`self.Arm_Core`) (`KismetMathLibrary.MakeVector` (`self.Arm_Length`) 1.0 1.0))
  (`SceneComponent.SetRelativeScale3D` (`self.Arm_Back_End`) (`KismetMathLibrary.MakeVector` (/ 1.0 (`self.Arm_Length`)) 1.0 1.0))
  (`SceneComponent.SetRelativeScale3D` (`self.Arm_Front_End`) (`KismetMathLibrary.MakeVector` (/ 1.0 (`self.Arm_Length`)) 1.0 1.0))
  (`SceneComponent.K2_SetRelativeLocation` (`self.Arm_Front_End`) (`KismetMathLibrary.MakeVector` _returnvalue_x) false false)
  (`MeshComponent.SetColorParameterValueOnMaterials` (`self.Body`) "Colour" (`self.Core_Colour`))
  (`MeshComponent.SetColorParameterValueOnMaterials` (`self.Arm_Core`) "Colour" (`self.Arm_Colour`))
  (`MeshComponent.SetColorParameterValueOnMaterials` (`self.Arm_Front_End`) "Colour" (`self.Arm_Colour`))
  (`MeshComponent.SetColorParameterValueOnMaterials` (`self.Arm_Back_End`) "Colour" (`self.Arm_Colour`)))