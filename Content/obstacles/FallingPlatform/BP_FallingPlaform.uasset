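; Balloon-held platform obstacle that sinks when an actor tagged Player overlaps its box, then drops and respawns.
; A timeline lowers it by HeightDrop over FallingTime before BurstBalloon hides the balloon, plays a random pop and runs a free-fall timeline.
; It then hides the rope and platform, waits RespawnTime, and resets position and visibility.
; The construction script applies size, part colours and balloon visibility.
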(event `self.ReceiveBeginPlay`
  (set `self.StartLocation` (`SceneComponent.K2_GetComponentLocation` (`self.DefaultSceneRoot`))))

(event `self.Box.OnComponentBeginOverlap`
  (params (OverlappedComponent :type "PrimitiveComponent Object Reference") (OtherActor :type "Actor Object Reference") (OtherComp :type "PrimitiveComponent Object Reference") (OtherBodyIndex :type Integer) (bFromSweep :type Boolean) (SweepResult :type "HitResult Structure (by ref)"))
  (bind (_startlocation_x _startlocation_y _startlocation_z) (`KismetMathLibrary.BreakVector` (`self.StartLocation`)))
  (if (and (`SceneComponent.bVisible` (`self.Platform`)) (`self.ActorHasTag` OtherActor "Player") (not (`self.isFalling`)))
    (`TimelineComponent.SetPlayRate` (`self.Falling`) (/ 1.0 (`self.FallingTime`)))
    (set `self.isFalling` true)
    (bind (_direction _falltrack) (`Timeline|Falling` :!via `PlayFromStart`)
      (:`Update`
        (`SceneComponent.K2_SetWorldLocation` (`self.DefaultSceneRoot`) (`KismetMathLibrary.MakeVector` _startlocation_x _startlocation_y (- _startlocation_z (* _falltrack (`self.HeightDrop`)))) false false))
      (:`Finished`
        (`self.BurstBalloon`)))))

(event `BurstBalloon`
  (bind (_startlocation_x _startlocation_y _startlocation_z) (`KismetMathLibrary.BreakVector` (`self.StartLocation`)))
  (`SceneComponent.SetVisibility` (`self.BalloonHandle`) false false)
  (`SceneComponent.SetVisibility` (`self.Balloon`) false false)
  (`GameplayStatics.PlaySound2D` (`KismetArrayLibrary.Array_Random` (`self.PopSounds`)) 1.0 1.0 0.0 null null)
  (bind (_direction _freefall) (`Timeline|PlatformFreeFall` :!via `PlayFromStart`)
    (:`Update`
      (`SceneComponent.K2_SetWorldLocation` (`self.DefaultSceneRoot`) (`KismetMathLibrary.MakeVector` _startlocation_x _startlocation_y (- _startlocation_z _freefall (`self.HeightDrop`))) false false))
    (:`Finished`
      (`SceneComponent.SetVisibility` (`self.Rope`) false false)
      (`SceneComponent.SetVisibility` (`self.Platform`) false false)
      (`KismetSystemLibrary.Delay` (`self.RespawnTime`))
      (`self.RespawnPlatform`))))

(event `RespawnPlatform`
  (`SceneComponent.K2_SetWorldLocation` (`self.DefaultSceneRoot`) (`self.StartLocation`) false false)
  (`SceneComponent.SetVisibility` (`self.BalloonHandle`) false false)
  (`SceneComponent.SetVisibility` (`self.Balloon`) true false)
  (`SceneComponent.SetVisibility` (`self.Rope`) true false)
  (`SceneComponent.SetVisibility` (`self.Platform`) true false)
  (set `self.isFalling` false))

(fn `UserConstructionScript`
  (`SceneComponent.SetRelativeScale3D` (`self.Platforms`) (`KismetMathLibrary.MakeVector` (`self.SizeX`) (`self.SizeY`) 1.0))
  (`MeshComponent.SetColorParameterValueOnMaterials` (`self.Balloon`) "Colour" (`self.Balloon_Colour`))
  (`MeshComponent.SetColorParameterValueOnMaterials` (`self.Rope`) "Colour" (`self.Rope_Colour`))
  (`MeshComponent.SetColorParameterValueOnMaterials` (`self.Platform`) "Colour" (`self.Platform_Colour`))
  (`SceneComponent.SetVisibility` (`self.Balloon`) (`self.ShowBalloon`) true))