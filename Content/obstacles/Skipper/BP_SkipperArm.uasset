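; BP_SkipperArm is the arm-and-rope piece of the Skipper obstacle, sized through its SetLength function.
; SetLength multiplies the Arm's Z scale by ArmLength and sets the Rope's X scale from RopeLength and the Arm's base scale.
; It then shifts the Rope along local Z using the Arm's bounds, less a scale-compensated margin.
; Both Arm scaling and Rope offset are relative, so repeated calls accumulate.
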(fn `SetLength`
  (params (Arm_Length :type "Float (double-precision)") (Rope_Length :type "Float (double-precision)"))
  (locals (Core_Scale :type "Vector Structure"))
  (bind (_core_scale_x _core_scale_y _core_scale_z) (`KismetMathLibrary.BreakVector` (`local.Core_Scale`)))
  (bind (_min _max) (`StaticMeshComponent.GetLocalBounds` (`self.Arm`)))
  (bind (_returnvalue_x _returnvalue_y _returnvalue_z) (`KismetMathLibrary.BreakVector` (`SceneComponent.K2_GetComponentScale` (`self.Arm`))))
  (bind (_returnvalue_x_2 _returnvalue_y_2 _returnvalue_z_2) (`KismetMathLibrary.BreakVector` (`SceneComponent.K2_GetComponentScale` (`self.Arm`))))
  (bind (_returnvalue_x_3 _returnvalue_y_3 _returnvalue_z_3) (`KismetMathLibrary.BreakVector` (+ _min _max)))
  ; Arm Scale/Length
  (bind _output_get (set `local.Core_Scale` (`KismetMathLibrary.MakeVector` _returnvalue_x_2 _returnvalue_y_2 _returnvalue_z_2)))
  (`SceneComponent.SetWorldScale3D` (`self.Arm`) (`KismetMathLibrary.MakeVector` (.x _output_get) (.y _output_get) (* _returnvalue_z_2 Arm_Length)))
  ; Rope Scale/Length
  (`SceneComponent.SetWorldScale3D` (`self.Rope`) (`KismetMathLibrary.MakeVector` (* Rope_Length _core_scale_x) _core_scale_y _core_scale_z))
  ; Rope Location
  (`SceneComponent.K2_AddLocalOffset` (`self.Rope`) (`KismetMathLibrary.MakeVector` 0.0 0.0 (- _returnvalue_z_3 (* (/ _core_scale_z _returnvalue_z) 25.0))) false false))

(fn `UserConstructionScript`)