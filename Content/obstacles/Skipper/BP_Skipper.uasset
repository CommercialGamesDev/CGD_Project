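; Skipper obstacle: a core ringed by evenly spaced arms with ropes that spin around its roll axis.
; The construction script builds preview arm and rope meshes scaled by the length settings, then tints them and the core.
; BeginPlay destroys the preview, spawns BP_SkipperArm actors at the core with those lengths, and negates speed if anticlockwise.
; Tick rotates each spawned arm by speed and delta time.
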(event `self.ReceiveBeginPlay`
  ; While there still aren't enough arms in the array
  (for _array_element (`self.Display_Rope_Ends`)
    (`ActorComponent.K2_DestroyComponent` _array_element))
  (for _array_element_2 (`self.Display_Rope_Cores`)
    (`ActorComponent.K2_DestroyComponent` _array_element_2))
  (for _array_element_3 (`self.Display_Arm_Ends`)
    (`ActorComponent.K2_DestroyComponent` _array_element_3))
  (for _array_element_4 (`self.Display_Arm_Cores`)
    (`ActorComponent.K2_DestroyComponent` _array_element_4))
  (while (!= (`KismetArrayLibrary.Array_Length` (`self.Arms`)) (`self.Number_Of_Arms`))
    ; Set each arm's position and scale to that of the core
    (bind _returnvalue (`|SpawnActorFromClass` "/Game/obstacles/Skipper/BP_SkipperArm.BP_SkipperArm_C" (`SceneComponent.K2_GetComponentToWorld` (`self.Core`)) "Undefined" "MultiplyWithRoot" null null))
    (`/Game/obstacles/Skipper/BP_SkipperArm.SetLength` _returnvalue (`self.Length_Of_Arms`) (`self.Length_Of_Ropes`))
    ; Rotate each arm to be around the core
    (`SceneComponent.K2_AddLocalRotation` (`Actor.RootComponent` _returnvalue) (`KismetMathLibrary.MakeRotator` (* (`KismetArrayLibrary.Array_Length` (`self.Arms`)) (/ 360 (`self.Number_Of_Arms`)))) false false)
    ; Add each arm to the array of arms
    (`KismetArrayLibrary.Array_Add` (`self.Arms`) _returnvalue))
  ; Reverse Direction
  (if (`self.Anti-Clockwise`)
    (set `self.Speed_Of_Arms` (* -1.0 (`self.Speed_Of_Arms`)))))

(event `self.ReceiveTick`
  (params (DeltaSeconds :type "Float (single-precision)"))
  ; Spin
  (for _array_element (`self.Arms`)
    (`SceneComponent.K2_AddLocalRotation` (`Actor.RootComponent` _array_element) (`KismetMathLibrary.MakeRotator` (* DeltaSeconds (`self.Speed_Of_Arms`))) false false)))

(fn `UserConstructionScript`
  (bind (_returnvalue_x _returnvalue_y _returnvalue_z) (`KismetMathLibrary.BreakVector` (`SceneComponent.K2_GetComponentScale` (`self.Core`))))
  (bind (_returnvalue_x_2 _returnvalue_y_2 _returnvalue_z_2) (`KismetMathLibrary.BreakVector` (`SceneComponent.K2_GetComponentScale` (`self.Core`))))
  ; While there still aren't enough arms in the array
  (while (!= (`KismetArrayLibrary.Array_Length` (`self.Display_Arm_Cores`)) (`self.Number_Of_Arms`))
    ; Set each arm's position and scale to that of the core
    (bind _returnvalue (`AddComponent|NODE_AddStaticMeshComponent-0` :`bManualAttachment` true))
    (`StaticMeshComponent.SetStaticMesh` _returnvalue "/Game/obstacles/Skipper/SM_SkipperArmCore.SM_SkipperArmCore")
    (`SceneComponent.K2_AttachToComponent` _returnvalue (`self.Core`) "None" "KeepRelative" "KeepRelative" "KeepRelative" false)
    (`SceneComponent.SetWorldScale3D` _returnvalue (`KismetMathLibrary.MakeVector` _returnvalue_x _returnvalue_y (* _returnvalue_z (`self.Length_Of_Arms`))))
    (bind _returnvalue_2 (`AddComponent|NODE_AddStaticMeshComponent-2` :`bManualAttachment` true))
    (`StaticMeshComponent.SetStaticMesh` _returnvalue_2 "/Game/obstacles/Skipper/SM_SkipperArmEnd.SM_SkipperArmEnd")
    (`SceneComponent.K2_AttachToComponent` _returnvalue_2 _returnvalue "None" "KeepRelative" "KeepRelative" "KeepRelative" false)
    (`SceneComponent.SetWorldScale3D` _returnvalue_2 (`SceneComponent.K2_GetComponentScale` (`self.Core`)))
    (bind (_min _max) (`StaticMeshComponent.GetLocalBounds` _returnvalue))
    (bind (_returnvalue_x_3 _returnvalue_y_3 _returnvalue_z_3) (`KismetMathLibrary.BreakVector` (+ _min _max)))
    (`SceneComponent.K2_AddLocalOffset` _returnvalue_2 (`KismetMathLibrary.MakeVector` 0.0 0.0 _returnvalue_z_3) false false)
    ; Rotate each arm to be around the core
    (bind _returnvalue_3 (`AddComponent|NODE_AddStaticMeshComponent-1` :`bManualAttachment` true))
    (`StaticMeshComponent.SetStaticMesh` _returnvalue_3 "/Game/obstacles/Skipper/SM_SkipperRopeCore.SM_SkipperRopeCore")
    (`SceneComponent.K2_AttachToComponent` _returnvalue_3 _returnvalue "None" "KeepRelative" "KeepRelative" "KeepRelative" false)
    (`SceneComponent.SetWorldScale3D` _returnvalue_3 (`KismetMathLibrary.MakeVector` (* (`self.Length_Of_Ropes`) _returnvalue_x_2) _returnvalue_y_2 _returnvalue_z_2))
    (bind (_min_2 _max_2) (`StaticMeshComponent.GetLocalBounds` _returnvalue))
    (bind (_returnvalue_x_4 _returnvalue_y_4 _returnvalue_z_4) (`KismetMathLibrary.BreakVector` (+ _min_2 _max_2)))
    (bind (_returnvalue_x_5 _returnvalue_y_5 _returnvalue_z_5) (`KismetMathLibrary.BreakVector` (`SceneComponent.K2_GetComponentScale` _returnvalue)))
    (`SceneComponent.K2_AddLocalOffset` _returnvalue_3 (`KismetMathLibrary.MakeVector` 0.0 0.0 (- _returnvalue_z_4 (* (/ _returnvalue_z_2 _returnvalue_z_5) 10.0))) false false)
    (bind _returnvalue_4 (`AddComponent|NODE_AddStaticMeshComponent-3` :`bManualAttachment` true))
    (`StaticMeshComponent.SetStaticMesh` _returnvalue_4 "/Game/obstacles/Skipper/SM_SkipperRopeEnd.SM_SkipperRopeEnd")
    (`SceneComponent.K2_AttachToComponent` _returnvalue_4 _returnvalue_3 "None" "KeepRelative" "KeepRelative" "KeepRelative" false)
    (`SceneComponent.SetWorldScale3D` _returnvalue_4 (`SceneComponent.K2_GetComponentScale` (`self.Core`)))
    (bind (_min_3 _max_3) (`StaticMeshComponent.GetLocalBounds` _returnvalue_3))
    (bind _returnvalue_x_6 (`KismetMathLibrary.BreakVector` (+ _min_3 _max_3)))
    (`SceneComponent.K2_AddLocalOffset` _returnvalue_4 (`KismetMathLibrary.MakeVector` _returnvalue_x_6) false false)
    (`SceneComponent.K2_AddLocalRotation` _returnvalue (`KismetMathLibrary.MakeRotator` (* (`KismetArrayLibrary.Array_Length` (`self.Display_Arm_Cores`)) (/ 360 (`self.Number_Of_Arms`)))) false false)
    (`KismetArrayLibrary.Array_Add` (`self.Display_Arm_Cores`) _returnvalue)
    (`KismetArrayLibrary.Array_Add` (`self.Display_Arm_Ends`) _returnvalue_2)
    (`KismetArrayLibrary.Array_Add` (`self.Display_Rope_Cores`) _returnvalue_3)
    (`KismetArrayLibrary.Array_Add` (`self.Display_Rope_Ends`) _returnvalue_4))
  (`|ExecutionSequence`
    (:`then_0`
      (for _index (range (`self.Number_Of_Arms`))
        (`MeshComponent.SetColorParameterValueOnMaterials` (`|GetArrayItem` (`self.Display_Arm_Cores`) _index) "Colour" (`self.Arm_Colour`))
        (`MeshComponent.SetColorParameterValueOnMaterials` (`|GetArrayItem` (`self.Display_Arm_Ends`) _index) "Colour" (`self.Arm_Colour`))
        (`MeshComponent.SetColorParameterValueOnMaterials` (`|GetArrayItem` (`self.Display_Rope_Cores`) _index) "Colour" (`self.Rope_Colour`))
        (`MeshComponent.SetColorParameterValueOnMaterials` (`|GetArrayItem` (`self.Display_Rope_Ends`) _index) "Colour" (`self.Rope_Colour`))))
    (:`then_1`
      (`MeshComponent.SetColorParameterValueOnMaterials` (`self.Core`) "Colour" (`self.Core_Colour`)))))