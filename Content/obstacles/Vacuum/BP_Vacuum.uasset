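; BP_Vacuum is a vacuum obstacle that moves overlapping actors tagged "Pushable" while it is active.
; Each tick it offsets actors inside its Box along the Arrow's forward vector, using a swept move scaled by VacuumPull and delta time rather than physics forces.
; The construction script sets the X scale of Collisions from VacuumRange and applies editable colours to the Base and Cone materials.
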(event `self.ReceiveTick`
  (params (DeltaSeconds :type "Float (single-precision)"))
  (if (`self.IsActive`)
    (for _array_element (`PrimitiveComponent.GetOverlappingActors` (`self.Box`) null)
      (if (`self.ActorHasTag` _array_element "Pushable")
        (`self.K2_AddActorWorldOffset` _array_element (* (`KismetMathLibrary.GetForwardVector` (`SceneComponent.K2_GetComponentRotation` (`self.Arrow`))) (* DeltaSeconds (`self.VacuumPull`))) true false)))))

(fn `UserConstructionScript`
  (bind (_returnvalue_x _returnvalue_y _returnvalue_z) (`KismetMathLibrary.BreakVector` (`SceneComponent.K2_GetComponentScale` (`self.Collisions`))))
  (`SceneComponent.SetWorldScale3D` (`self.Collisions`) (`KismetMathLibrary.MakeVector` (`self.VacuumRange`) _returnvalue_y _returnvalue_z))
  (`MeshComponent.SetColorParameterValueOnMaterials` (`self.Base`) "Colour" (`self.Base_Colour`))
  (`MeshComponent.SetColorParameterValueOnMaterials` (`self.Cone`) "Colour" (`self.Cone_Colour`)))