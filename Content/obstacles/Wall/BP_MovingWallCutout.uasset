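; Modular wall obstacle piece, configured entirely in the Construction Script, with no active event logic or movement in its graphs.
; With Cutout on, it scales the middle mesh along Y to MiddleLength using its bounds and snaps visible front and rear caps to the ends.
; Reversed swaps the caps and turns them around.
; With Cutout off, it hides the caps and shows the wall-hole mesh at actor scale.
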(fn `UserConstructionScript`
  (bind _sm_wallmiddle (`self.SM_WallMiddle`))
  (bind _cutout (`self.Cutout`))
  (bind _sm_wallmiddle_2 (`self.SM_WallMiddle`))
  (bind _reversed (`self.Reversed`))
  (bind (_min _max) (`StaticMeshComponent.GetLocalBounds` (`self.SM_WallMiddle`)))
  (bind (_min_2 _max_2) (`StaticMeshComponent.GetLocalBounds` _sm_wallmiddle))
  (bind _returnvalue (`self.GetActorScale3D` self))
  (bind _returnvalue_2 (`KismetMathLibrary.SelectFloat` 180.0 0.0 _reversed))
  (bind (_returnvalue_x _returnvalue_y) (`KismetMathLibrary.BreakVector` (`SceneComponent.K2_GetComponentScale` _sm_wallmiddle)))
  (bind (_returnvalue_x_2 _returnvalue_y_2) (`KismetMathLibrary.BreakVector` (* _max_2 _returnvalue_y)))
  (bind (_returnvalue_x_3 _returnvalue_y_3) (`KismetMathLibrary.BreakVector` (* _min_2 _returnvalue_y)))
  (bind (_returnvalue_x_4 _returnvalue_y_4) (`KismetMathLibrary.BreakVector` (+ _max _max)))
  (`SceneComponent.SetVisibility` (`self.SM_WallFront`) _cutout false)
  (`SceneComponent.SetVisibility` (`self.SM_WallRear`) _cutout false)
  (if (`self.Cutout`)
    (`StaticMeshComponent.SetStaticMesh` _sm_wallmiddle_2 "/Game/Models/Wall/SM_WallMiddle.SM_WallMiddle")
    (`SceneComponent.SetWorldScale3D` (`self.SM_WallMiddle`) (* (`KismetMathLibrary.MakeVector` 1.0 (/ (`self.Middle_Length`) _returnvalue_y_4) 1.0) _returnvalue))
    (`SceneComponent.K2_SetRelativeLocationAndRotation` (`self.SM_WallFront`) (`KismetMathLibrary.MakeVector` 0.0 (`KismetMathLibrary.SelectFloat` _returnvalue_y_2 _returnvalue_y_3 _reversed)) (`KismetMathLibrary.MakeRotator` 0.0 0.0 _returnvalue_2) false false)
    (`SceneComponent.K2_SetRelativeLocationAndRotation` (`self.SM_WallRear`) (`KismetMathLibrary.MakeVector` 0.0 (`KismetMathLibrary.SelectFloat` _returnvalue_y_3 _returnvalue_y_2 _reversed)) (`KismetMathLibrary.MakeRotator` 0.0 0.0 _returnvalue_2) false false)
    (else
      (`StaticMeshComponent.SetStaticMesh` _sm_wallmiddle_2 "/Game/Models/Wall/SM_WallHole.SM_WallHole")
      (`SceneComponent.SetWorldScale3D` _sm_wallmiddle_2 _returnvalue))))