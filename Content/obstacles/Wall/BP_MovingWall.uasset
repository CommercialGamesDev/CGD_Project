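; Moving wall obstacle that sends one randomized BP_MovingWallCutout at a time along its spline.
; Spline duration scales with spline length, and Tick positions the wall by elapsed time using the spline component's rotation.
; Each wall gets random reversal, cutout and middle length values on spawn.
; It is destroyed at the last point, and the next spawns once the timer passes the travel duration plus DelayBetweenWalls.
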(event `self.ReceiveBeginPlay`
  (bind _output_get (set `SplineComponent.Duration` (/ (`SplineComponent.GetSplineLength` (`self.Spline`)) 100.0) (`self.Spline`)))
  (set `self.Delay` (+ _output_get (`self.Delay_Between_Walls`)))
  (set `self.Timer` 0.0 :!label _label)
  (bind _returnvalue (`|SpawnActorFromClass` "/Game/obstacles/Wall/BP_MovingWallCutout.BP_MovingWallCutout_C" (`SplineComponent.GetTransformAtSplinePoint` (`self.Spline`) 0 "Local" false) "Undefined" "MultiplyWithRoot" null null))
  (set `self.Wall` _returnvalue)
  (set `/Game/obstacles/Wall/BP_MovingWallCutout.Reversed` (`KismetMathLibrary.RandomBool`) (`self.Wall`))
  (set `/Game/obstacles/Wall/BP_MovingWallCutout.Cutout` (`KismetMathLibrary.RandomBool`) (`self.Wall`))
  (set `/Game/obstacles/Wall/BP_MovingWallCutout.Middle_Length` (`KismetMathLibrary.RandomIntegerInRange` 0 200) (`self.Wall`))
  (`/Game/obstacles/Wall/BP_MovingWallCutout.Update_Wall_Values` (`self.Wall`)))

(event `self.ReceiveTick`
  (params (DeltaSeconds :type "Float (single-precision)"))
  (bind _output_get (set `self.Delta_Seconds` DeltaSeconds))
  (bind _output_get_2 (set `self.Timer` (+ _output_get (`self.Timer`))))
  (if (`KismetSystemLibrary.IsValid` (`self.Wall`))
    (if (== (`self.K2_GetActorLocation` (`self.Wall`)) (`SplineComponent.GetLocationAtSplinePoint` (`self.Spline`) (- (`SplineComponent.GetNumberOfSplinePoints` (`self.Spline`)) 1) "World") :`ErrorTolerance` 1.0)
      (`self.K2_DestroyActor` (`self.Wall`))
      (else
        (`self.K2_SetActorLocationAndRotation` (`self.Wall`) (`SplineComponent.GetLocationAtTime` (`self.Spline`) (`self.Timer`) "World" false) (`SceneComponent.K2_GetComponentRotation` (`self.Spline`)) false false)))
    (elif (>= _output_get_2 (`self.Delay`))
      (goto _label))))

(fn `UserConstructionScript`)