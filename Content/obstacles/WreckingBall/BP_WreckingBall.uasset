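; Wrecking ball obstacle that swings and spins on its chain, with configurable motion, ball size and colours.
; BeginPlay starts a timeline at the swing speed, whose track, multiplied by swing distance, drives the chain's relative roll.
; Tick adds frame-rate-independent yaw spin while preserving that roll, combining both motions.
; The construction script applies ball scale and tints base, chain and ball through a material colour parameter.
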(event `self.ReceiveBeginPlay`
  (`TimelineComponent.SetPlayRate` (`self.Timeline`) (`self.SwingSpeed`))
  (`self.SwingBall`))

(event `SwingBall`
  (bind _chain (`self.Chain`))
  (bind (_relativerotation_roll _relativerotation_pitch _relativerotation_yaw) (`KismetMathLibrary.BreakRotator` (`SceneComponent.RelativeRotation` _chain)))
  (bind (_direction _swingtrack) (`Timeline|Timeline` :!via `PlayFromStart`)
    (:`Update`
      (`SceneComponent.K2_SetRelativeRotation` _chain (`KismetMathLibrary.MakeRotator` (* _swingtrack (`self.SwingDistance`)) 0.0 _relativerotation_yaw) false false))))

(event `self.ReceiveTick`
  (params (DeltaSeconds :type "Float (single-precision)"))
  (bind _chain (`self.Chain`))
  (bind (_relativerotation_roll _relativerotation_pitch _relativerotation_yaw) (`KismetMathLibrary.BreakRotator` (`SceneComponent.RelativeRotation` _chain)))
  (`SceneComponent.K2_SetRelativeRotation` _chain (`KismetMathLibrary.MakeRotator` _relativerotation_roll 0.0 (+ _relativerotation_yaw (* DeltaSeconds (`self.SpinSpeed`)))) false false))

(fn `UserConstructionScript`
  (bind _ballscale (`self.BallScale`))
  (`SceneComponent.SetWorldScale3D` (`self.Ball`) (`KismetMathLibrary.MakeVector` _ballscale _ballscale _ballscale))
  (`MeshComponent.SetColorParameterValueOnMaterials` (`self.Base`) "Colour" (`self.Base_Colour`))
  (`MeshComponent.SetColorParameterValueOnMaterials` (`self.Chain`) "Colour" (`self.Chain_Colour`))
  (`MeshComponent.SetColorParameterValueOnMaterials` (`self.Ball`) "Colour" (`self.Ball_Colour`)))