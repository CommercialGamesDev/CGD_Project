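; Repeller obstacle with an arm that moves vertically and periodically fires a radial force burst.
; On BeginPlay a speed-scaled timeline lerps the arm's height up to its own mesh bounds.
; Timeline values above 1 act as markers that flip a Falling flag, triggering a random sound, Niagara effect and brief force pulse on alternate flips.
; The construction script applies force settings and per-part colours.
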(event `self.ReceiveBeginPlay`
  (`TimelineComponent.SetPlayRate` (`self.Timeline`) (`self.Speed`))
  (`self.MoveRepeller`))

(event `MoveRepeller`
  (bind (_direction _repellertimeline) (`Timeline|Timeline` :!via `PlayFromStart`)
    (:`Update`
      (if (> _repellertimeline 1.0)
        (if (`self.Falling`)
          (`self.Repel`))
        (set `self.Falling` (not (`self.Falling`)))
        (else
          (bind _result (`/Engine/EditorBlueprintResources/StandardMacros.NegateFloat` (`KismetMathLibrary.Lerp` 0.0 (.z (`.Max` (`StaticMeshComponent.GetLocalBounds` (`self.Arm`)))) _repellertimeline))
            (:`  `
              (`SceneComponent.K2_SetRelativeLocation` (`self.Arm`) (`KismetMathLibrary.MakeVector` 0.0 0.0 _result) false false))))))))

(event `Repel`
  (bind _radialforce (`self.RadialForce`))
  (`GameplayStatics.PlaySoundAtLocation` (`KismetArrayLibrary.Array_Random` (`self.SoundArray`)) (`SceneComponent.K2_GetComponentLocation` (`self.Base`)) (struct) 1.0 1.0 0.0 "/Game/Audio/sound/Obstacles/Thumper/SA_Thumper.SA_Thumper" null null null)
  (`ActorComponent.Activate` (`self.Niagara`) false)
  (`ActorComponent.Activate` _radialforce false)
  (`KismetSystemLibrary.Delay` 0.2)
  (`ActorComponent.Deactivate` _radialforce))

(fn `UserConstructionScript`
  (bind _radialforce (`self.RadialForce`))
  (set `RadialForceComponent.Radius` (`self.RepelRadius`) _radialforce)
  (set `RadialForceComponent.ImpulseStrength` (`self.ImpulseStrength`) _radialforce)
  (set `RadialForceComponent.ForceStrength` (`self.ForceStrength`) _radialforce)
  (`MeshComponent.SetColorParameterValueOnMaterials` (`self.Base`) "Colour" (`self.Base_Colour`))
  (`MeshComponent.SetColorParameterValueOnMaterials` (`self.Arm`) "Colour" (`self.Arm_Colour`))
  (`MeshComponent.SetColorParameterValueOnMaterials` (`self.Head_Main`) "Colour" (`self.Head_Main_Colour`))
  (`MeshComponent.SetColorParameterValueOnMaterials` (`self.Head_Accent`) "Colour" (`self.Head_Accent_Colour`)))