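; BP_SequencedThrowManager is an audience-throw obstacle manager that groups lobber actors for sequenced throwing.
; On BeginPlay it finds every BP_Lobber whose GroupNo matches its GroupOwner, stores it in AllThrowers and sets itself as that lobber's owner reference.
; The construction script binds an event to lobber progress, while the LobberObjectHit event is currently an empty stub.
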(event `self.ReceiveBeginPlay`
  (bind _outactors (`GameplayStatics.GetAllActorsOfClass` "/Game/obstacles/AudienceThrow/BP_Lobber.BP_Lobber_C"))
  (for _array_element _outactors
    (if (== (`/Game/obstacles/AudienceThrow/BP_Lobber.GroupNo` _array_element) (`self.GroupOwner`))
      (`KismetArrayLibrary.Array_Add` (`self.AllThrowers`) _array_element)
      (set `/Game/obstacles/AudienceThrow/BP_Lobber.BelongsTo` self _array_element))))

(event `LobberObjectHit`
  (params (LobberNo :type Integer :default -1)))

(fn `UserConstructionScript`
  (add `self.LobberProgress` (`|CreateDelegate` :!event `LobberObjectHit`)))