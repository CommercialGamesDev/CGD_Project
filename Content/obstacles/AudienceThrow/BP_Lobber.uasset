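; BP_Lobber is an audience-throw obstacle that lobs throwable objects from a throw origin to a target.
; LobObject solves an arced launch velocity, predicts its path without collision tracing, then spawns a BP_ThrowableObject.
; The spawned object receives the predicted points as its travel arc, plus the list of objects to throw.
; ObjectHitReport passes hit notifications to the owning BelongsTo via LastLobberHit, identifying this lobber.
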(event `self.ReceiveBeginPlay`)

(event `LobObject`
  (bind _returnvalue (`SceneComponent.K2_GetComponentLocation` (`self.ThrowOrigin`)))
  (bind _outlaunchvelocity (`GameplayStatics.SuggestProjectileVelocity_CustomArc` _returnvalue (`SceneComponent.K2_GetComponentLocation` (`self.ThrowTarget`)) 0.0 0.2))
  (bind (_outhit _outpathpositions) (`GameplayStatics.Blueprint_PredictProjectilePath_ByObjectType` :`StartPos` _returnvalue :`LaunchVelocity` _outlaunchvelocity :`bTracePath` false :`ProjectileRadius` 3.0 :`ObjectTypes` (`|MakeArray` "ObjectTypeQuery2" :!type "EObjectTypeQuery Enum") :`DrawDebugTime` 1.0 :`SimFrequency` 200.0 :`MaxSimTime` 5.0))
  (bind _returnvalue_2 (`|SpawnActorFromClass` "/Game/obstacles/AudienceThrow/BP_ThrowableObject.BP_ThrowableObject_C" (`KismetMathLibrary.MakeTransform` (`SceneComponent.K2_GetComponentLocation` (`self.ThrowOrigin`))) "AlwaysSpawn" "MultiplyWithRoot" self null))
  (set `/Game/obstacles/AudienceThrow/BP_ThrowableObject.TravelArc` _outpathpositions _returnvalue_2)
  (set `/Game/obstacles/AudienceThrow/BP_ThrowableObject.ObjectsToThrow` (`self.Objects to Throw`) _returnvalue_2)
  (set `self.LobbedObject` _returnvalue_2))

(event `ObjectHitReport`
  (bind _belongsto (`self.BelongsTo`))
  (`/Engine/EditorBlueprintResources/StandardMacros.IsValid` _belongsto
    (:`Is Valid`
      (`/Game/obstacles/AudienceThrow/BP_SequencedThrowManager.LastLobberHit` _belongsto self))))

(fn `UserConstructionScript`)