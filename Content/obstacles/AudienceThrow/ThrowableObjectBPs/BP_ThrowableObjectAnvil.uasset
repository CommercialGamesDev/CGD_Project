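; Anvil variant of an audience-thrown obstacle that adds an impact sound when it hits a player.
; When its Hitbox begins overlapping an actor tagged Player, it casts to BP_ThirdPersonCharacter and checks that the character is not already in ragdoll.
; It then plays the anvil impact sound in 2D with slight random pitch variation.
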(event `self.Hitbox.OnComponentBeginOverlap`
  (params (OverlappedComponent :type "PrimitiveComponent Object Reference") (OtherActor :type "Actor Object Reference") (OtherComp :type "PrimitiveComponent Object Reference") (OtherBodyIndex :type Integer) (bFromSweep :type Boolean) (SweepResult :type "HitResult Structure (by ref)"))
  (if (`self.ActorHasTag` OtherActor "Player")
    (bind _asbp_third_person_character (cast `/Game/ThirdPerson/Blueprints/BP_ThirdPersonCharacter` OtherActor))
    (if (not (`/Game/ThirdPerson/Blueprints/BP_ThirdPersonCharacter.InRagdoll` _asbp_third_person_character))
      (`GameplayStatics.PlaySound2D` "/Game/Audio/sound/Obstacles/Throwables/AnvilImpact.AnvilImpact" 1.0 (`KismetMathLibrary.RandomFloatInRange` 0.9 1.1) 0.0 null null))))

(fn `UserConstructionScript`
  (`parent.UserConstructionScript`))