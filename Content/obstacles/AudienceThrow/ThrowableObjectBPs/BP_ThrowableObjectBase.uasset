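; Base actor for objects thrown by a BP_Lobber as obstacles, ragdolling and registering a hit on players they strike.
; A looping timer sweeps it along the TravelArc points with random spin, switching to physics near the arc's end before despawning.
; Tick line-traces down to place a drop-shadow decal, scaled and faded by height.
; The first player overlap enables physics, notifies game mode and lobber, then destroys it after a delay.
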(event `self.ReceiveBeginPlay`
  ; Choose mesh and start locomotion event to travel pre-defined arc
  (`KismetSystemLibrary.Delay` 0.05)
  (bind _asbp_lobber (cast `/Game/obstacles/AudienceThrow/BP_Lobber` (`self.GetOwner`)))
  (set `self.LobberOwner` _asbp_lobber)
  (`self.MakeRandomSpin`)
  (bind _returnvalue (`KismetSystemLibrary.K2_SetTimerDelegate` (delegate `MoveLobbedObject`) 0.009 true))
  (set `self.LocomoteObject` _returnvalue))

(event `MoveLobbedObject`
  (bind _travelarc (`self.TravelArc`))
  ; Move lobbed object through vectors of defined arc
  (`self.K2_SetActorLocation` (`|GetArrayItem` _travelarc (`self.ObjectStep`)) true)
  (`SceneComponent.K2_AddLocalRotation` (`self.Object`) (`self.RandomSpin`) false false)
  (bind _result (`/Engine/EditorBlueprintResources/StandardMacros.IncrementInt` (`self.ObjectStep`))
    (:`  `
      (if (== _result (- (`KismetArrayLibrary.Array_Length` _travelarc) 10))
        (`self.ResetLob`)
        (`KismetSystemLibrary.Delay` 10.0)
        (`self.K2_DestroyActor`)))))

(event `self.ReceiveTick`
  (params (DeltaSeconds :type "Float (single-precision)"))
  (bind _dropshadow (`self.DropShadow`))
  (bind _object (`self.Object`))
  (bind (_returnvalue_x _returnvalue_y) (`KismetMathLibrary.BreakVector` (`SceneComponent.K2_GetComponentLocation` _object)))
  ; Place drop shadow with line trace to the floor
  (`/Engine/EditorBlueprintResources/StandardMacros.IsValid` (`self.DropShadow`)
    (:`Is Valid`
      (bind _outhit (`KismetSystemLibrary.LineTraceSingle` (`SceneComponent.K2_GetComponentLocation` _object) (`KismetMathLibrary.MakeVector` _returnvalue_x _returnvalue_y -500.0) "TraceTypeQuery1"))
      (bind (_bblockinghit _binitialoverlap _time _distance _location _impactpoint) (`GameplayStatics.BreakHitResult` _outhit))
      (`SceneComponent.K2_SetWorldLocation` _dropshadow _impactpoint false false)
      (bind _returnvalue (/ (`KismetMathLibrary.FClamp` _distance 0.0 1000.0) 1000.0))
      (bind _returnvalue_2 (`KismetMathLibrary.Lerp` 2.0 0.5 _returnvalue))
      ; Change size and opacity of drop shadow as object falls
      (`SceneComponent.SetWorldScale3D` _dropshadow (`KismetMathLibrary.MakeVector` 1.0 _returnvalue_2 _returnvalue_2))
      (`DecalComponent.SetDecalColor` _dropshadow (make `LinearColor` 1.0 1.0 1.0 (`KismetMathLibrary.Lerp` 1.0 0.1 _returnvalue))))))

(event `self.Hitbox.OnComponentBeginOverlap`
  (params (OverlappedComponent :type "PrimitiveComponent Object Reference") (OtherActor :type "Actor Object Reference") (OtherComp :type "PrimitiveComponent Object Reference") (OtherBodyIndex :type Integer) (bFromSweep :type Boolean) (SweepResult :type "HitResult Structure (by ref)"))
  ; HitBox overlap to enable physics and look for hits
  (if (`self.ActorHasTag` OtherActor "Player")
    (`/Engine/EditorBlueprintResources/StandardMacros.DoOnce` false
      (:`Completed`
        (`PrimitiveComponent.SetSimulatePhysics` (`self.Object`) true)
        (bind _dropshadow (`self.DropShadow`)
          (:`then`
            (`ActorComponent.K2_DestroyComponent` _dropshadow))
          (:`else`
            _))
        (bind _asbp_third_person_character (cast `/Game/ThirdPerson/Blueprints/BP_ThirdPersonCharacter` OtherActor))
        (if (not (`/Game/ThirdPerson/Blueprints/BP_ThirdPersonCharacter.InRagdoll` _asbp_third_person_character))
          (`/Game/ThirdPerson/Blueprints/BP_ThirdPersonCharacter.Ragdoll Fall` _asbp_third_person_character false))
        (bind _asgm_multiplayer (cast `/Game/ThirdPerson/Blueprints/GM_Multiplayer` (`GameplayStatics.GetGameMode`)))
        (`/Game/ThirdPerson/Blueprints/GM_Multiplayer.PlayerHit` _asgm_multiplayer)
        ; Report back to lobber that it has hit and destroy object
        (`/Game/obstacles/AudienceThrow/BP_Lobber.ObjectHitReport` (`self.LobberOwner`))
        (`KismetSystemLibrary.Delay` 5.0)
        (`self.K2_DestroyActor`)))))

(fn `MakeRandomSpin`
  (bind (_spinrange_x _spinrange_y) (`KismetMathLibrary.BreakVector2D` (`self.SpinRange`)))
  (set `self.RandomSpin` (`KismetMathLibrary.MakeRotator` (`KismetMathLibrary.RandomFloatInRange` _spinrange_x _spinrange_y) (`KismetMathLibrary.RandomFloatInRange` _spinrange_x _spinrange_y) (`KismetMathLibrary.RandomFloatInRange` _spinrange_x _spinrange_y))))

(fn `ResetLob`
  (`KismetSystemLibrary.K2_ClearAndInvalidateTimerHandle` (`self.LocomoteObject`))
  (`KismetArrayLibrary.Array_Clear` (`self.TravelArc`))
  (set `self.ObjectStep` 0)
  (`PrimitiveComponent.SetSimulatePhysics` (`self.Object`) true))

(fn `UserConstructionScript`)