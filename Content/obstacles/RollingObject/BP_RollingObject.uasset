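; BP_RollingObject is an obstacle actor for a rolling object with a configurable static mesh.
; Its construction script passes MeshInput to SetMesh, which assigns the mesh, scales the Collider from that mesh's box extent and applies the PM_Ragdoll physical material override.
; The event graph holds only disabled placeholder events, so the Blueprint adds no runtime movement or overlap logic.
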(fn `SetMesh`
  (params (Mesh :type "StaticMesh Object Reference"))
  (bind (_returnvalue_origin _returnvalue_boxextent) (`KismetMathLibrary.BreakBoxSphereBounds` (`StaticMesh.GetBounds` (`StaticMeshComponent.StaticMesh` (`self.Mesh`)))))
  (`StaticMeshComponent.SetStaticMesh` (`self.Mesh`) Mesh)
  (`SceneComponent.SetWorldScale3D` (`self.Collider`) (/ _returnvalue_boxextent 50.0))
  (`PrimitiveComponent.SetPhysMaterialOverride` (`self.Mesh`) "/Game/Materials/Physics/PM_Ragdoll.PM_Ragdoll"))

(fn `UserConstructionScript`
  (`self.SetMesh` (`self.MeshInput`)))