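; Obstacle spawner actor that periodically emits rolling objects while enabled.
; Tick counts down a cooldown, then spawns a BP_RollingObject at the Billboard component's world transform and gives it a random mesh from the Meshes list.
; Each new cooldown is the mean interval plus a random offset within the allowed variance, with the construction script setting the first to the mean.
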(event `self.ReceiveTick`
  (params (DeltaSeconds :type "Float (single-precision)"))
  (if (`self.Enabled`)
    (bind _output_get (set `self.Cooldown` (- (`self.Cooldown`) DeltaSeconds)))
    (if (<= _output_get 0.0)
      (bind _returnvalue (`|SpawnActorFromClass` "/Game/obstacles/RollingObject/BP_RollingObject.BP_RollingObject_C" (`SceneComponent.K2_GetComponentToWorld` (`self.Billboard`)) "Undefined" "MultiplyWithRoot" null null))
      (`/Game/obstacles/RollingObject/BP_RollingObject.SetMesh` _returnvalue (`KismetArrayLibrary.Array_Random` (`self.Meshes`)))
      (set `self.Cooldown` (+ (`self.Mean Frequency`) (`KismetMathLibrary.RandomFloatInRange` (- 0.0 (`self.Max Variance`)) (`self.Max Variance`)))))))

(fn `UserConstructionScript`
  (set `self.Cooldown` (`self.Mean Frequency`)))