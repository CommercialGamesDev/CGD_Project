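; BP_BigFan is a fan obstacle that pushes actors tagged Pushable with wind while it is active.
; Each tick it finds actors overlapping its box and moves them with a swept offset along the arrow's forward direction, scaled by wind push and frame time.
; The same wind push drives the propeller's spin.
; The construction script sets the X scale of the Collisions component from the wind range.
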(event `self.ReceiveTick`
  (params (DeltaSeconds :type "Float (single-precision)"))
  (bind _returnvalue (* DeltaSeconds (`self.WindPush`)))
  (if (`self.IsActive`)
    (`|ExecutionSequence`
      (:`then_0`
        (for _array_element (`PrimitiveComponent.GetOverlappingActors` (`self.Box`) null)
          (if (`self.ActorHasTag` _array_element "Pushable")
            (`self.K2_AddActorWorldOffset` _array_element (* (`KismetMathLibrary.GetForwardVector` (`SceneComponent.K2_GetComponentRotation` (`self.Arrow`))) _returnvalue) true false))))
      (:`then_1`
        (`SceneComponent.K2_AddLocalRotation` (`self.Propellers`) (`KismetMathLibrary.MakeRotator` (* _returnvalue 2.0)) false false)))))

(fn `UserConstructionScript`
  (bind (_returnvalue_x _returnvalue_y _returnvalue_z) (`KismetMathLibrary.BreakVector` (`SceneComponent.K2_GetComponentScale` (`self.Collisions`))))
  (`SceneComponent.SetWorldScale3D` (`self.Collisions`) (`KismetMathLibrary.MakeVector` (`self.WindRange`) _returnvalue_y _returnvalue_z)))