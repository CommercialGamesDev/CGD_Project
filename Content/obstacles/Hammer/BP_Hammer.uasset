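; BP_Hammer is a hammer obstacle that either swings or rotates continuously, depending on Oscillate.
; The construction script sizes the arm, head and end caps from length and scale settings, positions them using local bounds, applies colours and stores the starting yaw.
; At BeginPlay, a speed-scaled timeline drives actor pitch at that yaw when oscillating; otherwise RotatingMovement spins it at SpeedOfRotation.
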(event `self.ReceiveBeginPlay`
  (if (`self.Oscillate`)
    (`TimelineComponent.SetPlayRate` (`self.Timeline`) (/ (`self.Speed_Of_Rotation`) 180.0))
    (`self.RotateAxeToEnd`)
    (else
      (set `RotatingMovementComponent.RotationRate` (`KismetMathLibrary.MakeRotator` 0.0 (`self.Speed_Of_Rotation`)) (`self.RotatingMovement`)))))

(event `RotateAxeToEnd`
  (bind (_direction _newtrack_0) (`Timeline|Timeline` :!via `PlayFromStart`)
    (:`Update`
      (`self.K2_SetActorRotation` (`KismetMathLibrary.MakeRotator` 0.0 (+ 0.0 _newtrack_0) (`self.Start_Rotation`))))))

(fn `UserConstructionScript`
  (bind _head (`self.Head`))
  (bind _front_end (`self.Front_End`))
  (bind _back_end (`self.Back_End`))
  (bind (_scale_of_head_x _scale_of_head_y _scale_of_head_z) (`KismetMathLibrary.BreakVector` (`self.Scale_Of_Head`)))
  (bind (_scale_of_head_x_2 _scale_of_head_y_2 _scale_of_head_z_2) (`KismetMathLibrary.BreakVector` (`self.Scale_Of_Head`)))
  (bind (_min _max) (`StaticMeshComponent.GetLocalBounds` (`self.Arm`)))
  (bind (_returnvalue_x _returnvalue_y _returnvalue_z) (`KismetMathLibrary.BreakVector` (`SceneComponent.K2_GetComponentScale` (`self.Arm`))))
  (bind (_returnvalue_roll _returnvalue_pitch _returnvalue_yaw) (`KismetMathLibrary.BreakRotator` (`SceneComponent.K2_GetComponentRotation` (`self.Core`))))
  (bind (_returnvalue_x_2 _returnvalue_y_2 _returnvalue_z_2) (`KismetMathLibrary.BreakVector` (+ _min _max)))
  ; Arm Scale/Length
  (bind _output_get (set `self.Core_Scale` (`KismetMathLibrary.MakeVector` _returnvalue_x _returnvalue_y _returnvalue_z)))
  (`SceneComponent.SetWorldScale3D` (`self.Arm`) (`KismetMathLibrary.MakeVector` (.x _output_get) (.y _output_get) (* _returnvalue_z (`self.Length_Of_Arm`))))
  ; Head Scale
  (`SceneComponent.SetWorldScale3D` (`self.Head`) (* (`self.Scale_Of_Head`) (`self.Core_Scale`)))
  ; Head Location
  (`SceneComponent.K2_SetRelativeLocation` _head (0.0 0.0 0.0) false false)
  (`SceneComponent.K2_AddLocalOffset` _head (`KismetMathLibrary.MakeVector` 0.0 0.0 _returnvalue_z_2) false false)
  ; Front End Scale
  (`SceneComponent.SetWorldScale3D` (`self.Front_End`) (* (`KismetMathLibrary.MakeVector` (/ (+ _scale_of_head_y_2 _scale_of_head_z_2) 2.0) _scale_of_head_y_2 _scale_of_head_z_2) (`self.Core_Scale`)))
  ; Front End Location
  (`SceneComponent.K2_SetRelativeLocation` _front_end (0.0 0.0 0.0) false false)
  (`SceneComponent.K2_AddLocalOffset` _front_end (`KismetMathLibrary.MakeVector` (.x (`.Max` (`StaticMeshComponent.GetLocalBounds` (`self.Head`))))) false false)
  ; Back End Scale
  (`SceneComponent.SetWorldScale3D` (`self.Back_End`) (* (`KismetMathLibrary.MakeVector` (/ (+ _scale_of_head_y _scale_of_head_z) 2.0) _scale_of_head_y _scale_of_head_z) (`self.Core_Scale`)))
  ; Back End Location
  (`SceneComponent.K2_SetRelativeLocation` _back_end (0.0 0.0 0.0) false false)
  (`SceneComponent.K2_AddLocalOffset` _back_end (`KismetMathLibrary.MakeVector` (.x (`.Max` (`StaticMeshComponent.GetLocalBounds` (`self.Head`))))) false false)
  (set `self.Start_Rotation` _returnvalue_yaw)
  (`MeshComponent.SetColorParameterValueOnMaterials` (`self.Core`) "Colour" (`self.Core_Colour`))
  (`MeshComponent.SetColorParameterValueOnMaterials` (`self.Arm`) "Colour" (`self.Arm_Colour`))
  (`MeshComponent.SetColorParameterValueOnMaterials` (`self.Head`) "Colour" (`self.Head_Colour`))
  (`MeshComponent.SetColorParameterValueOnMaterials` (`self.Front_End`) "Colour" (`self.Head_Colour`))
  (`MeshComponent.SetColorParameterValueOnMaterials` (`self.Back_End`) "Colour" (`self.Head_Colour`)))