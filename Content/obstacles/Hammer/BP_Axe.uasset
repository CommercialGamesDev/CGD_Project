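; BP_Axe is a swinging or spinning axe obstacle with configurable speed, arm length and head scale.
; Its construction script scales the arm and head, offsets the head using the arm's bounds, and stores the core's starting yaw.
; On BeginPlay, Oscillate selects either a Timeline that drives actor pitch at a speed-scaled play rate, or continuous rotation through RotatingMovement.
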(event `self.ReceiveBeginPlay`
  (if (`self.Oscillate`)
    (`TimelineComponent.SetPlayRate` (`self.Timeline`) (/ (`self.Speed_Of_Rotation`) 180.0))
    (`self.RotateAxeToEnd`)
    (else
      (set `RotatingMovementComponent.RotationRate` (`KismetMathLibrary.MakeRotator` 0.0 (`self.Speed_Of_Rotation`)) (`self.RotatingMovement`)))))

(event `RotateAxeToEnd`
  (bind (_direction _newtrack_0) (`Timeline|Timeline` :!via `PlayFromStart`)
    (:`Update`
      (`self.K2_SetActorRotation` (`KismetMathLibrary.MakeRotator` 0.0 (+ 0.0 _newtrack_0) (`self.StartRotation`))))))

(fn `UserConstructionScript`
  (bind _head (`self.Head`))
  (bind (_min _max) (`StaticMeshComponent.GetLocalBounds` (`self.Arm`)))
  (bind (_returnvalue_x _returnvalue_y _returnvalue_z) (`KismetMathLibrary.BreakVector` (`SceneComponent.K2_GetComponentScale` (`self.Arm`))))
  (bind (_returnvalue_roll _returnvalue_pitch _returnvalue_yaw) (`KismetMathLibrary.BreakRotator` (`SceneComponent.K2_GetComponentRotation` (`self.Core`))))
  (bind (_returnvalue_x_2 _returnvalue_y_2 _returnvalue_z_2) (`KismetMathLibrary.BreakVector` (+ _min _max)))
  ; Arm Scale/Length
  (bind _output_get (set `self.Core_Scale` (`KismetMathLibrary.MakeVector` _returnvalue_x _returnvalue_y _returnvalue_z)))
  (`SceneComponent.SetWorldScale3D` (`self.Arm`) (`KismetMathLibrary.MakeVector` (.x _output_get) (.y _output_get) (* _returnvalue_z (`self.Length_Of_Arm`))))
  ; Head Scale
  (`SceneComponent.SetWorldScale3D` (`self.Head`) (* (`self.Scale_Of_Head`) (`self.Core_Scale`)))
  ; Head Location
  (`SceneComponent.K2_SetRelativeLocation` _head (0.0 0.0 0.0) false false)
  (`SceneComponent.K2_AddLocalOffset` _head (`KismetMathLibrary.MakeVector` 0.0 0.0 _returnvalue_z_2) false false)
  (set `self.StartRotation` _returnvalue_yaw))