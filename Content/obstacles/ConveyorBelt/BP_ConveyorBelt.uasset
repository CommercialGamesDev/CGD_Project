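; BP_ConveyorBelt is a conveyor belt obstacle that carries actors tagged "Pushable" along its arrow's direction.
; Each tick, it moves tagged actors overlapping its box with a swept world offset scaled by Speed and delta time.
; The construction script sizes the thin box from SizeX and SizeY and creates a dynamic belt material.
; The material's speed parameter derives from Speed divided by belt length, tying the visual to the push rate.
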(event `self.ReceiveTick`
  (params (DeltaSeconds :type "Float (single-precision)"))
  (for _array_element (`PrimitiveComponent.GetOverlappingActors` (`self.Box`) null)
    (if (`self.ActorHasTag` _array_element "Pushable")
      (`self.K2_AddActorWorldOffset` _array_element (* (`KismetMathLibrary.GetForwardVector` (`SceneComponent.K2_GetComponentRotation` (`self.Arrow`))) (* DeltaSeconds (`self.Speed`))) true false))))

(fn `UserConstructionScript`
  (`SceneComponent.SetRelativeScale3D` (`self.Box`) (`KismetMathLibrary.MakeVector` (`self.SizeX`) (`self.SizeY`) 0.05))
  (bind _returnvalue (`PrimitiveComponent.CreateDynamicMaterialInstance` (`self.SM_Conveyor`) 0 "/Game/obstacles/ConveyorBelt/M_Conveyor.M_Conveyor" "None"))
  (bind _output_get (set `self.Conveyor_Material` _returnvalue))
  (`MaterialInstanceDynamic.SetScalarParameterValue` _output_get "Speed" (/ (`self.Speed`) (* (`self.SizeY`) 100.0)))
  (`PrimitiveComponent.SetMaterial` (`self.SM_Conveyor`) 0 (`self.Conveyor_Material`)))