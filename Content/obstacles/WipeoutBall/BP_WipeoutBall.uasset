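; BP_WipeoutBall is a Wipeout-style obstacle ball that repels physics objects when its sphere is overlapped.
; An overlap briefly activates a radial force, plays a random sound and runs a timeline that dips and restores the ball's height, with a short cooldown before the next bounce.
; The construction script applies radius and strength variables to the force component.
; An optional flag also switches the BP_CameraDrone style on each hit.
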(event `self.ReceiveBeginPlay`
  (`ActorComponent.Deactivate` (`self.RadialForce`)))

(event `self.Sphere.OnComponentBeginOverlap`
  (params (OverlappedComponent :type "PrimitiveComponent Object Reference") (OtherActor :type "Actor Object Reference") (OtherComp :type "PrimitiveComponent Object Reference") (OtherBodyIndex :type Integer) (bFromSweep :type Boolean) (SweepResult :type "HitResult Structure (by ref)"))
  (bind _radialforce (`self.RadialForce`))
  (if (`self.CanBounce`)
    (if (`self.DoesTheCameraThings`)
      (bind _returnvalue (`GameplayStatics.GetActorOfClass` "/Game/ThirdPerson/Camera/BP_CameraDrone.BP_CameraDrone_C"))
      (set `/Game/ThirdPerson/Camera/BP_CameraDrone.Style` "NewEnumerator8" _returnvalue))
    (`GameplayStatics.PlaySoundAtLocation` (`KismetArrayLibrary.Array_Random` (`self.SoundArray`)) (`SceneComponent.K2_GetComponentLocation` (`self.BallPart`)) (struct) 1.0 1.0 0.0 "/Game/Audio/sound/Obstacles/Thumper/SA_Thumper.SA_Thumper" null null null)
    (set `self.CanBounce` false)
    (`ActorComponent.Activate` _radialforce false)
    (`self.AnimateBounce`)
    (`KismetSystemLibrary.Delay` 0.5)
    (`ActorComponent.Deactivate` _radialforce)
    (set `self.CanBounce` true)))

(event `AnimateBounce`
  (bind (_direction _newtrack_0) (`Timeline|Timeline` :!via `PlayFromStart`)
    (:`Update`
      (`SceneComponent.K2_SetRelativeLocation` (`self.BallPart`) (`KismetMathLibrary.MakeVector` 0.0 0.0 (`KismetMathLibrary.Lerp` 75.0 55.0 _newtrack_0)) false false))))

(fn `UserConstructionScript`
  (bind _radialforce (`self.RadialForce`))
  (set `RadialForceComponent.Radius` (`self.RepelRadius`) _radialforce)
  (set `RadialForceComponent.ImpulseStrength` (`self.ImpulseStrength`) _radialforce)
  (set `RadialForceComponent.ForceStrength` (`self.ForceStrength`) _radialforce))