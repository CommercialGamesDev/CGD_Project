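; Falling-platform obstacle that disappears after a Character touches it and later respawns.
; Box overlap swaps the Platform to a collision material, waits a delay, then hides it and disables its collision.
; Leaving the Box starts a respawn timer, with no actor filter, that restores the standard material, visibility and collision.
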(event `self.Box.OnComponentBeginOverlap`
  (params (OverlappedComponent :type "PrimitiveComponent Object Reference") (OtherActor :type "Actor Object Reference") (OtherComp :type "PrimitiveComponent Object Reference") (OtherBodyIndex :type Integer) (bFromSweep :type Boolean) (SweepResult :type "HitResult Structure (by ref)"))
  (cast `Character` OtherActor)
  (`PrimitiveComponent.SetMaterial` (`self.Platform`) 0 (`self.CollisionMaterial`))
  (`KismetSystemLibrary.Delay` (`self.Delay`))
  (`SceneComponent.SetVisibility` (`self.Platform`) false false)
  (`PrimitiveComponent.SetCollisionEnabled` (`self.Platform`) "NoCollision"))

(event `self.Box.OnComponentEndOverlap`
  (params (OverlappedComponent :type "PrimitiveComponent Object Reference") (OtherActor :type "Actor Object Reference") (OtherComp :type "PrimitiveComponent Object Reference") (OtherBodyIndex :type Integer))
  (`KismetSystemLibrary.Delay` (`self.RespawnTime`))
  (`PrimitiveComponent.SetMaterial` (`self.Platform`) 0 (`self.StandardMaterial`))
  (`SceneComponent.SetVisibility` (`self.Platform`) true false)
  (`PrimitiveComponent.SetCollisionEnabled` (`self.Platform`) "QueryAndPhysics"))

(fn `UserConstructionScript`)