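; Launch pad obstacle that flings overlapping "Pushable"-tagged characters and objects along a set direction, optionally requiring two players to launch characters.
; Overlap launches characters or applies impulses to other actors' primitive components.
; In two-player mode, Tick poses pad and spring as rest, compressed or extended by player count, disabling pad collision during a cooldown after firing.
; BeginPlay caches those poses, and the construction script aligns an arrow to the launch direction.
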(event `self.Collider.OnComponentBeginOverlap`
  (params (OverlappedComponent :type "PrimitiveComponent Object Reference") (OtherActor :type "Actor Object Reference") (OtherComp :type "PrimitiveComponent Object Reference") (OtherBodyIndex :type Integer) (bFromSweep :type Boolean) (SweepResult :type "HitResult Structure (by ref)"))
  (bind _returnvalue (* (`self.Launch_Direction`) (`self.LaunchDistance`)))
  (for _array_element (`PrimitiveComponent.GetOverlappingActors` (`self.Collider`) null)
    (if (`self.ActorHasTag` _array_element "Pushable")
      (bind _asbp_third_person_character (cast `/Game/ThirdPerson/Blueprints/BP_ThirdPersonCharacter` _array_element)
        (:`then`
          (if (`self.2_Players_Required`)
            (if (not (`self.Fired`))
              (`self.2PlayerLaunch`))
            (else
              (`Character.LaunchCharacter` _asbp_third_person_character _returnvalue false false))))
        (:`CastFailed`
          (for _array_element_2 (`self.K2_GetComponentsByClass` _array_element "/Script/Engine.PrimitiveComponent")
            (`PrimitiveComponent.AddImpulse` _array_element_2 _returnvalue "None" false)))))))

(event `self.ReceiveTick`
  (params (DeltaSeconds :type "Float (single-precision)"))
  (set `self.DeltaSeconds` DeltaSeconds)
  (if (and (`self.2_Players_Required`) (not (`self.Fired`)))
    (switch `int` (`KismetArrayLibrary.Array_Length` (`PrimitiveComponent.GetOverlappingActors` (`self.Collider`) "/Game/ThirdPerson/Blueprints/BP_ThirdPersonCharacter.BP_ThirdPersonCharacter_C"))
      (:`0`
        (`SceneComponent.K2_SetRelativeLocation` (`self.LaunchPad`) (`self.Pad_Rest_Location`) false false)
        (`SceneComponent.SetRelativeScale3D` (`self.LaunchSpring`) (`self.Spring_Rest_Scale`)))
      (:`1`
        (`SceneComponent.K2_SetRelativeLocation` (`self.LaunchPad`) (`self.Pad_Compressed_Location`) false false)
        (`SceneComponent.SetRelativeScale3D` (`self.LaunchSpring`) (`self.Spring_Compressed_Scale`)))
      (:`2`
        (`PrimitiveComponent.SetCollisionEnabled` (`self.LaunchPad`) "NoCollision")
        (`SceneComponent.K2_SetRelativeLocation` (`self.LaunchPad`) (`self.Pad_Extended_Location`) false false)
        (`SceneComponent.SetRelativeScale3D` (`self.LaunchSpring`) (`self.Spring_Extended_Scale`))
        (set `self.Fired` true)
        (`KismetSystemLibrary.Delay` (`self.Cooldown_Time`))
        (set `self.Fired` false)
        (`PrimitiveComponent.SetCollisionEnabled` (`self.LaunchPad`) "QueryAndPhysics")))))

(event `2PlayerLaunch`
  (bind _overlappingactors (`PrimitiveComponent.GetOverlappingActors` (`self.Collider`) "/Game/ThirdPerson/Blueprints/BP_ThirdPersonCharacter.BP_ThirdPersonCharacter_C"))
  (if (== (`KismetArrayLibrary.Array_Length` _overlappingactors) 2)
    (for _array_element _overlappingactors
      (bind _asbp_third_person_character (cast `/Game/ThirdPerson/Blueprints/BP_ThirdPersonCharacter` _array_element))
      (`Character.LaunchCharacter` _asbp_third_person_character (* (`self.Launch_Direction`) (`self.LaunchDistance`)) false false))))

(event `self.ReceiveBeginPlay`
  (bind (_relativescale3d_x _relativescale3d_y _relativescale3d_z) (`KismetMathLibrary.BreakVector` (`SceneComponent.RelativeScale3D` (`self.LaunchSpring`))))
  (bind (_relativelocation_x _relativelocation_y _relativelocation_z) (`KismetMathLibrary.BreakVector` (`SceneComponent.RelativeLocation` (`self.LaunchPad`))))
  (bind (_relativescale3d_x_2 _relativescale3d_y_2 _relativescale3d_z_2) (`KismetMathLibrary.BreakVector` (`SceneComponent.RelativeScale3D` (`self.LaunchSpring`))))
  (bind (_relativelocation_x_2 _relativelocation_y_2 _relativelocation_z_2) (`KismetMathLibrary.BreakVector` (`SceneComponent.RelativeLocation` (`self.LaunchPad`))))
  (set `self.LaunchDistance` (* (`self.LaunchDistance`) 10.0))
  (`|ExecutionSequence`
    (:`then_0`
      (set `self.Spring_Rest_Scale` (`SceneComponent.RelativeScale3D` (`self.LaunchSpring`))))
    (:`then_1`
      (set `self.Spring_Compressed_Scale` (`KismetMathLibrary.MakeVector` _relativescale3d_x_2 _relativescale3d_y_2 (* _relativescale3d_z_2 (`self.Compression_Factor`)))))
    (:`then_2`
      (set `self.Spring_Extended_Scale` (`KismetMathLibrary.MakeVector` _relativescale3d_x _relativescale3d_y (* _relativescale3d_z (`self.Extension_Factor`)))))
    (:`then_3`
      (set `self.Pad_Rest_Location` (`SceneComponent.RelativeLocation` (`self.LaunchPad`))))
    (:`then_4`
      (set `self.Pad_Compressed_Location` (`KismetMathLibrary.MakeVector` _relativelocation_x_2 _relativelocation_y_2 (* _relativelocation_z_2 (`self.Compression_Factor`)))))
    (:`then_5`
      (set `self.Pad_Extended_Location` (`KismetMathLibrary.MakeVector` _relativelocation_x _relativelocation_y (* _relativelocation_z (`self.Extension_Factor`)))))))

(fn `UserConstructionScript`
  (bind (_launch_direction_roll _launch_direction_pitch _launch_direction_yaw) (`KismetMathLibrary.BreakRotator` (`self.Launch_Direction`)))
  (`SceneComponent.K2_SetWorldRotation` (`self.Arrow`) (`KismetMathLibrary.MakeRotator` _launch_direction_roll _launch_direction_pitch _launch_direction_yaw) false false))