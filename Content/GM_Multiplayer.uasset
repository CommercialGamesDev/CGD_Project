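; Game mode for local multiplayer that handles level transitions, music and the level timer.
; LoadLevel stores the level index in the BP_Level game instance, opens the matching map by name and, outside the menu, requests a BP_CameraDrone if none exists.
; BeginPlay ensures a second local player, then plays menu intro-to-loop music or a random track with a timer widget.
; Tick derives minutes and seconds; EndTimer records the end time and removes the widget.
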(event `Load Level`
  (params (`Level to load` :type Integer))
  ; The functionality at the end of a level to open and load the next played level
  (bind _asbp_level (cast `/Game/Util/BP_Level` (`GameplayStatics.GetGameInstance`)))
  (bind _output_get (set `/Game/Util/BP_Level.Level` `Level to load` _asbp_level))
  (switch `int` _output_get
    (:`Default`
      (set `self.LevelName` (`KismetStringLibrary.Conv_StringToName` (`KismetStringLibrary.Concat_StrStr` "Level" (`KismetStringLibrary.Conv_IntToString` _output_get)))))
    (:`-1`
      (set `self.LevelName` "MainMenu"))
    (:`0`
      (set `self.LevelName` "TutorialLevel")))
  (`GameplayStatics.OpenLevel` (`self.LevelName`))
  (if (!= _output_get -1)
    (bind _returnvalue (`GameplayStatics.GetActorOfClass` "/Game/ThirdPerson/Blueprints/camera/BP_CameraDrone.BP_CameraDrone_C"))
    (if (not (`KismetSystemLibrary.IsValid` _returnvalue))
      (`|SpawnActorFromClass` "/Game/ThirdPerson/Blueprints/camera/BP_CameraDrone.BP_CameraDrone_C" (`KismetMathLibrary.MakeTransform` (0.0 0.0 0.0)) "Undefined" "MultiplyWithRoot" null null))))

(event `self.ReceiveBeginPlay`
  ; The level start (load level on the NEW level)
  (if (< (`GameplayStatics.GetNumPlayerControllers`) 2)
    (`GameplayStatics.CreatePlayer` -1))
  (set `self.Start Time` (`KismetSystemLibrary.GetGameTimeInSeconds`))
  (bind _returnvalue (`GameplayStatics.GetCurrentLevelName` true))
  (if (`KismetStringLibrary.EqualEqual_StrStr` _returnvalue "MainMenu")
    (`self.PlaySong` "/Game/Audio/music/PHOCTheme1611INTRO.PHOCTheme1611INTRO")
    (`KismetSystemLibrary.Delay` 4.5)
    (`self.PlaySong` "/Game/Audio/music/PHOCTheme1611LOOP.PHOCTheme1611LOOP")
    (else
      (`self.PlaySong` (`KismetArrayLibrary.Array_Random` (`self.MusicPool`)))
      (bind _returnvalue_2 (`|CreateWidget` "/Game/UI/WBP_TimerUI.WBP_TimerUI_C"))
      (bind _output_get (set `self.On screen timer` _returnvalue_2))
      (`UserWidget.AddToViewport` _output_get 0))))

(event `End Timer`
  ; Timer handling
  (set `self.End Time` (`KismetSystemLibrary.GetGameTimeInSeconds`))
  (`Widget.RemoveFromParent` (`self.On screen timer`)))

(event `self.ReceiveTick`
  (params (DeltaSeconds :type "Float (single-precision)"))
  ; Timer handling
  (set `self.Current Minute` (/ (`KismetMathLibrary.FFloor` (`KismetSystemLibrary.GetGameTimeInSeconds`)) 60))
  (set `self.Current Second` (mod (`KismetMathLibrary.FTrunc` (`KismetSystemLibrary.GetGameTimeInSeconds`)) 60)))

(fn `PlaySong`
  (params (Song :type "SoundBase Object Reference"))
  (`AudioComponent.SetSound` (`self.Music`) Song)
  (`AudioComponent.Play` (`self.Music`) 0.0))

(fn `UserConstructionScript`)