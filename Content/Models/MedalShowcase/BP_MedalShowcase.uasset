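; Medal showcase display that presents one level's name, horse emblem and saved completion progress.
; The construction script sets the name from DT_LevelData and the medal's horse texture, or shows "Coming Soon..." for index -1.
; After a short BeginPlay delay, it reads the Completion save to hide unearned ribbons.
; If a screenshot index exists, it loads that PNG from disk for completed levels, colours three objective horseshoes and tints the medal by count.
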(event `self.ReceiveBeginPlay`
  (bind _sm_horseshoe2 (`self.SM_HorseShoe2`))
  (bind _sm_horseshoe (`self.SM_HorseShoe`))
  (bind _sm_horseshoe1 (`self.SM_HorseShoe1`))
  ; Put dis in construkt 4 nao
  (`KismetSystemLibrary.Delay` 0.2)
  (bind _returnvalue (`GameplayStatics.LoadGameFromSlot` "Completion"))
  (bind _asbp_completion_data (cast `/Game/Data/BP_CompletionData` _returnvalue))
  (bind (_output_levelcomplete _output_objective1 _output_objective2 _output_objective3 _output_fastesttime _output_screenshotindex) (break `/Game/Data/S_LevelCompletion` (`|GetArrayItem` (`/Game/Data/BP_CompletionData.LevelCompletion` _asbp_completion_data) (+ (`self.LevelIndex`) 1))))
  (if (not _output_levelcomplete)
    (`SceneComponent.SetVisibility` (`self.SM_Ribbon`) false true))
  (if (!= _output_screenshotindex -1)
    (bind _returnvalue_2 (`KismetRenderingLibrary.ImportFileAsTexture2D` (`KismetStringLibrary.Concat_StrStr` (`KismetSystemLibrary.GetProjectDirectory`) "Saved/SaveGames/Screenshots/lol" (`KismetStringLibrary.Conv_Int64ToString` _output_screenshotindex) ".png")))
    (if (and _output_levelcomplete (!= _returnvalue_2 null))
      (bind _returnvalue_3 (`PrimitiveComponent.CreateDynamicMaterialInstance` (`self.Plane`) 0 "/Game/Models/ScreenshotShowcase/M_ScreenshotMaterial.M_ScreenshotMaterial" "None"))
      (`MaterialInstanceDynamic.SetTextureParameterValue` _returnvalue_3 "ScreenshotTexture" _returnvalue_2))
    (if _output_objective1
      (`/Engine/EditorBlueprintResources/StandardMacros.IncrementInt` (`self.CompletedObjectives`)
        (:`  `
          (`PrimitiveComponent.SetMaterial` _sm_horseshoe 1 "/Game/Models/BeachBall/yellow.yellow")))
      (else
        (`PrimitiveComponent.SetMaterial` _sm_horseshoe 1 "/Game/Models/MedalShowcase/M_DarkGrey.M_DarkGrey")))
    (if _output_objective2
      (`/Engine/EditorBlueprintResources/StandardMacros.IncrementInt` (`self.CompletedObjectives`)
        (:`  `
          (`PrimitiveComponent.SetMaterial` _sm_horseshoe1 1 "/Game/Models/BeachBall/yellow.yellow")))
      (else
        (`PrimitiveComponent.SetMaterial` _sm_horseshoe1 1 "/Game/Models/MedalShowcase/M_DarkGrey.M_DarkGrey")))
    (if _output_objective3
      (`/Engine/EditorBlueprintResources/StandardMacros.IncrementInt` (`self.CompletedObjectives`)
        (:`  `
          (`PrimitiveComponent.SetMaterial` _sm_horseshoe2 1 "/Game/Models/BeachBall/yellow.yellow")))
      (else
        (`PrimitiveComponent.SetMaterial` _sm_horseshoe2 1 "/Game/Models/MedalShowcase/M_DarkGrey.M_DarkGrey")))
    (`MeshComponent.SetColorParameterValueOnMaterials` (`self.SM_Medal`) "Colour" (`|GetArrayItem` (`self.Tier_Colours`) (`KismetMathLibrary.Clamp` (- (`self.CompletedObjectives`) 1) 0 2)))))

(fn `UserConstructionScript`
  (if (== (`self.LevelIndex`) -1)
    (`TextRenderComponent.K2_SetText` (`self.LevelName`) (`KismetTextLibrary.Conv_StringToText` "Coming Soon..."))
    (else
      (bind _outrownames (`DataTableFunctionLibrary.GetDataTableRowNames` "/Game/Levels/LevelSystem/DT_LevelData.DT_LevelData"))
      (bind _returnvalue (`|GetDataTableRow` "/Game/Levels/LevelSystem/DT_LevelData.DT_LevelData" (`|GetArrayItem` _outrownames (`self.LevelIndex`)))
        (:`then`
          (`TextRenderComponent.K2_SetText` (`self.LevelName`) (`KismetTextLibrary.Conv_StringToText` (break `/Game/Levels/LevelSystem/F_LevelStruct` _returnvalue)))
          (bind _returnvalue_2 (`PrimitiveComponent.CreateDynamicMaterialInstance` (`self.SM_Medal`) 1 (`self.HorseMaterial`) "None"))
          (`MaterialInstanceDynamic.SetTextureParameterValue` _returnvalue_2 "Horse" (`|GetArrayItem` (`self.HorseTextures`) (+ (`self.LevelIndex`) 1))))))))