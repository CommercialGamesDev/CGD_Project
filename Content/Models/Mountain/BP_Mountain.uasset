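; BP_Mountain is a procedurally built mountain actor: a scalable cone ringed with floor-panel platforms, with no active runtime logic.
; The construction script scales and lifts the Cone from ConeScale, then adds a static mesh component for each PlatformData entry.
; Each entry gives angle and height, converted by trigonometry to a spot around the tapering cone, pushed out by Extension.
; Yaw follows that angle, while Orientation sets roll and pitch.
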(fn `UserConstructionScript`
  (bind (_conescale_x _conescale_y) (`KismetMathLibrary.BreakVector2D` (`self.ConeScale`)))
  (bind (_conescale_x_2 _conescale_y_2) (`KismetMathLibrary.BreakVector2D` (`self.ConeScale`)))
  (`SceneComponent.SetWorldScale3D` (`self.Cone`) (`KismetMathLibrary.MakeVector` _conescale_x _conescale_x _conescale_y))
  (`SceneComponent.K2_SetRelativeLocation` (`self.Cone`) (`KismetMathLibrary.MakeVector` 0.0 0.0 (* _conescale_y 50.0)) false false)
  (for _array_element (`self.PlatformData`)
    (bind _returnvalue (`AddComponent|NODE_AddStaticMeshComponent-0` :`bManualAttachment` true))
    (`StaticMeshComponent.SetStaticMesh` _returnvalue "/Game/Models/Platform/FloorPanel.FloorPanel")
    (`SceneComponent.K2_AttachToComponent` _returnvalue (`self.DefaultSceneRoot`) "None" "KeepRelative" "KeepRelative" "KeepRelative" false)
    (`KismetArrayLibrary.Array_Add` (`self.Platforms`) _returnvalue)
    (bind _returnvalue_2 (- 1.0 (/ (`.Y` (`KismetMathLibrary.BreakVector2D` (break `/Game/Models/Mountain/S_MountainPlatform` _array_element))) (* _conescale_y_2 50.0)) -1.0))
    (`SceneComponent.K2_SetRelativeLocationAndRotation` _returnvalue (`KismetMathLibrary.MakeVector` (* (`KismetMathLibrary.DegCos` (`KismetMathLibrary.BreakVector2D` (break `/Game/Models/Mountain/S_MountainPlatform` _array_element))) (+ (* _conescale_x_2 25.0 _returnvalue_2) 75.0 (`.Extension_18_26A830184F072121451E809024C15334` (break `/Game/Models/Mountain/S_MountainPlatform` _array_element)))) (* (`KismetMathLibrary.DegSin` (`KismetMathLibrary.BreakVector2D` (break `/Game/Models/Mountain/S_MountainPlatform` _array_element))) (+ (* _conescale_x_2 25.0 _returnvalue_2) 75.0 (`.Extension_18_26A830184F072121451E809024C15334` (break `/Game/Models/Mountain/S_MountainPlatform` _array_element)))) (`.Y` (`KismetMathLibrary.BreakVector2D` (break `/Game/Models/Mountain/S_MountainPlatform` _array_element)))) (`KismetMathLibrary.MakeRotator` (`KismetMathLibrary.BreakVector2D` (`.Orientation_13_3A33B98142D48ABD9EC42091C98502AC` (break `/Game/Models/Mountain/S_MountainPlatform` _array_element))) (`.Y` (`KismetMathLibrary.BreakVector2D` (`.Orientation_13_3A33B98142D48ABD9EC42091C98502AC` (break `/Game/Models/Mountain/S_MountainPlatform` _array_element)))) (`KismetMathLibrary.BreakVector2D` (break `/Game/Models/Mountain/S_MountainPlatform` _array_element))) false false)))