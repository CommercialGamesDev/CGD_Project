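; BP_Medal is a medal prop whose appearance is configured by tier, ribbon and horse design.
; Its Construction Script applies the ribbon material and sets the medal's Colour parameter from a per-tier colour list.
; It also creates a dynamic material instance on the medal's second slot to show a horse texture picked by index.
; BeginPlay does nothing.
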(event `self.ReceiveBeginPlay`)

(fn `UserConstructionScript`
  (`PrimitiveComponent.SetMaterial` (`self.SM_Ribbon`) 0 (`self.RibbonMaterial`))
  (`MeshComponent.SetColorParameterValueOnMaterials` (`self.SM_Medal`) "Colour" (`|GetArrayItem` (`self.Tier_Colours`) (`self.Tier`)))
  (bind _returnvalue (`PrimitiveComponent.CreateDynamicMaterialInstance` (`self.SM_Medal`) 1 (`self.HorseMaterial`) "None"))
  (`MaterialInstanceDynamic.SetTextureParameterValue` _returnvalue "Horse" (`|GetArrayItem` (`self.HorseTextures`) (`self.Horse_Material_Index`))))