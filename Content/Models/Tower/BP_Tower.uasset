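; BP_Tower procedurally builds a circular tower of static mesh blocks in its construction script.
; It derives the angular step and block count per ring from the radius, scaled mesh bounds and gap, and floor spacing from block height.
; Nested loops add a mesh component per block, positioned with sine and cosine, yawed around the ring and offset in angle per floor.
; Each block gets a random material from the Materials array.
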(fn `UserConstructionScript`
  (bind _radius (`self.Radius`))
  (bind _blockheightscale (`self.BlockHeightScale`))
  (bind (_origin _boxextent) (`KismetMathLibrary.BreakBoxSphereBounds` (`StaticMesh.GetBounds` (`self.BlockType`))))
  (bind _output_get (set `self.Circumference` (* (`self.Radius`) (`KismetMathLibrary.GetPI`) 2.0)))
  (bind _returnvalue (`KismetMathLibrary.FTrunc` (/ _output_get (+ (* (.y _boxextent) (`self.BlockWidthScale`)) (`self.Gap Between Blocks`)))))
  (set `self.AngleIncrement` (/ 360.0 _returnvalue))
  (set `self.HeightofBlock` (+ (* (.z _boxextent) _blockheightscale) (* _blockheightscale 40.0)))
  (bind _output_get_2 (set `self.End Index` (+ _returnvalue 1)))
  (for _index (range (+ (`self.NumberofFloors`) 1))
    (set `self.CurrentHeight` (* _index (`self.CurrentHeight`)))
    (for _index_2 (range (+ _output_get_2 1))
      (set `self.CurrentIndex` _index_2)
      (bind _returnvalue_2 (+ (* (`self.Angle Offset per floor`) _index) (* (`self.CurrentIndex`) (`self.AngleIncrement`))))
      (bind _returnvalue_3 (`AddComponent|NODE_AddStaticMeshComponent-1` :`RelativeTransform` (`KismetMathLibrary.MakeTransform` (`KismetMathLibrary.MakeVector` (* (`KismetMathLibrary.DegCos` _returnvalue_2) _radius) (* _radius (`KismetMathLibrary.DegSin` _returnvalue_2)) (* _index (`self.HeightofBlock`))) (`KismetMathLibrary.MakeRotator` 0.0 0.0 _returnvalue_2) (`KismetMathLibrary.MakeVector` 1.0 (`self.BlockWidthScale`) (`self.BlockHeightScale`)))))
      (`StaticMeshComponent.SetStaticMesh` _returnvalue_3 (`self.BlockType`))
      (`PrimitiveComponent.SetMaterial` _returnvalue_3 0 (`KismetArrayLibrary.Array_Random` (`self.Materials`))))))