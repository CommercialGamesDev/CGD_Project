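; Procedural fence actor that builds a row of posts and three-piece panels in its construction script, with an optional right-angle corner.
; Posts are spaced by panel width, switching from X to Y at the corner index, and their positions anchor the top, middle and bottom panel meshes.
; Panel count is clamped against post count, and posts and each panel layer get their own colour through the "Colour" material parameter.
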(fn `UserConstructionScript`
  (locals (Panel_Top :type "StaticMesh Object Reference" :default "/Script/Engine.StaticMesh'/Game/Models/Fence/FencePanelTop.FencePanelTop'") (Panel_Middle :type "StaticMesh Object Reference" :default "/Script/Engine.StaticMesh'/Game/Models/Fence/FencePanelMiddle.FencePanelMiddle'") (Panel_Bottom :type "StaticMesh Object Reference" :default "/Script/Engine.StaticMesh'/Game/Models/Fence/FencePanelBottom.FencePanelBottom'") (Panel_Width :type "Float (double-precision)" :default 400.0))
  (bind _panel_width (`local.Panel_Width`))
  (bind _posts (`self.Posts`))
  (bind _returnvalue (/ (`local.Panel_Width`) 2.0))
  (bind _returnvalue_2 (select `int` (`self.Panel_Piece`) :`0` (`self.Panel_Tops`) :`1` (`self.Panel_Middles`) :`2` (`self.Panel_Bottoms`)))
  (bind _returnvalue_3 (`KismetArrayLibrary.Array_Length` _returnvalue_2))
  (bind _output (`|GetArrayItem` _posts (- (`KismetArrayLibrary.Array_Length` _posts) 1)))
  (bind _output_2 (`|GetArrayItem` (`self.Posts`) _returnvalue_3))
  (bind _returnvalue_4 (`KismetMathLibrary.SelectVector` (`KismetMathLibrary.MakeVector` 0.0 _panel_width) (`KismetMathLibrary.MakeVector` _panel_width) (and (> (`KismetArrayLibrary.Array_Length` (`self.Posts`)) (`self.Corner_Post_Index`)) (`self.Corner`))))
  (bind _returnvalue_5 (and (>= _returnvalue_3 (`self.Corner_Post_Index`)) (`self.Corner`)))
  (bind _returnvalue_6 (`KismetMathLibrary.SelectRotator` (struct :`Yaw` 90.0) (struct) _returnvalue_5))
  (`KismetArrayLibrary.Array_Clear` (`self.Posts`))
  (`KismetArrayLibrary.Array_Clear` (`self.Panel_Bottoms`))
  (`KismetArrayLibrary.Array_Clear` (`self.Panel_Middles`))
  (`KismetArrayLibrary.Array_Clear` (`self.Panel_Tops`))
  (set `self.Number_Of_Panels` (`KismetMathLibrary.Clamp` (`self.Number_Of_Panels`) 0 (`KismetMathLibrary.Max` (`self.Number_Of_Posts`) 1)))
  (while (< (`KismetArrayLibrary.Array_Length` (`self.Posts`)) (`self.Number_Of_Posts`))
    (if (`KismetSystemLibrary.IsValid` _output)
      (bind _returnvalue_7 (`AddComponent|NODE_AddStaticMeshComponent-1` :`RelativeTransform` (`KismetMathLibrary.MakeTransform` (+ _returnvalue_4 (`SceneComponent.RelativeLocation` _output)))))
      (`StaticMeshComponent.SetStaticMesh` _returnvalue_7 "/Game/Models/Fence/FencePost.FencePost")
      (`KismetArrayLibrary.Array_Add` (`self.Posts`) _returnvalue_7)
      (else
        (bind _returnvalue_8 (`AddComponent|NODE_AddStaticMeshComponent-3` :`RelativeTransform` (`KismetMathLibrary.MakeTransform` (+ _returnvalue_4 (-400.0 0.0 0.0)))))
        (`StaticMeshComponent.SetStaticMesh` _returnvalue_8 "/Game/Models/Fence/FencePost.FencePost")
        (`KismetArrayLibrary.Array_Add` (`self.Posts`) _returnvalue_8))))
  (for _index (range 3)
    (set `self.Panel_Piece` _index)
    (while (< _returnvalue_3 (`self.Number_Of_Panels`))
      (if (`KismetSystemLibrary.IsValid` _output_2)
        (bind _returnvalue_9 (`AddComponent|NODE_AddStaticMeshComponent-2` :`RelativeTransform` (`KismetMathLibrary.MakeTransform` (+ (`SceneComponent.RelativeLocation` _output_2) (`KismetMathLibrary.SelectVector` (`KismetMathLibrary.MakeVector` 0.0 _returnvalue) (`KismetMathLibrary.MakeVector` _returnvalue) _returnvalue_5)) _returnvalue_6)))
        (`StaticMeshComponent.SetStaticMesh` _returnvalue_9 (select `int` (`self.Panel_Piece`) :`0` (`local.Panel_Top`) :`1` (`local.Panel_Middle`) :`2` (`local.Panel_Bottom`)))
        (`KismetArrayLibrary.Array_Add` (select `int` (`self.Panel_Piece`) :`0` (`self.Panel_Tops`) :`1` (`self.Panel_Middles`) :`2` (`self.Panel_Bottoms`)) _returnvalue_9)
        (else
          (bind _returnvalue_10 (`AddComponent|NODE_AddStaticMeshComponent-4` :`RelativeTransform` (`KismetMathLibrary.MakeTransform` (0.0 0.0 0.0) _returnvalue_6)))
          (`StaticMeshComponent.SetStaticMesh` _returnvalue_10 (select `int` (`self.Panel_Piece`) :`0` (`local.Panel_Top`) :`1` (`local.Panel_Middle`) :`2` (`local.Panel_Bottom`)))
          (`KismetArrayLibrary.Array_Add` (select `int` (`self.Panel_Piece`) :`0` (`self.Panel_Tops`) :`1` (`self.Panel_Middles`) :`2` (`self.Panel_Bottoms`)) _returnvalue_10))))
    (for _array_element _returnvalue_2
      (`MeshComponent.SetColorParameterValueOnMaterials` _array_element "Colour" (select `int` (`self.Panel_Piece`) :`0` (`self.Panel_Top_Colour`) :`1` (`self.Panel_Middle_Colour`) :`2` (`self.Panel_Bottom_Colour`)))))
  (for _array_element_2 (`self.Posts`)
    (`MeshComponent.SetColorParameterValueOnMaterials` _array_element_2 "Colour" (`self.Post_Colour`))))