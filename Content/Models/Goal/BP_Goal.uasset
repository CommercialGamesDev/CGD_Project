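; BP_Goal is a goal actor that sets off confetti when a beach ball enters its detection volume.
; A GoalDetection begin overlap with BP_BeachBall passes a DoOnce and spawns scaled-up NS_Confetti Niagara systems at two emitter locations.
; When the ball ends the overlap, the stored emitter references are cleared, without explicitly deactivating the systems, and the DoOnce resets for the next goal.
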(event `self.GoalDetection.OnComponentBeginOverlap`
  (params (OverlappedComponent :type "PrimitiveComponent Object Reference") (OtherActor :type "Actor Object Reference") (OtherComp :type "PrimitiveComponent Object Reference") (OtherBodyIndex :type Integer) (bFromSweep :type Boolean) (SweepResult :type "HitResult Structure (by ref)"))
  (bind _emmiterlocation1 (`self.EmmiterLocation1`))
  (bind _emitterlocation2 (`self.EmitterLocation2`))
  ; Needs testing more, better particles and be for beach ball and not player
  (if (`GameplayStatics.ObjectIsA` OtherActor "/Game/Models/BeachBall/BP_BeachBall.BP_BeachBall_C")
    (`/Engine/EditorBlueprintResources/StandardMacros.DoOnce` false :!label _label
      (:`Completed`
        (bind _returnvalue (`NiagaraFunctionLibrary.SpawnSystemAtLocationWithParams` (make `FXSystemSpawnParameters` _emmiterlocation1 "/Game/Particles/NiagaraSystems/NS_Confetti.NS_Confetti" (`SceneComponent.K2_GetComponentLocation` _emmiterlocation1) (struct) (40.0 40.0 40.0))))
        (set `self.Emmiter1` _returnvalue)
        (bind _returnvalue_2 (`NiagaraFunctionLibrary.SpawnSystemAtLocationWithParams` (make `FXSystemSpawnParameters` _emitterlocation2 "/Game/Particles/NiagaraSystems/NS_Confetti.NS_Confetti" (`SceneComponent.K2_GetComponentLocation` _emitterlocation2) (struct) (40.0 40.0 40.0))))
        (set `self.Emmiter2` _returnvalue_2)))))

(event `self.GoalDetection.OnComponentEndOverlap`
  (params (OverlappedComponent :type "PrimitiveComponent Object Reference") (OtherActor :type "Actor Object Reference") (OtherComp :type "PrimitiveComponent Object Reference") (OtherBodyIndex :type Integer))
  (if (`GameplayStatics.ObjectIsA` OtherActor "/Game/Models/BeachBall/BP_BeachBall.BP_BeachBall_C")
    (set `self.Emmiter1` null)
    (set `self.Emmiter2` null)
    (goto _label :!via `Reset`)))

(fn `UserConstructionScript`)