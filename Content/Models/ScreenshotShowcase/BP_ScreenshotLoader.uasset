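; BP_ScreenshotLoader is a showcase actor that displays a saved screenshot for a given level on a plane.
; On BeginPlay it loads the "Completion" save slot and reads the screenshot index recorded for its LevelIndex.
; If one exists, it imports the matching PNG from the project's saved Screenshots folder at runtime.
; The texture is applied to the plane through a dynamic instance of M_ScreenshotMaterial.
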(event `self.ReceiveBeginPlay`
  (bind _returnvalue (`GameplayStatics.LoadGameFromSlot` "Completion"))
  (bind _asbp_completion_data (cast `/Game/Data/BP_CompletionData` _returnvalue))
  (bind (_output_levelcomplete _output_objective1 _output_objective2 _output_objective3 _output_fastesttime _output_screenshotindex) (break `/Game/Data/S_LevelCompletion` (`|GetArrayItem` (`/Game/Data/BP_CompletionData.LevelCompletion` _asbp_completion_data) (`self.LevelIndex`))))
  (if (!= _output_screenshotindex -1)
    (bind _returnvalue_2 (`KismetRenderingLibrary.ImportFileAsTexture2D` (`KismetStringLibrary.Concat_StrStr` (`KismetSystemLibrary.GetProjectDirectory`) "Saved/SaveGames/Screenshots/lol" (`KismetStringLibrary.Conv_Int64ToString` _output_screenshotindex) ".png")))
    (if (!= _returnvalue_2 null)
      (bind _returnvalue_3 (`PrimitiveComponent.CreateDynamicMaterialInstance` (`self.Plane`) 0 "/Game/Models/ScreenshotShowcase/M_ScreenshotMaterial.M_ScreenshotMaterial" "None"))
      (`MaterialInstanceDynamic.SetTextureParameterValue` _returnvalue_3 "ScreenshotTexture" _returnvalue_2))))

(fn `UserConstructionScript`)