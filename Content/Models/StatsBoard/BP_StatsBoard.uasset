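; BP_StatsBoard is a board that displays the player's saved lifetime stats, such as levels played, hits, respawns, playtime and fastest level.
; On BeginPlay or SetUpStats it loads the PlayerStats save slot, casts it to BP_PlayerStats and fills each text element.
; Two helper functions format zero-padded times, with a placeholder when no fastest level exists.
; The long-time helper divides by zero for hours and never wraps minutes at sixty.
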(event `self.ReceiveBeginPlay`
  (bind _returnvalue (`GameplayStatics.LoadGameFromSlot` "PlayerStats" :!label _label))
  (bind _asbp_player_stats (cast `/Game/Data/BP_PlayerStats` _returnvalue))
  (`TextRenderComponent.K2_SetText` (`self.LevelsClearedStat`) (`KismetTextLibrary.Conv_IntToText` (`/Game/Data/BP_PlayerStats.LevelsCleared` _asbp_player_stats)))
  (`TextRenderComponent.K2_SetText` (`self.LevelsPlayedStat`) (`KismetTextLibrary.Conv_IntToText` (`/Game/Data/BP_PlayerStats.LevelsPlayed` _asbp_player_stats)))
  (`TextRenderComponent.K2_SetText` (`self.ObjectivesCompleteStat`) (`KismetTextLibrary.Conv_IntToText` (`/Game/Data/BP_PlayerStats.ObjectivesCompleted` _asbp_player_stats)))
  (`TextRenderComponent.K2_SetText` (`self.TimesHitStat`) (`KismetTextLibrary.Conv_IntToText` (`/Game/Data/BP_PlayerStats.Hits` _asbp_player_stats)))
  (`TextRenderComponent.K2_SetText` (`self.RespawnsStat`) (`KismetTextLibrary.Conv_IntToText` (`/Game/Data/BP_PlayerStats.Respawns` _asbp_player_stats)))
  (bind _timestring (`self.SecondsToLongTimeString` (`KismetMathLibrary.Conv_IntToDouble` (`/Game/Data/BP_PlayerStats.Playtime` _asbp_player_stats))))
  (`TextRenderComponent.K2_SetText` (`self.PlaytimeStat`) (`KismetTextLibrary.Conv_StringToText` _timestring))
  (bind _fastestlevelname (`/Game/Data/BP_PlayerStats.FastestLevelName` _asbp_player_stats))
  (`TextRenderComponent.K2_SetText` (`self.FastestLevelStat`) (`KismetTextLibrary.Conv_StringToText` _fastestlevelname))
  (if (== _fastestlevelname "None")
    (`TextRenderComponent.K2_SetText` (`self.FastestLevelTimeStat`) "0:00")
    (else
      (bind _timestring_2 (`self.SecondsToTimeString` (`/Game/Data/BP_PlayerStats.FastestLevelTime` _asbp_player_stats)))
      (`TextRenderComponent.K2_SetText` (`self.FastestLevelTimeStat`) (`KismetTextLibrary.Conv_StringToText` _timestring_2)))))

(event `SetUpStats`
  (goto _label))

(fn `SecondsToLongTimeString`
  (params (Seconds :type "Float (double-precision)"))
  (returns (TimeString :type String))
  (bind _returnvalue (`KismetMathLibrary.FFloor` (mod Seconds 60.0)))
  (bind _returnvalue_2 (`KismetMathLibrary.FFloor` (/ Seconds 60.0)))
  (set `self.Hours` (`KismetStringLibrary.Conv_IntToString` (`KismetMathLibrary.FFloor` (/ Seconds 0.0))))
  (bind _output_get (set `self.Minutes` (`KismetStringLibrary.Conv_IntToString` _returnvalue_2)))
  (bind _output_get_2 (set `self.Seconds` (`KismetStringLibrary.Conv_IntToString` _returnvalue)))
  (if (< _returnvalue_2 10)
    (set `self.Minutes` (`KismetStringLibrary.Concat_StrStr` "0" _output_get)))
  (if (< _returnvalue 10)
    (set `self.Seconds` (`KismetStringLibrary.Concat_StrStr` "0" _output_get_2)))
  (return (`KismetStringLibrary.Concat_StrStr` (`KismetStringLibrary.Concat_StrStr` (`KismetStringLibrary.Concat_StrStr` (`KismetStringLibrary.Concat_StrStr` (`self.Hours`) ":") (`self.Minutes`)) ":") (`self.Seconds`))))

(fn `SecondsToTimeString`
  (params (Seconds :type "Float (double-precision)"))
  (returns (TimeString :type String))
  (bind _returnvalue (`KismetMathLibrary.FFloor` (/ Seconds 60.0)))
  (bind _returnvalue_2 (- Seconds (* _returnvalue 60)))
  (if (< _returnvalue 10)
    (set `self.Minutes` (`KismetStringLibrary.Concat_StrStr` "0" (`KismetStringLibrary.Conv_IntToString` _returnvalue)))
    (else
      (set `self.Minutes` (`KismetStringLibrary.Conv_IntToString` _returnvalue))))
  (if (< _returnvalue_2 10)
    (set `self.Seconds` (`KismetStringLibrary.Concat_StrStr` "0" (`KismetStringLibrary.Conv_IntToString` _returnvalue_2)))
    (else
      (set `self.Seconds` (`KismetStringLibrary.Conv_IntToString` _returnvalue_2))))
  (return (`KismetStringLibrary.Concat_StrStr` (`KismetStringLibrary.Concat_StrStr` (`self.Minutes`) ":") (`self.Seconds`))))

(fn `UserConstructionScript`)