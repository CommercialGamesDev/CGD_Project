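; Settings data Blueprint that holds the game's graphics options and applies them to the engine.
; InitSettings disables Nanite, Lumen diffuse GI and virtual shadow maps, caps FPS, loads any non-zero preset, then applies and saves.
; ApplyPreset copies DT_GraphicsDefaults rows into quality, audience and TV variables.
; ApplyAllSettings sets window mode and resolution through GameUserSettings, builds scalability console commands for quality levels, then calls save.
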(event `InitSettings`
  (`KismetSystemLibrary.ExecuteConsoleCommand` null "r.Nanite 0" null)
  (`KismetSystemLibrary.ExecuteConsoleCommand` null "r.LumenDiffuseIndirect.Allow 0" null)
  (`KismetSystemLibrary.ExecuteConsoleCommand` null "r.Shadow.Virtual.Enable 0" null)
  (`KismetSystemLibrary.ExecuteConsoleCommand` null "t.maxfps 60" null)
  (if (not (== (`self.PresetMode`) 0))
    (`self.ApplyPreset`))
  (`self.ApplyAllSettings`)
  (`self.OnSave`))

(fn `ApplyAllSettings`
  (`self.ApplyFullscreen`)
  (`self.ApplyShadowQuality`)
  (`self.ApplyTextureQuality`)
  (`self.ApplyAntiAliasingQuality`)
  (`self.ApplyParticleQuality`)
  (`self.ApplyPostProcessQuality`)
  (`self.OnSave`))

(fn `ApplyAntiAliasingQuality`
  (`KismetSystemLibrary.ExecuteConsoleCommand` null (`KismetStringLibrary.Concat_StrStr` "sg.AntiAliasingQuality " (`KismetStringLibrary.Conv_IntToString` (`self.Anti-AliasingQuality`))) null))

(fn `ApplyFullscreen`
  (bind _returnvalue (`GameUserSettings.GetGameUserSettings`))
  (switch `int` (`self.FullscreenStatus`)
    (:`0`
      (`GameUserSettings.SetFullscreenMode` _returnvalue "Fullscreen")
      (`GameUserSettings.SetScreenResolution` _returnvalue (`GameUserSettings.GetDesktopResolution` _returnvalue) :!label _label))
    (:`1`
      (`GameUserSettings.SetFullscreenMode` _returnvalue "WindowedFullscreen")
      (goto _label))
    (:`2`
      (`GameUserSettings.SetFullscreenMode` _returnvalue "Windowed")
      (if (`KismetMathLibrary.Equal_IntPointIntPoint` (`GameUserSettings.GetScreenResolution` _returnvalue) (`GameUserSettings.GetDesktopResolution` _returnvalue))
        (`GameUserSettings.SetScreenResolution` _returnvalue (make `IntPoint` 1280 720)))))
  (`GameUserSettings.ApplySettings` _returnvalue false))

(fn `ApplyParticleQuality`
  (`KismetSystemLibrary.ExecuteConsoleCommand` null (`KismetStringLibrary.Concat_StrStr` "sg.EffectsQuality " (`KismetStringLibrary.Conv_IntToString` (`self.ParticleQuality`))) null))

(fn `ApplyPostProcessQuality`
  (`KismetSystemLibrary.ExecuteConsoleCommand` null (`KismetStringLibrary.Concat_StrStr` "sg.PostProcessQuality " (`KismetStringLibrary.Conv_IntToString` (`self.PostProcessQuality`))) null))

(fn `ApplyPreset`
  (bind (_presetvalues_shadowquality _presetvalues_texturequality _presetvalues_antialiasingquality _presetvalues_particlequality _presetvalues_postprocessquality _presetvalues_audiencedensity _presetvalues_audienceanimation _presetvalues_tvenabled) (break `/Game/Data/S_GraphicsDefaults` (`self.PresetValues`)))
  (switch `int` (`self.PresetMode`)
    (:`1`
      (bind _returnvalue (`|GetDataTableRow` "/Game/Data/DT_GraphicsDefaults.DT_GraphicsDefaults" "Low")
        (:`then`
          (set `self.PresetValues` _returnvalue))))
    (:`2`
      (bind _returnvalue_2 (`|GetDataTableRow` "/Game/Data/DT_GraphicsDefaults.DT_GraphicsDefaults" "Medium")
        (:`then`
          (set `self.PresetValues` _returnvalue_2))))
    (:`3`
      (bind _returnvalue_3 (`|GetDataTableRow` "/Game/Data/DT_GraphicsDefaults.DT_GraphicsDefaults" "High")
        (:`then`
          (set `self.PresetValues` _returnvalue_3)))))
  (set `self.ShadowQuality` _presetvalues_shadowquality)
  (set `self.TextureQuality` _presetvalues_texturequality)
  (set `self.Anti-AliasingQuality` _presetvalues_antialiasingquality)
  (set `self.ParticleQuality` _presetvalues_particlequality)
  (set `self.PostProcessQuality` _presetvalues_postprocessquality)
  (set `self.AudienceDensity` _presetvalues_audiencedensity)
  (set `self.AudienceAnimations` _presetvalues_audienceanimation)
  (set `self.TVToggle` _presetvalues_tvenabled))

(fn `ApplyShadowQuality`
  (`KismetSystemLibrary.ExecuteConsoleCommand` null (`KismetStringLibrary.Concat_StrStr` "sg.ShadowQuality " (`KismetStringLibrary.Conv_IntToString` (`self.ShadowQuality`))) null))

(fn `ApplyTextureQuality`
  (`KismetSystemLibrary.ExecuteConsoleCommand` null (`KismetStringLibrary.Concat_StrStr` "sg.TextureQuality " (`KismetStringLibrary.Conv_IntToString` (`self.TextureQuality`))) null))