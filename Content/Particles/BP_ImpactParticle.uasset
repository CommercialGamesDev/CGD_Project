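; Comic-style impact effect actor that pops a layered sprite of lettering, bubble, impact lines and stars, then destroys itself.
; InitaliseImage takes a forced or random type, looks up each layer's sprite in its map, zeroes the scales and opens a gate.
; Through that gate, Tick scales each layer by its own float curve over ShrinkFactor at a delayed interval, until the duration ends and cleanup runs.
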(event `Initalise Image`
  (params (`Force Type` :type Name) (IsRandom :type Boolean))
  ; Called when the particles are spawned
  (if IsRandom
    (bind _keys (`BlueprintMapLibrary.Map_Keys` (`self.Lettering Map`)))
    (`KismetArrayLibrary.Array_Shuffle` _keys)
    (set `self.Image ID` (`|GetArrayItem` _keys))
    (else
      (set `self.Image ID` `Force Type`)))
  ; Set up all the corresponding parts of the full sprite
  (`PaperSpriteComponent.SetSprite` (`self.Lettering`) (`BlueprintMapLibrary.Map_Find` (`self.Lettering Map`) (`self.Image ID`)))
  (`PaperSpriteComponent.SetSprite` (`self.Bubble`) (`BlueprintMapLibrary.Map_Find` (`self.Bubble Map`) (`self.Image ID`)))
  (`PaperSpriteComponent.SetSprite` (`self.Impact Lines`) (`BlueprintMapLibrary.Map_Find` (`self.Impact Line Map`) (`self.Image ID`)))
  (`PaperSpriteComponent.SetSprite` (`self.Stars`) (`BlueprintMapLibrary.Map_Find` (`self.Star Map`) (`self.Image ID`)))
  (`SceneComponent.SetRelativeScale3D` (`self.Stars`) (0.0 0.0 0.0))
  (`SceneComponent.SetRelativeScale3D` (`self.Impact Lines`) (0.0 0.0 0.0))
  (`SceneComponent.SetRelativeScale3D` (`self.Bubble`) (0.0 0.0 0.0))
  (`SceneComponent.SetRelativeScale3D` (`self.Lettering`) (0.0 0.0 0.0))
  (set `self.Time Accumulator` 0.0)
  (`self.StartAnimation`))

(event `self.ReceiveTick`
  (params (DeltaSeconds :type "Float (single-precision)"))
  (bind _returnvalue (`CurveFloat.GetFloatValue` (`self.LetteringCurve`) (`self.Time Accumulator`)))
  (bind _returnvalue_2 (`CurveFloat.GetFloatValue` (`self.StarCurve`) (`self.Time Accumulator`)))
  (bind _returnvalue_3 (`CurveFloat.GetFloatValue` (`self.LineCurve`) (`self.Time Accumulator`)))
  (bind _returnvalue_4 (`CurveFloat.GetFloatValue` (`self.BubbleCurve`) (`self.Time Accumulator`)))
  (`/Engine/EditorBlueprintResources/StandardMacros.Gate` true :!label _label
    (:`Exit`
      (`KismetSystemLibrary.Delay` (`self.Animation Interval`))
      (`SceneComponent.SetRelativeScale3D` (`self.Stars`) (/ (`KismetMathLibrary.MakeVector` _returnvalue_2 _returnvalue_2 _returnvalue_2) (`self.ShrinkFactor`)))
      (`SceneComponent.SetRelativeScale3D` (`self.Impact Lines`) (/ (`KismetMathLibrary.MakeVector` _returnvalue_3 _returnvalue_3 _returnvalue_3) (`self.ShrinkFactor`)))
      (`SceneComponent.SetRelativeScale3D` (`self.Bubble`) (/ (`KismetMathLibrary.MakeVector` _returnvalue_4 _returnvalue_4 _returnvalue_4) (`self.ShrinkFactor`)))
      (`SceneComponent.SetRelativeScale3D` (`self.Lettering`) (/ (`KismetMathLibrary.MakeVector` _returnvalue _returnvalue _returnvalue) (`self.ShrinkFactor`)))
      (set `self.Time Accumulator` (+ (`self.Animation Interval`) (`self.Time Accumulator`)))
      (if (>= (`self.Time Accumulator`) (`self.AnimationDuration`))
        (`self.StopAnimation`)
        (`self.Cleanup`)))))

(event `StartAnimation`
  (goto _label :!via `Open`))

(event `StopAnimation`
  (goto _label :!via `Close`))

(event `Cleanup`
  (`KismetSystemLibrary.Delay` 0.2)
  (`ActorComponent.K2_DestroyComponent` (`self.Bubble`))
  (`ActorComponent.K2_DestroyComponent` (`self.Lettering`))
  (`ActorComponent.K2_DestroyComponent` (`self.Impact Lines`))
  (`ActorComponent.K2_DestroyComponent` (`self.Stars`))
  (`self.K2_DestroyActor`))

(fn `UserConstructionScript`)