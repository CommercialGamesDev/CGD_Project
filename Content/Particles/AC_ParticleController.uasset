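; Actor component that drives a player's despawn, respawn and impact Niagara effects.
; BeginPlay sorts the owner's Niagara components by FX_Despawn and FX_Respawn tags for the play events to activate.
; Respawn fast-forwards the simulation to skip the outward explosion and show the implosion into the character's shape.
; CreateRandomImpactParticle spawns an impact billboard offset from HitLocation, with a shuffled texture applied through a dynamic material instance.
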(event `PlayDespawnFX`
  (for _array_element (`self.NS_Despawns`)
    (`self.Activate` _array_element true)
    (`KismetSystemLibrary.PrintString` "Goodbye")))

(event `PlayRespawnFX`
  ; Visibility of Respawn Particles is set to FALSE in Event Graph, sequence must play from 1.0s to skip the outward explosion, and jump to the implosion back into the SKM shape + location
  (for _array_element (`self.NS_Respawns`)
    (`self.Activate` _array_element true)
    (`NiagaraComponent.AdvanceSimulationByTime` _array_element 2.0 3.0)
    (`KismetSystemLibrary.PrintString` "Hello")))

(event `self.ReceiveBeginPlay`
  (bind _returnvalue (`Actor.K2_GetComponentsByClass` (`self.GetOwner`) "/Script/Niagara.NiagaraComponent"))
  ; Finds the Respective Particle Systems for each player
  (for _array_element _returnvalue
    (if (`self.ComponentHasTag` _array_element "FX_Respawn")
      (`KismetArrayLibrary.Array_Add` (`self.NS_Respawns`) _array_element)
      (`KismetSystemLibrary.PrintString` "AddedRespawn")))
  (for _array_element_2 _returnvalue
    (if (`self.ComponentHasTag` _array_element_2 "FX_Despawn")
      (`KismetArrayLibrary.Array_Add` (`self.NS_Despawns`) _array_element_2)
      (`KismetSystemLibrary.PrintString` "AddedDespawn"))))

(fn `Create Random Impact Particle`
  (params (`Hit Location` :type "Transform Structure") (ImpactTextures :type "Array of Texture Object Reference"))
  (locals (`Spawned Particle` :type "NiagaraComponent Object Reference") (Billboards :type "Array of Texture Object Reference"))
  (if (> (`KismetArrayLibrary.Array_Length` ImpactTextures) 0)
    (set `local.Billboards` ImpactTextures))
  (bind _returnvalue (`NiagaraFunctionLibrary.SpawnSystemAtLocation` "/Game/Particles/NiagaraSystems/NS_ImpactBillboard.NS_ImpactBillboard" (+ `Hit Location_Location` (50.0 150.0 50.0)) `Hit Location_Rotation` `Hit Location_Scale`))
  (set `local.Spawned Particle` _returnvalue)
  (bind _returnvalue_2 (`KismetMaterialLibrary.CreateDynamicMaterialInstance` "/Game/Particles/Materials/MI_Impact.MI_Impact"))
  (`KismetArrayLibrary.Array_Shuffle` (`local.Billboards`))
  (`MaterialInstanceDynamic.SetTextureParameterValue` _returnvalue_2 "ImpactBillboard" (`|GetArrayItem` (`local.Billboards`)))
  (`NiagaraComponent.SetVariableMaterial` (`local.Spawned Particle`) "Billboard" _returnvalue_2))