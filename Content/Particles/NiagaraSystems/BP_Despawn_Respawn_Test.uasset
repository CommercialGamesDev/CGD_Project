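; Test Blueprint that previews Niagara respawn and despawn effects on three meshes, with no gameplay logic.
; On BeginPlay, a one-shot chain of delays toggles mesh visibility through appear, vanish and reappear.
; The first appearance restarts three respawn systems and the vanish restarts three despawn systems; the final reappearance triggers no effect.
; Hair-colour tinting and a player movement delay appear only as an author note.
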(event `self.ReceiveBeginPlay`
  ; Can be used to set particle colour to the current hair colour of the player. PLS ADD A 3 SEC DELAY TO PLAYER MOVEMENT ON RESPAWN XXXX
  (`SceneComponent.SetVisibility` (`self.TestMesh`) false false)
  (`SceneComponent.SetVisibility` (`self.TestMesh1`) false false)
  (`SceneComponent.SetVisibility` (`self.MIDDLE`) false false)
  (`KismetSystemLibrary.Delay` 1.0)
  (`SceneComponent.SetVisibility` (`self.TestMesh`) true false)
  (`SceneComponent.SetVisibility` (`self.TestMesh1`) true false)
  (`SceneComponent.SetVisibility` (`self.MIDDLE`) true false)
  (`ActorComponent.SetActive` (`self.NS_Respawn`) true true)
  (`ActorComponent.SetActive` (`self.NS_Respawn1`) true true)
  (`ActorComponent.SetActive` (`self.NS_Respawn2`) true true)
  (`KismetSystemLibrary.Delay` 3.0)
  (`SceneComponent.SetVisibility` (`self.TestMesh`) false false)
  (`SceneComponent.SetVisibility` (`self.TestMesh1`) false false)
  (`SceneComponent.SetVisibility` (`self.MIDDLE`) false false)
  (`ActorComponent.SetActive` (`self.NS_Despawn`) true true)
  (`ActorComponent.SetActive` (`self.NS_Despawn1`) true true)
  (`ActorComponent.SetActive` (`self.NS_Despawn2`) true true)
  (`KismetSystemLibrary.Delay` 3.0)
  (`SceneComponent.SetVisibility` (`self.TestMesh`) true false)
  (`SceneComponent.SetVisibility` (`self.TestMesh1`) true false)
  (`SceneComponent.SetVisibility` (`self.MIDDLE`) true false))

(fn `UserConstructionScript`)