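; BP_SpawnZone is a trigger volume meant to spawn and despawn obstacles as either of two player characters enters or leaves it.
; BeginPlay caches DT_ObstacleData row names matching TriggerID plus the row's index in the whole table.
; Overlap begin and end look up each cached row and pass it to SpawnObstacle or DespawnObstacle.
; Both functions are placeholders that only print the obstacle ID.
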(event `self.ReceiveBeginPlay`
  ;[0.02227 0.15 0 0.5] Init -> Get initial data ONCE (this data table will be read only)
  (`self.InitialiseTriggerData`))

(event `self.CollisionBox.OnComponentBeginOverlap`
  (params (OverlappedComponent :type "PrimitiveComponent Object Reference") (OtherActor :type "Actor Object Reference") (OtherComp :type "PrimitiveComponent Object Reference") (OtherBodyIndex :type Integer) (bFromSweep :type Boolean) (SweepResult :type "HitResult Structure (by ref)"))
  ;[0.1444 0.05636 0.15 0.5] Spawn
  (bind _return (`self.SanitiseActorInput` OtherActor))
  (if _return
    (for _array_element (`self.AllTriggerIDs`)
      (bind _returnvalue (`|GetDataTableRow` "/Game/SpawnSystem/DT_ObstacleData.DT_ObstacleData" _array_element)
        (:`then`
          (`self.SpawnObstacle` _returnvalue))
        (:`RowNotFound`
          (`KismetSystemLibrary.PrintString` (`KismetStringLibrary.Concat_StrStr` (`KismetStringLibrary.Conv_NameToString` _array_element) " not found")))))))

(event `self.CollisionBox.OnComponentEndOverlap`
  (params (OverlappedComponent :type "PrimitiveComponent Object Reference") (OtherActor :type "Actor Object Reference") (OtherComp :type "PrimitiveComponent Object Reference") (OtherBodyIndex :type Integer))
  ;[0.0216 0.1265 0.15 0.5] Despawn
  (bind _return (`self.SanitiseActorInput` OtherActor))
  (if _return
    (for _array_element (`self.AllTriggerIDs`)
      (bind _returnvalue (`|GetDataTableRow` "/Game/SpawnSystem/DT_ObstacleData.DT_ObstacleData" _array_element)
        (:`then`
          (`self.DespawnObstacle` _returnvalue))
        (:`RowNotFound`
          (`KismetSystemLibrary.PrintString` (`KismetStringLibrary.Concat_StrStr` (`KismetStringLibrary.Conv_NameToString` _array_element) " not found")))))))

(fn `DespawnObstacle`
  (params (ObstacleData :type "/Game/SpawnSystem/F_ObstacleStruct Structure"))
  (`KismetSystemLibrary.PrintString` (`KismetStringLibrary.Concat_StrStr` "Removing " (`KismetStringLibrary.Conv_NameToString` ObstacleData_ObstacleID_11_5A80A6A145CEE13DE2995892894810F0) " obstacle in zone.")))

(fn `SpawnObstacle`
  (params (ObstacleData :type "/Game/SpawnSystem/F_ObstacleStruct Structure"))
  (`KismetSystemLibrary.PrintString` (`KismetStringLibrary.Concat_StrStr` "Creating " (`KismetStringLibrary.Conv_NameToString` ObstacleData_ObstacleID_11_5A80A6A145CEE13DE2995892894810F0) " obstacle in zone.")))

(fn `UserConstructionScript`)