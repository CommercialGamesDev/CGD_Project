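; BP_Swingaling is an actor that swings a configurable static mesh by animating its pitch.
; The construction script applies the Mesh variable, caches the starting rotation and slows the SwingSwingSwingaling timeline to a tenth of normal speed.
; Tick calls Play on that timeline, whose update offsets the cached pitch by the negated curve value scaled to degrees, leaving roll and yaw at their starting values.
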(event `self.ReceiveTick`
  (params (DeltaSeconds :type "Float (single-precision)"))
  (bind (_startingrotation_roll _startingrotation_pitch _startingrotation_yaw) (`KismetMathLibrary.BreakRotator` (`self.StartingRotation`)))
  (bind (_direction _swingalinga) (`Timeline|SwingSwingSwingaling`)
    (:`Update`
      (`self.K2_SetActorRotation` self (`KismetMathLibrary.MakeRotator` _startingrotation_roll (+ _startingrotation_pitch (* (- _swingalinga (* _swingalinga 2.0)) 30.0)) _startingrotation_yaw) false))))

(fn `UserConstructionScript`
  (`StaticMeshComponent.SetStaticMesh` (`self.StaticMesh`) (`self.Mesh`))
  (set `self.StartingRotation` (`self.K2_GetActorRotation` self))
  (`TimelineComponent.SetPlayRate` (`self.SwingSwingSwingaling`) 0.1))