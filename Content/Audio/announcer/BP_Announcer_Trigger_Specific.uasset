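; A trigger actor that makes the level's BP_Announcer say a specific sound as the two players enter or leave it.
; It counts player pawns 0 and 1 through overlap begin and end events.
; Flags select whether it fires on one player inside, both inside, or both gone, with an optional once-only limit.
; When it fires, it looks up the announcer by class and passes the sound to SaySpecific.
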(event `self.ReceiveActorBeginOverlap`
  (params (OtherActor :type "Actor Object Reference"))
  (if (or (== OtherActor (`GameplayStatics.GetPlayerPawn` 0)) (== OtherActor (`GameplayStatics.GetPlayerPawn` 1)))
    (`/Engine/EditorBlueprintResources/StandardMacros.IncrementInt` (`self.NoPlayersInside`)
      (:`  `
        (if (and (or (and (`self.OnBothPlayersEntering`) (== (`self.NoPlayersInside`) 2)) (and (`self.On1PlayerEntering`) (== (`self.NoPlayersInside`) 1))) (or (not (`self.DoOnce`)) (not (`self.HaveDone`))))
          (bind _returnvalue (`GameplayStatics.GetActorOfClass` "/Game/Audio/announcer/BP_Announcer.BP_Announcer_C"))
          (`/Game/Audio/announcer/BP_Announcer.SaySpecific` _returnvalue (`self.Sound`))
          (set `self.HaveDone` true))))))

(event `self.ReceiveActorEndOverlap`
  (params (OtherActor :type "Actor Object Reference"))
  (if (or (== OtherActor (`GameplayStatics.GetPlayerPawn` 0)) (== OtherActor (`GameplayStatics.GetPlayerPawn` 1)))
    (`/Engine/EditorBlueprintResources/StandardMacros.DecrementInt` (`self.NoPlayersInside`)
      (:`  `
        (if (and (and (`self.OnBothPlayersLeaving`) (== (`self.NoPlayersInside`) 0)) (or (not (`self.DoOnce`)) (not (`self.HaveDone`))))
          (bind _returnvalue (`GameplayStatics.GetActorOfClass` "/Game/Audio/announcer/BP_Announcer.BP_Announcer_C"))
          (`/Game/Audio/announcer/BP_Announcer.SaySpecific` _returnvalue (`self.Sound`))
          (set `self.HaveDone` true))))))

(fn `UserConstructionScript`)