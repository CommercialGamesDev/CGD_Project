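; Announcer actor that voices game events with subtitled commentary and audience cheers.
; Say picks a random non-repeating line per category under a cooldown, often rerolling rare lines, then triggers crowd sound and animation.
; SaySpecific plays audio and subtitles, holding the line until any red curtain widget is gone.
; Respawn resets backtracker triggers and counts rapid respawns, triggering a comment and Pity state that the next checkpoint answers and clears.
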(event `self.ReceiveBeginPlay`
  (set `AudioComponent.bSuppressSubtitles` true (`self.Audio`))
  (bind _returnvalue (`|CreateWidget` "/Game/Audio/announcer/WBP_Announcer.WBP_Announcer_C"))
  (bind _output_get (set `self.Subtitles` _returnvalue))
  (`UserWidget.AddToPlayerScreen` _output_get 2147483647)
  (bind _returnvalue_2 (`GameplayStatics.GetActorOfClass` "/Game/Audience/BP_AudienceGlobalManager.BP_AudienceGlobalManager_C"))
  (set `self.AudienceCheerAnim` _returnvalue_2))

(event `self.ReceiveTick`
  (params (DeltaSeconds :type "Float (single-precision)"))
  (if (not (== (`self.LineToSay`) null))
    (bind _foundwidgets (`WidgetBlueprintLibrary.GetAllWidgetsOfClass` "/Game/UI/RedCurtain/WBP_RedCurtain.WBP_RedCurtain_C" false))
    (if (`KismetArrayLibrary.Array_IsEmpty` _foundwidgets)
      (`self.SaySpecific` (`self.LineToSay`))))
  (if (!= (`self.RespawnCount`) 0)
    (bind _output_get (set `self.RespawnTimer` (- (`self.RespawnTimer`) DeltaSeconds)))
    (if (<= _output_get 0.0)
      (set `self.RespawnTimer` 0.0)
      (set `self.RespawnCount` 0)))
  (if (!= (`self.Cooldown`) 0.0)
    (bind _output_get_2 (set `self.Cooldown` (- (`self.Cooldown`) DeltaSeconds)))
    (if (< _output_get_2 0.0)
      (set `self.Cooldown` 0.0))))

(fn `Checkpoint`
  (if (`self.Pity`)
    (set `self.Pity` false)
    (`self.Say` "NewEnumerator15")
    (set `self.RespawnTimer` 0.0)
    (set `self.RespawnCount` 0)))

(fn `Respawn`
  (bind _outactors (`GameplayStatics.GetAllActorsOfClass` "/Game/Audio/announcer/BP_Backtracker_Trigger.BP_Backtracker_Trigger_C"))
  (for _array_element _outactors
    (`/Game/Audio/announcer/BP_Backtracker_Trigger.Respawn` _array_element))
  (bind _result (`/Engine/EditorBlueprintResources/StandardMacros.IncrementInt` (`self.RespawnCount`))
    (:`  `
      (set `self.RespawnTimer` 20.0)
      (if (> _result 4)
        (`self.Say` "NewEnumerator5")
        (set `self.Pity` true)))))

(fn `Say`
  (params (`Voice Line` :type "/Game/Audio/announcer/E_VoiceLines Enum" :default "NewEnumerator0"))
  (locals (NextLine :type "SoundBase Object Reference"))
  (bind _returnvalue (`KismetMathLibrary.Conv_ByteToInt` `Voice Line`))
  (bind (_output_name _output_soundfiles) (break `/Game/Audio/announcer/S_VoiceLines` (`|GetArrayItem` (`self.AudienceSoundFiles`) _returnvalue)))
  (bind (_output_name_2 _output_soundfiles_2) (break `/Game/Audio/announcer/S_VoiceLines` (`|GetArrayItem` (`self.SoundFiles`) _returnvalue)))
  (bind _outitem (`KismetArrayLibrary.Array_Random` _output_soundfiles))
  (bind _duration (`SoundBase.Duration` _outitem))
  (if (== (`self.Cooldown`) 0.0)
    (set `self.Cooldown` (`self.MaxCooldown`))
    (set `local.NextLine` (`AudioComponent.Sound` (`self.Audio`)))
    (while (or (== (`AudioComponent.Sound` (`self.Audio`)) (`local.NextLine`)) (and (`KismetMathLibrary.RandomBool`) (`KismetArrayLibrary.Array_Contains` (`self.RareLines`) (`local.NextLine`))))
      (set `local.NextLine` (`KismetArrayLibrary.Array_Random` _output_soundfiles_2)))
    (`self.SaySpecific` (`local.NextLine`))
    (if (not (== _outitem null))
      (`/Engine/EditorBlueprintResources/StandardMacros.IsValid` _outitem
        (:`Is Valid`
          (`GameplayStatics.PlaySound2D` _outitem 1.0 1.0 0.0 null null)
          (if (!= _duration 0.0)
            (bind _audiencecheeranim (`self.AudienceCheerAnim`)
              (:`then`
                (`/Game/Audience/BP_AudienceGlobalManager.CheerAudience` _audiencecheeranim _duration))
              (:`else`
                _))))
        (:`Is Not Valid`
          _)))
    (if (or (`|EnumEquality` `Voice Line` "NewEnumerator0") (`|EnumEquality` `Voice Line` "NewEnumerator1") (`|EnumEquality` `Voice Line` "NewEnumerator2"))
      (`/Game/Audio/announcer/WBP_Announcer.MoveUp` (`self.Subtitles`)))))

(fn `SaySpecific`
  (params (`Say what?` :type "SoundBase Object Reference"))
  (bind _foundwidgets (`WidgetBlueprintLibrary.GetAllWidgetsOfClass` "/Game/UI/RedCurtain/WBP_RedCurtain.WBP_RedCurtain_C" false))
  (if (`KismetArrayLibrary.Array_IsEmpty` _foundwidgets)
    (`AudioComponent.SetSound` (`self.Audio`) `Say what?`)
    (`AudioComponent.Play` (`self.Audio`) 0.0)
    (`self.Subtitle`)
    (set `self.LineToSay` null)
    (else
      (set `self.LineToSay` `Say what?`))))

(fn `Subtitle`
  (locals (`Subtitles Copy` :type "Array of SubtitleCue Structure"))
  (if (`/Game/Audio/announcer/WBP_Announcer.Enabled` (`self.Subtitles`))
    (bind _assound_wave (cast `SoundWave` (`AudioComponent.Sound` (`self.Audio`))))
    (bind _output_get (set `local.Subtitles Copy` (`SoundWave.Subtitles` _assound_wave)))
    (`/Game/Audio/announcer/WBP_Announcer.Say` (`self.Subtitles`) _output_get)))

(fn `UserConstructionScript`)