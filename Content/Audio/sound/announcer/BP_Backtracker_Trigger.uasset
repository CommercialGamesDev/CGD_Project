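; BP_Backtracker_Trigger is a two-player trigger that makes BP_Announcer speak a line when players backtrack.
; Every Tick it polls pawn overlaps on its Forward and Backward components instead of using overlap events.
; Forward sets a flag for each of the first two player pawns and Backward clears it.
; The line plays only when clearing a flag leaves neither player flagged.
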(event `self.ReceiveTick`
  (params (DeltaSeconds :type "Float (single-precision)"))
  (bind _outactors (`KismetSystemLibrary.ComponentOverlapActors` (`self.Backward`) (`SceneComponent.K2_GetComponentToWorld` (`self.Backward`)) (`|MakeArray` "ObjectTypeQuery3" :!type "EObjectTypeQuery Enum")))
  (if (and (`KismetArrayLibrary.Array_Contains` _outactors (`GameplayStatics.GetPlayerPawn` 0)) (`self.Player1`))
    (set `self.Player1` false)
    (if (not (`self.Player2`))
      (bind _returnvalue (`GameplayStatics.GetActorOfClass` "/Game/Audio/sound/announcer/BP_Announcer.BP_Announcer_C"))
      (`/Game/Audio/sound/announcer/BP_Announcer.Say` _returnvalue "NewEnumerator8")
      (else
        (if (and (`KismetArrayLibrary.Array_Contains` _outactors (`GameplayStatics.GetPlayerPawn` 1)) (`self.Player2`)) :!label _label
          (set `self.Player2` false)
          (if (not (`self.Player1`))
            (bind _returnvalue_2 (`GameplayStatics.GetActorOfClass` "/Game/Audio/sound/announcer/BP_Announcer.BP_Announcer_C"))
            (`/Game/Audio/sound/announcer/BP_Announcer.Say` _returnvalue_2 "NewEnumerator8")
            (else
              (bind _outactors_2 (`KismetSystemLibrary.ComponentOverlapActors` (`self.Forward`) (`SceneComponent.K2_GetComponentToWorld` (`self.Forward`)) (`|MakeArray` "ObjectTypeQuery3" :!type "EObjectTypeQuery Enum") :!label _label_2))
              (if (and (`KismetArrayLibrary.Array_Contains` _outactors_2 (`GameplayStatics.GetPlayerPawn` 0)) (not (`self.Player1`)))
                (set `self.Player1` true))
              (if (and (`KismetArrayLibrary.Array_Contains` _outactors_2 (`GameplayStatics.GetPlayerPawn` 1)) (not (`self.Player2`)))
                (set `self.Player2` true))))
          (else
            (goto _label_2)))))
    (else
      (goto _label))))

(fn `UserConstructionScript`)