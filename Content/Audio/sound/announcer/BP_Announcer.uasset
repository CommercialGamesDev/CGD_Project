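; Announcer Blueprint that plays queued voice lines one at a time and shows their subtitles in its own WBP_Announcer widget, with the audio component's built-in subtitles suppressed.
; Tick starts the next queued category once audio is idle, picking a random variant that avoids the previous index and rerolls rare lines by coin flip.
; Respawn counts repeated respawns within a refreshing cooldown and queues a comment at certain counts.
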(event `self.ReceiveBeginPlay`
  (`KismetArrayLibrary.Array_Clear` (`self.Queue`))
  (set `AudioComponent.bSuppressSubtitles` true (`self.Audio`))
  (bind _returnvalue (`|CreateWidget` "/Game/Audio/sound/announcer/WBP_Announcer.WBP_Announcer_C"))
  (bind _output_get (set `self.Subtitles` _returnvalue))
  (`UserWidget.AddToPlayerScreen` _output_get 0))

(event `self.ReceiveTick`
  (params (DeltaSeconds :type "Float (single-precision)"))
  (bind (_output_name _output_soundfiles) (break `/Game/Audio/sound/announcer/S_VoiceLines` (`|GetArrayItem` (`self.SoundFiles`) (`KismetMathLibrary.Conv_ByteToInt` (`|GetArrayItem` (`self.Queue`))))))
  (bind (_output_name_2 _output_soundfiles_2) (break `/Game/Audio/sound/announcer/S_VoiceLines` (`|GetArrayItem` (`self.SoundFiles`) (`KismetMathLibrary.Conv_ByteToInt` (`|GetArrayItem` (`self.Queue`))))))
  (bind (_output_name_3 _output_soundfiles_3) (break `/Game/Audio/sound/announcer/S_VoiceLines` (`|GetArrayItem` (`self.SoundFiles`) (`KismetMathLibrary.Conv_ByteToInt` (`|GetArrayItem` (`self.Queue`))))))
  (if (and (`KismetArrayLibrary.Array_IsNotEmpty` (`self.Queue`)) (not (`AudioComponent.IsPlaying` (`self.Audio`))))
    (set `self.NextVoiceLine` (`self.PrevVoiceLine`))
    (while (or (== (`self.PrevVoiceLine`) (`self.NextVoiceLine`)) (and (`KismetMathLibrary.RandomBool`) (`KismetArrayLibrary.Array_Contains` (`self.RareLines`) (`|GetArrayItem` _output_soundfiles_3 (`self.NextVoiceLine`)))))
      (set `self.NextVoiceLine` (`.OutIndex` (`KismetArrayLibrary.Array_Random` _output_soundfiles_2))))
    (`AudioComponent.SetSound` (`self.Audio`) (`|GetArrayItem` _output_soundfiles (`self.NextVoiceLine`)))
    (set `self.PrevVoiceLine` (`self.NextVoiceLine`))
    (`AudioComponent.Play` (`self.Audio`) 0.0)
    (`KismetArrayLibrary.Array_Remove` (`self.Queue`))
    (bind _assound_wave (cast `SoundWave` (`AudioComponent.Sound` (`self.Audio`)))
      (:`then`
        (set `self.Subtitles_0` (`SoundWave.Subtitles` _assound_wave))
        (`/Game/Audio/sound/announcer/WBP_Announcer.Say` (`self.Subtitles`) (`self.Subtitles_0`)))
      (:`CastFailed`
        _)))
  (if (!= (`self.RespawnCount`) 0)
    (bind _output_get (set `self.RespawnTimer` (- (`self.RespawnTimer`) DeltaSeconds)))
    (if (<= _output_get 0.0)
      (set `self.RespawnTimer` 0.0)
      (set `self.RespawnCount` 0))))

(fn `Respawn`
  (bind _result (`/Engine/EditorBlueprintResources/StandardMacros.IncrementInt` (`self.RespawnCount`))
    (:`  `
      (set `self.RespawnTimer` 20.0)
      (if (or (== _result 3) (> _result 4))
        (`self.Say` "NewEnumerator5")))))

(fn `Say`
  (params (`Voice Line` :type "/Game/Audio/sound/announcer/E_VoiceLines Enum" :default "NewEnumerator0"))
  (`KismetArrayLibrary.Array_Add` (`self.Queue`) `Voice Line`))

(fn `UserConstructionScript`)