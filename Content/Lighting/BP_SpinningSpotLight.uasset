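; A spotlight Blueprint that continuously sweeps its SpotLight component through a repeating rotation.
; Tick passes through a DoOnce gate to play a Timeline from the start at SpinRate, and the Timeline resets the gate on finishing, so the motion loops.
; The Timeline track interpolates between StartRotation and EndRotation, setting relative yaw to that value and pitch to its negative, with zero roll.
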(event `self.ReceiveTick`
  (params (DeltaSeconds :type "Float (single-precision)"))
  (`/Engine/EditorBlueprintResources/StandardMacros.DoOnce` false :!label _label
    (:`Completed`
      (`TimelineComponent.SetPlayRate` (`self.Timeline`) (`self.SpinRate`))
      (bind (_direction _newtrack_0) (`Timeline|Timeline` :!via `PlayFromStart`)
        (:`Update`
          (bind _returnvalue (`KismetMathLibrary.Lerp` (`self.StartRotation`) (`self.EndRotation`) _newtrack_0))
          (`SceneComponent.K2_SetRelativeRotation` (`self.SpotLight`) (`KismetMathLibrary.MakeRotator` 0.0 (- 0.0 _returnvalue) _returnvalue) false false))
        (:`Finished`
          (goto _label :!via `Reset`))))))

(fn `UserConstructionScript`)