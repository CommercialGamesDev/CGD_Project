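; BP_StageLight is a stage light prop that pairs a spot light with a tinted Light component.
; The construction script applies exposed distance, colour, brightness and cone angle variables to the SpotLight.
; It also pushes the same colour into the Colour parameter on the Light component's materials, so the fixture matches the beam.
; The event graph holds only disabled placeholder events, so nothing runs at play time.
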(fn `UserConstructionScript`
  (bind _spotlight (`self.SpotLight`))
  (`LocalLightComponent.SetAttenuationRadius` _spotlight (`self.Distance`))
  (`LightComponent.SetLightColor` _spotlight (`KismetMathLibrary.Conv_ColorToLinearColor` (`self.Colour`)) false)
  (`LightComponent.SetIntensity` _spotlight (`self.Brightness`))
  (`SpotLightComponent.SetOuterConeAngle` _spotlight (`self.OuterConeAngle`))
  (`SpotLightComponent.SetInnerConeAngle` _spotlight (`self.InnerConeAngle`))
  (`MeshComponent.SetColorParameterValueOnMaterials` (`self.Light`) "Colour" (`KismetMathLibrary.Conv_ColorToLinearColor` (`self.Colour`))))