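; BP_OscSpotLight is a spotlight that continuously swings back and forth.
; Tick passes through a DoOnce that sets the timeline's play rate from SwingRate and uses TurnPoint to alternate between playing and reversing it.
; Timeline updates lerp the light's relative pitch and yaw between negative and positive MaxRotationY and MaxRotationX.
; Each finish resets the DoOnce, starting the next swing.
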(event `self.ReceiveTick`
  (params (DeltaSeconds :type "Float (single-precision)"))
  (bind _maxrotationx (`self.MaxRotationX`))
  (bind _maxrotationy (`self.MaxRotationY`))
  (`/Engine/EditorBlueprintResources/StandardMacros.DoOnce` false :!label _label
    (:`Completed`
      (`TimelineComponent.SetPlayRate` (`self.Timeline`) (`self.SwingRate`))
      (if (`self.Turn Point`)
        (set `self.Turn Point` false)
        (bind (_direction _newtrack_0) (`Timeline|Timeline` :!via `Reverse` :!label _label_2)
          (:`Update`
            (`SceneComponent.K2_SetRelativeRotation` (`self.SpotLight`) (`KismetMathLibrary.MakeRotator` 0.0 (`KismetMathLibrary.Lerp` (- 0.0 _maxrotationy) _maxrotationy _newtrack_0) (`KismetMathLibrary.Lerp` (- 0.0 _maxrotationx) _maxrotationx _newtrack_0)) false false))
          (:`Finished`
            (goto _label :!via `Reset`)))
        (else
          (set `self.Turn Point` true)
          (goto _label_2))))))

(fn `UserConstructionScript`)