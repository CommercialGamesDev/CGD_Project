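; Light area trigger actor that shows its assigned light actors while a BP_ThirdPersonCharacter is inside and hides them when it leaves.
; Collision overlap events toggle an Active flag to skip redundant switches, then scan every row of DT_LightTable.
; EvaluateLight resolves each row's soft area and light references, returning the light as valid only when the area is this actor.
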(event `self.Collision.OnComponentBeginOverlap`
  (params (OverlappedComponent :type "PrimitiveComponent Object Reference") (OtherActor :type "Actor Object Reference") (OtherComp :type "PrimitiveComponent Object Reference") (OtherBodyIndex :type Integer) (bFromSweep :type Boolean) (SweepResult :type "HitResult Structure (by ref)"))
  (if (and (`GameplayStatics.ObjectIsA` OtherActor "/Game/ThirdPerson/Blueprints/BP_ThirdPersonCharacter.BP_ThirdPersonCharacter_C") (!= (`self.Active?`) true))
    (set `self.Active?` true)
    (bind _outrownames (`DataTableFunctionLibrary.GetDataTableRowNames` "/Game/Lighting/DataTables/DT_LightTable.DT_LightTable"))
    (for _array_element _outrownames
      (bind (_isvalid _light) (`self.EvaluateLight` _array_element))
      (if _isvalid
        (`self.SetActorHiddenInGame` _light false)))))

(event `self.Collision.OnComponentEndOverlap`
  (params (OverlappedComponent :type "PrimitiveComponent Object Reference") (OtherActor :type "Actor Object Reference") (OtherComp :type "PrimitiveComponent Object Reference") (OtherBodyIndex :type Integer))
  (if (and (`GameplayStatics.ObjectIsA` OtherActor "/Game/ThirdPerson/Blueprints/BP_ThirdPersonCharacter.BP_ThirdPersonCharacter_C") (!= (`self.Active?`) false))
    (set `self.Active?` false)
    (bind _outrownames (`DataTableFunctionLibrary.GetDataTableRowNames` "/Game/Lighting/DataTables/DT_LightTable.DT_LightTable"))
    (for _array_element _outrownames
      (bind (_isvalid _light) (`self.EvaluateLight` _array_element))
      (if _isvalid
        (`self.SetActorHiddenInGame` _light true)))))

(fn `EvaluateLight`
  (params (DataRow :type Name))
  (returns (IsValid :type Boolean) (Light :type "Actor Object Reference"))
  (bind _returnvalue (`|GetDataTableRow` "/Game/Lighting/DataTables/DT_LightTable.DT_LightTable" DataRow)
    (:`then`
      (if (and (`KismetSystemLibrary.IsValidSoftObjectReference` (break `/Game/Lighting/DataTables/F_LightData` _returnvalue)) (`KismetSystemLibrary.IsValidSoftObjectReference` (`.LightObject_7_7B81F3E64AAC8BC41F122EA65FDD0375` (break `/Game/Lighting/DataTables/F_LightData` _returnvalue))))
        (bind _output_get (set `self.AreaObject` (`|ConvertAsset` (break `/Game/Lighting/DataTables/F_LightData` _returnvalue))))
        (bind _output_get_2 (set `self.LightObject` (`|ConvertAsset` (`.LightObject_7_7B81F3E64AAC8BC41F122EA65FDD0375` (break `/Game/Lighting/DataTables/F_LightData` _returnvalue)))))
        (return (== _output_get self) _output_get_2)
        (else
          (return false null))))
    (:`RowNotFound`
      (return false null))))

(fn `UserConstructionScript`)